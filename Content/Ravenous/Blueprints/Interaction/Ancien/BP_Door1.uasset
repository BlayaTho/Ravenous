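; Hand-operated door that the first-person player pushes or pulls by holding left mouse and moving forward or backward.
; Interact glides the player to an anchor mesh, then Tick rotates the door from that input while pinning the player there.
; Anchor and look-at meshes interpolate with door yaw, steering player position and camera.
; Past the angle limit, a timeline swings the door fully open, and the next Interact closes it.
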(event `self.ReceiveBeginPlay`
  (bind _asbp_first_person_character (cast `/Game/Ravenous/Blueprints/Player/BP_FirstPersonCharacter` (`GameplayStatics.GetPlayerCharacter` 0)))
  (set `self.As BP First Person Character` _asbp_first_person_character))

(event `self.ReceiveTick`
  (params (DeltaSeconds :type "Float (single-precision)"))
  (bind _staticmeshp (`self.StaticMeshP`))
  (bind _as_bp_first_person_character (`self.As BP First Person Character`))
  (bind _openangle (`self.OpenAngle`))
  (bind _staticmeshp_2 (`self.StaticMeshP`))
  (bind _interp_speed (`self.Interp Speed`))
  (bind _interp_speed_2 (`self.Interp Speed`))
  (bind _staticmeshp_3 (`self.StaticMeshP`))
  (bind _interp_speed_3 (`self.Interp Speed`))
  (bind _staticmeshp_4 (`self.StaticMeshP`))
  (bind _as_bp_first_person_character_2 (`self.As BP First Person Character`))
  (bind _interp_speed_4 (`self.Interp Speed`))
  (bind _door (`self.Door`))
  (bind (_returnvalue_x _returnvalue_y) (`KismetMathLibrary.BreakVector` (`SceneComponent.K2_GetComponentLocation` (`self.StaticMeshPlayer`))))
  (bind (_returnvalue_roll _returnvalue_pitch _returnvalue_yaw) (`KismetMathLibrary.BreakRotator` (`SceneComponent.K2_GetComponentRotation` (`self.Door`))))
  (bind (_returnvalue_x_2 _returnvalue_y_2 _returnvalue_z) (`KismetMathLibrary.BreakVector` (`self.K2_GetActorLocation` _as_bp_first_person_character)))
  (bind (_returnvalue_roll_2 _returnvalue_pitch_2 _returnvalue_yaw_2) (`KismetMathLibrary.BreakRotator` (`SceneComponent.K2_GetComponentRotation` (`self.Door`))))
  (bind (_relativelocation_x _relativelocation_y _relativelocation_z) (`KismetMathLibrary.BreakVector` (`SceneComponent.RelativeLocation` _staticmeshp)))
  (bind (_relativerotation_roll _relativerotation_pitch _relativerotation_yaw) (`KismetMathLibrary.BreakRotator` (`SceneComponent.RelativeRotation` (`self.Door`))))
  (bind (_relativelocation_x_2 _relativelocation_y_2 _relativelocation_z_2) (`KismetMathLibrary.BreakVector` (`SceneComponent.RelativeLocation` (`self.StaticMeshPlayer`))))
  (bind (_relativelocation_x_3 _relativelocation_y_3) (`KismetMathLibrary.BreakVector` (`SceneComponent.RelativeLocation` (`self.StaticMeshCiblePlayer`))))
  (bind (_relativerotation_roll_2 _relativerotation_pitch_2 _relativerotation_yaw_2) (`KismetMathLibrary.BreakRotator` (`SceneComponent.RelativeRotation` (`self.Door`))))
  (bind (_relativelocation_x_4 _relativelocation_y_4 _relativelocation_z_3) (`KismetMathLibrary.BreakVector` (`SceneComponent.RelativeLocation` (`self.StaticMeshPlayer`))))
  (bind (_relativelocation_x_5 _relativelocation_y_5 _relativelocation_z_4) (`KismetMathLibrary.BreakVector` (`SceneComponent.RelativeLocation` _staticmeshp_2)))
  (bind (_relativelocation_x_6 _relativelocation_y_6 _relativelocation_z_5) (`KismetMathLibrary.BreakVector` (`SceneComponent.RelativeLocation` _staticmeshp_3)))
  (bind (_relativelocation_x_7 _relativelocation_y_7 _relativelocation_z_6) (`KismetMathLibrary.BreakVector` (`SceneComponent.RelativeLocation` _staticmeshp_4)))
  (bind (_relativelocation_x_8 _relativelocation_y_8) (`KismetMathLibrary.BreakVector` (`SceneComponent.RelativeLocation` (`self.StaticMeshP1`))))
  (bind (_relativelocation_x_9 _relativelocation_y_9) (`KismetMathLibrary.BreakVector` (`SceneComponent.RelativeLocation` (`self.StaticMeshP1`))))
  (bind (_relativerotation_roll_3 _relativerotation_pitch_3 _relativerotation_yaw_3) (`KismetMathLibrary.BreakRotator` (`SceneComponent.RelativeRotation` _door)))
  (bind _returnvalue (> _relativerotation_yaw_2 15.0))
  (bind _returnvalue_2 (< _relativerotation_yaw_2 -20.0))
  (`KismetSystemLibrary.PrintString` (`KismetStringLibrary.Conv_DoubleToString` _relativerotation_yaw) true true (struct :`G` 0.66 :`B` 1.0 :`A` 1.0) 0.0)
  (if (`/Game/Ravenous/Blueprints/Player/BP_FirstPersonCharacter.inDoorInteraction` _as_bp_first_person_character_2)
    (if (`/Game/Ravenous/Blueprints/Player/BP_FirstPersonCharacter.isHoldingLMB` _as_bp_first_person_character_2)
      (if (`self.CanStartIntera`)
        (`self.K2_SetActorLocation` _as_bp_first_person_character (`KismetMathLibrary.MakeVector` _returnvalue_x _returnvalue_y _returnvalue_z) false false)
        (if (not (== _returnvalue_yaw (`KismetMathLibrary.ClampAngle` _returnvalue_yaw _openangle (* _openangle -1.0))))
          (`SceneComponent.K2_AddRelativeRotation` (`self.Door`) (`KismetMathLibrary.MakeRotator` 0.0 0.0 (* (`/Game/Ravenous/Blueprints/Player/BP_FirstPersonCharacter.ForwardBackward` (`self.As BP First Person Character`)) (`self.Sensi`))) false false)
          (`|ExecutionSequence`
            (:`then_0`
              (if (or _returnvalue_2 _returnvalue)
                (if _returnvalue_2
                  (`SceneComponent.K2_SetRelativeLocation` (`self.StaticMeshPlayer`) (`KismetMathLibrary.MakeVector` (`KismetMathLibrary.FInterpTo` _relativelocation_x_2 _relativelocation_x_3 (`GameplayStatics.GetWorldDeltaSeconds`) _interp_speed) (`KismetMathLibrary.FInterpTo` _relativelocation_y_2 _relativelocation_y_3 (`GameplayStatics.GetWorldDeltaSeconds`) _interp_speed) _relativelocation_z_2) false false)
                  (`SceneComponent.K2_SetRelativeLocation` _staticmeshp_3 (`KismetMathLibrary.MakeVector` _relativelocation_x_6 _relativelocation_y_6 (`KismetMathLibrary.FInterpTo` _relativelocation_z_5 140.0 (`GameplayStatics.GetWorldDeltaSeconds`) _interp_speed)) false false)
                  (elif _returnvalue
                    (if (> _relativerotation_yaw_2 30.0)
                      (`SceneComponent.K2_SetRelativeLocation` _staticmeshp_2 (`KismetMathLibrary.MakeVector` (`KismetMathLibrary.FInterpTo` _relativelocation_x_5 0.0 (`GameplayStatics.GetWorldDeltaSeconds`) _interp_speed_4) (`KismetMathLibrary.FInterpTo` _relativelocation_y_5 _relativelocation_y_9 (`GameplayStatics.GetWorldDeltaSeconds`)) (`KismetMathLibrary.FInterpTo` _relativelocation_z_4 140.0 (`GameplayStatics.GetWorldDeltaSeconds`) _interp_speed_4)) false false)
                      (else
                        (`SceneComponent.K2_SetRelativeLocation` _staticmeshp_4 (`KismetMathLibrary.MakeVector` (`KismetMathLibrary.FInterpTo` _relativelocation_x_7 _relativelocation_x_8 (`GameplayStatics.GetWorldDeltaSeconds`) (`self.Interp Speed`)) (`KismetMathLibrary.FInterpTo` _relativelocation_y_7 _relativelocation_y_8 (`GameplayStatics.GetWorldDeltaSeconds`) (`self.Interp Speed`)) _relativelocation_z_6) false false)))))
                (else
                  (`SceneComponent.K2_SetRelativeLocation` (`self.StaticMeshPlayer`) (`KismetMathLibrary.MakeVector` (`KismetMathLibrary.FInterpTo` _relativelocation_x_4 -30.0 (`GameplayStatics.GetWorldDeltaSeconds`) _interp_speed_2) (`KismetMathLibrary.FInterpTo` _relativelocation_y_4 -70.0 (`GameplayStatics.GetWorldDeltaSeconds`) _interp_speed_2) _relativelocation_z_3) false false)
                  (`SceneComponent.K2_SetRelativeLocation` _staticmeshp (`KismetMathLibrary.MakeVector` (`KismetMathLibrary.FInterpTo` _relativelocation_x 15.0 (`GameplayStatics.GetWorldDeltaSeconds`) _interp_speed_3) (`KismetMathLibrary.FInterpTo` _relativelocation_y -85.0 (`GameplayStatics.GetWorldDeltaSeconds`) _interp_speed_3) (`KismetMathLibrary.FInterpTo` _relativelocation_z 115.0 (`GameplayStatics.GetWorldDeltaSeconds`) _interp_speed_3)) false false))))
            (:`then_1`
              (`self.PlayerFaceDoor` :!label _label)))
          (else
            (if (>= _returnvalue_yaw_2 (`self.OpenAngle`))
              (set `self.TargetAngleOpen` 100.0)
              (else
                (set `self.TargetAngleOpen` -100.0)))
            (`/Engine/EditorBlueprintResources/StandardMacros.DoOnce` false :!label _label_2
              (:`Completed`
                (`|ExecutionSequence`
                  (:`then_0`
                    (set `self.StopClamp` true)
                    (set `/Game/Ravenous/Blueprints/Player/BP_FirstPersonCharacter.inDoorInteraction` false (`self.As BP First Person Character`))
                    (set `self.CanStartIntera` false))
                  (:`then_1`
                    (bind (_direction _lerp) (`Timeline|Timeline_0` :!via `PlayFromStart`)
                      (:`Update`
                        (`SceneComponent.K2_SetRelativeRotation` _door (`KismetMathLibrary.MakeRotator` 0.0 0.0 (`KismetMathLibrary.Lerp` _relativerotation_yaw_3 (`self.TargetAngleOpen`) _lerp)) false false)))))))))
        (else
          (goto _label)))
      (else
        (set `/Game/Ravenous/Blueprints/Player/BP_FirstPersonCharacter.inDoorInteraction` false _as_bp_first_person_character_2)
        (set `self.CanStartIntera` false)))))

(event `self.Interact`
  (params (ForDoor :type Boolean) (ForLock :type Boolean) (Name :type String))
  (bind _as_bp_first_person_character (`self.As BP First Person Character`))
  (bind _door (`self.Door`))
  (bind (_returnvalue_x _returnvalue_y) (`KismetMathLibrary.BreakVector` (`SceneComponent.K2_GetComponentLocation` (`self.StaticMeshPlayer`))))
  (bind (_returnvalue_x_2 _returnvalue_y_2 _returnvalue_z) (`KismetMathLibrary.BreakVector` (`self.K2_GetActorLocation` _as_bp_first_person_character)))
  (bind (_relativerotation_roll _relativerotation_pitch _relativerotation_yaw) (`KismetMathLibrary.BreakRotator` (`SceneComponent.RelativeRotation` _door)))
  (if (`self.StopClamp`)
    (bind (_direction _lerp) (`Timeline|Timeline_1` :!via `PlayFromStart`)
      (:`Update`
        (`SceneComponent.K2_SetRelativeRotation` _door (`KismetMathLibrary.MakeRotator` 0.0 0.0 (`KismetMathLibrary.Lerp` _relativerotation_yaw 0.0 _lerp)) false false))
      (:`Finished`
        (set `self.StopClamp` false)))
    (else
      (set `/Game/Ravenous/Blueprints/Player/BP_FirstPersonCharacter.inDoorInteraction` true (`self.As BP First Person Character`))
      (bind (_direction_2 _lerp_2) (`Timeline|Timeline` :!via `PlayFromStart`)
        (:`Update`
          (`self.K2_SetActorLocation` _as_bp_first_person_character (`KismetMathLibrary.MakeVector` (`KismetMathLibrary.Lerp` _returnvalue_x_2 _returnvalue_x _lerp_2) (`KismetMathLibrary.Lerp` _returnvalue_y_2 _returnvalue_y _lerp_2) _returnvalue_z) false false))
        (:`Finished`
          (set `self.CanStartIntera` true)
          (`self.resetDoOnce`))))))

(event `resetDoOnce`
  (goto _label_2 :!via `Reset`))

(event `PlayerFaceDoor`
  (bind _as_bp_first_person_character (`self.As BP First Person Character`))
  (`Controller.SetControlRotation` (`GameplayStatics.GetPlayerController` 0) (`KismetMathLibrary.RInterpTo` (`Pawn.GetControlRotation` _as_bp_first_person_character) (`KismetMathLibrary.FindLookAtRotation` (`SceneComponent.K2_GetComponentLocation` (`/Game/Ravenous/Blueprints/Player/BP_FirstPersonCharacter.FirstPersonCamera` _as_bp_first_person_character)) (`SceneComponent.K2_GetComponentLocation` (`self.StaticMeshP`))) (`GameplayStatics.GetWorldDeltaSeconds`) 5.0)))

(fn `UserConstructionScript`)