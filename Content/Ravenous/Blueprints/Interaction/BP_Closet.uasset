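; BP_Closet is an interactable closet with separately operable drawers, selected by the component name passed to the Interact event.
; Most drawers toggle open and shut through a FlipFlop and timeline that lerps relative X from BeginLocationX to OpenAngle, a position despite its name.
; Closet01DrawerSmall2 and 3 instead replay a "Blockanim" roll, apparently as blocked-drawer feedback.
; Closet01DrawerSmall is matched by two branches, so two timelines drive it at once.
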(event `self.Interact`
  (params (ForDoor :type Boolean) (ForLock :type Boolean) (Name :type String))
  (bind _closet_01_drawer_long (`self.closet_01_drawer_long`))
  (bind _closet_01_drawer_long1 (`self.closet_01_drawer_long1`))
  (bind _closet_01_drawer_small (`self.closet_01_drawer_small`))
  (bind _closet_01_drawer_small_2 (`self.closet_01_drawer_small`))
  (bind _closet_01_drawer_small1 (`self.closet_01_drawer_small1`))
  (bind _closet_01_drawer_small2 (`self.closet_01_drawer_small2`))
  (bind _closet_01_drawer_small3 (`self.closet_01_drawer_small3`))
  (bind (_relativelocation_x _relativelocation_y _relativelocation_z) (`KismetMathLibrary.BreakVector` (`SceneComponent.RelativeLocation` _closet_01_drawer_long1)))
  (bind (_relativelocation_x_2 _relativelocation_y_2 _relativelocation_z_2) (`KismetMathLibrary.BreakVector` (`SceneComponent.RelativeLocation` _closet_01_drawer_small)))
  (bind (_relativelocation_x_3 _relativelocation_y_3 _relativelocation_z_3) (`KismetMathLibrary.BreakVector` (`SceneComponent.RelativeLocation` _closet_01_drawer_small_2)))
  (bind (_relativelocation_x_4 _relativelocation_y_4 _relativelocation_z_4) (`KismetMathLibrary.BreakVector` (`SceneComponent.RelativeLocation` _closet_01_drawer_small1)))
  (bind (_relativelocation_x_5 _relativelocation_y_5 _relativelocation_z_5) (`KismetMathLibrary.BreakVector` (`SceneComponent.RelativeLocation` _closet_01_drawer_long)))
  (`|ExecutionSequence`
    (:`then_0`
      (if (`KismetStringLibrary.EqualEqual_StrStr` Name (`KismetSystemLibrary.GetObjectName` _closet_01_drawer_long))
        (`/Engine/EditorBlueprintResources/StandardMacros.FlipFlop`
          (:`A`
            (bind (_direction _lerp) (`Timeline|Timeline_1` :!label _label)
              (:`Update`
                (`SceneComponent.K2_SetRelativeLocation` _closet_01_drawer_long (`KismetMathLibrary.MakeVector` (`KismetMathLibrary.Lerp` (`self.BeginLocationX`) (`self.OpenAngle`) _lerp) _relativelocation_y_5 _relativelocation_z_5) false false))))
          (:`B`
            (goto _label :!via `Reverse`)))))
    (:`then_1`
      (if (`KismetStringLibrary.EqualEqual_StrStr` Name (`KismetSystemLibrary.GetObjectName` _closet_01_drawer_long1))
        (`/Engine/EditorBlueprintResources/StandardMacros.FlipFlop`
          (:`A`
            (bind (_direction_2 _lerp_2) (`Timeline|Timeline` :!label _label_2)
              (:`Update`
                (`SceneComponent.K2_SetRelativeLocation` _closet_01_drawer_long1 (`KismetMathLibrary.MakeVector` (`KismetMathLibrary.Lerp` (`self.BeginLocationX`) (`self.OpenAngle`) _lerp_2) _relativelocation_y _relativelocation_z) false false))))
          (:`B`
            (goto _label_2 :!via `Reverse`)))))
    (:`then_2`
      (if (`KismetStringLibrary.EqualEqual_StrStr` Name (`KismetSystemLibrary.GetObjectName` _closet_01_drawer_small))
        (`/Engine/EditorBlueprintResources/StandardMacros.FlipFlop`
          (:`A`
            (bind (_direction_3 _lerp_3) (`Timeline|Timeline_0` :!label _label_3)
              (:`Update`
                (`SceneComponent.K2_SetRelativeLocation` _closet_01_drawer_small (`KismetMathLibrary.MakeVector` (`KismetMathLibrary.Lerp` (`self.BeginLocationX`) (`self.OpenAngle`) _lerp_3) _relativelocation_y_2 _relativelocation_z_2) false false))))
          (:`B`
            (goto _label_3 :!via `Reverse`)))))
    (:`then_3`
      (if (`KismetStringLibrary.EqualEqual_StrStr` Name (`KismetSystemLibrary.GetObjectName` _closet_01_drawer_small_2))
        (`/Engine/EditorBlueprintResources/StandardMacros.FlipFlop`
          (:`A`
            (bind (_direction_4 _lerp_4) (`Timeline|Timeline_2` :!label _label_4)
              (:`Update`
                (`SceneComponent.K2_SetRelativeLocation` _closet_01_drawer_small_2 (`KismetMathLibrary.MakeVector` (`KismetMathLibrary.Lerp` (`self.BeginLocationX`) (`self.OpenAngle`) _lerp_4) _relativelocation_y_3 _relativelocation_z_3) false false))))
          (:`B`
            (goto _label_4 :!via `Reverse`)))))
    (:`then_4`
      (if (`KismetStringLibrary.EqualEqual_StrStr` Name (`KismetSystemLibrary.GetObjectName` _closet_01_drawer_small1))
        (`/Engine/EditorBlueprintResources/StandardMacros.FlipFlop`
          (:`A`
            (bind (_direction_5 _lerp_5) (`Timeline|Timeline_3` :!label _label_5)
              (:`Update`
                (`SceneComponent.K2_SetRelativeLocation` _closet_01_drawer_small1 (`KismetMathLibrary.MakeVector` (`KismetMathLibrary.Lerp` (`self.BeginLocationX`) (`self.OpenAngle`) _lerp_5) _relativelocation_y_4 _relativelocation_z_4) false false))))
          (:`B`
            (goto _label_5 :!via `Reverse`)))))
    (:`then_5`
      (if (`KismetStringLibrary.EqualEqual_StrStr` Name (`KismetSystemLibrary.GetObjectName` _closet_01_drawer_small2))
        (bind (_direction_6 _blockanim) (`Timeline|Timeline_block` :!via `PlayFromStart`)
          (:`Update`
            (`SceneComponent.K2_SetRelativeRotation` _closet_01_drawer_small2 (`KismetMathLibrary.MakeRotator` (.x _blockanim)) false false)))))
    (:`then_6`
      (if (`KismetStringLibrary.EqualEqual_StrStr` Name (`KismetSystemLibrary.GetObjectName` _closet_01_drawer_small3))
        (bind (_direction_7 _blockanim_2) (`Timeline|Timeline_4` :!via `PlayFromStart`)
          (:`Update`
            (`SceneComponent.K2_SetRelativeRotation` _closet_01_drawer_small3 (`KismetMathLibrary.MakeRotator` (.x _blockanim_2)) false false)))))))

(fn `UserConstructionScript`)