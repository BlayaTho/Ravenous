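; Inspectable pot object, built on a parent inspection Blueprint, with two interactive parts that move when the player interacts with them.
; Tick shows the matching prompt widget while a part is touched and hides both when none is.
; IA_Interact fires a once-only Timeline for the touched part, chosen by PartName: one shifts and tilts, the other slides down.
; Endfonction reverses both Timelines to return the parts, without resetting the DoOnce gates.
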(event `self.ReceiveBeginPlay`
  ;[0.224 0.224 0.224] Begin Play
  (`parent.ReceiveBeginPlay`)
  (bind _asw_interaction_inspection (cast `/Game/Ravenous/UI/Widgets/W_InteractionInspection` (`WidgetComponent.GetUserWidgetObject` (`self.Widget`))))
  (set `self.W_Widget` _asw_interaction_inspection)
  (bind _asw_interaction_inspection_2 (cast `/Game/Ravenous/UI/Widgets/W_InteractionInspection` (`WidgetComponent.GetUserWidgetObject` (`self.Widget1`))))
  (set `self.W_Widget2` _asw_interaction_inspection_2))

(event `EnhancedInput|/Game/Ravenous/Input/Actions/Player/IA_Interact`
  (params (ActionValue :type Boolean) (ElapsedSeconds :type "Float (double-precision)") (TriggeredSeconds :type "Float (double-precision)") (InputAction :type "InputAction Object Reference" :default "/Game/Ravenous/Input/Actions/Player/IA_Interact.IA_Interact"))
  (bind _partname (`self.PartName`))
  (:`Started`
    (if (`self.TouchInteractebalePart?`)
      (`|ExecutionSequence`
        (:`then_0`
          (if (`KismetStringLibrary.EqualEqual_StrStr` _partname "Interaction")
            (`/Engine/EditorBlueprintResources/StandardMacros.DoOnce` false
              (:`Completed`
                (bind (_direction _lerp) (`Timeline|Timeline` :!via `PlayFromStart` :!label _label)
                  (:`Update`
                    (`SceneComponent.K2_SetRelativeLocationAndRotation` (`self.Interaction`) (`KismetMathLibrary.MakeVector` (`KismetMathLibrary.Lerp` 0.0 10.0 _lerp) 0.0 (`KismetMathLibrary.Lerp` 10.0 17.8 _lerp)) (`KismetMathLibrary.MakeRotator` 0.0 (`KismetMathLibrary.Lerp` 0.0 -50.0 _lerp)) false false)))))))
        (:`then_1`
          (if (`KismetStringLibrary.EqualEqual_StrStr` _partname "Interaction1")
            (`/Engine/EditorBlueprintResources/StandardMacros.DoOnce` false
              (:`Completed`
                (bind (_direction_2 _lerp_2) (`Timeline|Timeline_0` :!via `PlayFromStart` :!label _label_2)
                  (:`Update`
                    (`SceneComponent.K2_SetRelativeLocationAndRotation` :`self` (`self.Interaction1`) :`NewLocation` (`KismetMathLibrary.MakeVector` 0.0 0.0 (`KismetMathLibrary.Lerp` -10.0 -20.0 _lerp_2)))))))))))))

(event `self.ReceiveTick`
  (params (DeltaSeconds :type "Float (single-precision)"))
  (bind _partname (`self.PartName`))
  (if (`self.TouchInteractebalePart?`)
    (`|ExecutionSequence`
      (:`then_0`
        (if (`KismetStringLibrary.EqualEqual_StrStr` _partname "Interaction")
          (`SceneComponent.SetHiddenInGame` (`self.Widget`) false false)))
      (:`then_1`
        (if (`KismetStringLibrary.EqualEqual_StrStr` _partname "Interaction1")
          (`SceneComponent.SetHiddenInGame` (`self.Widget1`) false false))))
    (else
      (`SceneComponent.SetHiddenInGame` (`self.Widget`) true false)
      (`SceneComponent.SetHiddenInGame` (`self.Widget1`) true false))))

(event `EnhancedInput|/Game/Ravenous/Input/Actions/Player/IA_InteractInspection`
  (params (ActionValue :type Boolean) (ElapsedSeconds :type "Float (double-precision)") (TriggeredSeconds :type "Float (double-precision)") (InputAction :type "InputAction Object Reference" :default "/Game/Ravenous/Input/Actions/Player/IA_InteractInspection.IA_InteractInspection")))

(event `self.endfonction`
  (`|ExecutionSequence`
    (:`then_0`
      (goto _label :!via `Reverse`))
    (:`then_1`
      (goto _label_2 :!via `Reverse`))))

(fn `UserConstructionScript`
  (`parent.UserConstructionScript`))