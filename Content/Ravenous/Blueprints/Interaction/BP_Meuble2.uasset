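; BP_Meuble2 is an interactable piece of furniture with four sliding drawers and two rotating parts that the player can open and close.
; Its Interact event compares the received name to each component's object name to pick the part to move.
; Each part has its own FlipFlop and Timeline, which plays or reverses on alternate interactions.
; Timelines lerp drawer X location toward OpenAngleL, or pitch toward OpenAngleR for the rotating parts.
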(event `self.Interact`
  (params (ForDoor :type Boolean) (ForLock :type Boolean) (Name :type String))
  (bind _commode_drawer3 (`self.commode_drawer3`))
  (bind _commode_drawer4 (`self.commode_drawer4`))
  (bind _commode_drawer_01 (`self.commode_drawer_01`))
  (bind _commode_drawer1 (`self.commode_drawer1`))
  (bind _commode_drawer_02 (`self.commode_drawer_02`))
  (bind _commode_drawer2 (`self.commode_drawer2`))
  (bind (_relativelocation_x _relativelocation_y _relativelocation_z) (`KismetMathLibrary.BreakVector` (`SceneComponent.RelativeLocation` _commode_drawer2)))
  (bind (_relativelocation_x_2 _relativelocation_y_2 _relativelocation_z_2) (`KismetMathLibrary.BreakVector` (`SceneComponent.RelativeLocation` _commode_drawer3)))
  (bind (_relativelocation_x_3 _relativelocation_y_3 _relativelocation_z_3) (`KismetMathLibrary.BreakVector` (`SceneComponent.RelativeLocation` _commode_drawer4)))
  (bind (_relativelocation_x_4 _relativelocation_y_4 _relativelocation_z_4) (`KismetMathLibrary.BreakVector` (`SceneComponent.RelativeLocation` _commode_drawer1)))
  (`|ExecutionSequence`
    (:`then_0`
      (if (`KismetStringLibrary.EqualEqual_StrStr` Name (`KismetSystemLibrary.GetObjectName` _commode_drawer1))
        (`/Engine/EditorBlueprintResources/StandardMacros.FlipFlop`
          (:`A`
            (bind (_direction _lerp) (`Timeline|Timeline_1` :!label _label)
              (:`Update`
                (`SceneComponent.K2_SetRelativeLocation` _commode_drawer1 (`KismetMathLibrary.MakeVector` (`KismetMathLibrary.Lerp` (`self.BeginLocationX`) (`self.OpenAngleL`) _lerp) _relativelocation_y_4 _relativelocation_z_4) false false))))
          (:`B`
            (goto _label :!via `Reverse`)))))
    (:`then_1`
      (if (`KismetStringLibrary.EqualEqual_StrStr` Name (`KismetSystemLibrary.GetObjectName` _commode_drawer2))
        (`/Engine/EditorBlueprintResources/StandardMacros.FlipFlop`
          (:`A`
            (bind (_direction_2 _lerp_2) (`Timeline|Timeline` :!label _label_2)
              (:`Update`
                (`SceneComponent.K2_SetRelativeLocation` _commode_drawer2 (`KismetMathLibrary.MakeVector` (`KismetMathLibrary.Lerp` (`self.BeginLocationX`) (`self.OpenAngleL`) _lerp_2) _relativelocation_y _relativelocation_z) false false))))
          (:`B`
            (goto _label_2 :!via `Reverse`)))))
    (:`then_2`
      (if (`KismetStringLibrary.EqualEqual_StrStr` Name (`KismetSystemLibrary.GetObjectName` _commode_drawer3))
        (`/Engine/EditorBlueprintResources/StandardMacros.FlipFlop`
          (:`A`
            (bind (_direction_3 _lerp_3) (`Timeline|Timeline_0` :!label _label_3)
              (:`Update`
                (`SceneComponent.K2_SetRelativeLocation` _commode_drawer3 (`KismetMathLibrary.MakeVector` (`KismetMathLibrary.Lerp` (`self.BeginLocationX`) (`self.OpenAngleL`) _lerp_3) _relativelocation_y_2 _relativelocation_z_2) false false))))
          (:`B`
            (goto _label_3 :!via `Reverse`)))))
    (:`then_3`
      (if (`KismetStringLibrary.EqualEqual_StrStr` Name (`KismetSystemLibrary.GetObjectName` _commode_drawer4))
        (`/Engine/EditorBlueprintResources/StandardMacros.FlipFlop`
          (:`A`
            (bind (_direction_4 _lerp_4) (`Timeline|Timeline_2` :!label _label_4)
              (:`Update`
                (`SceneComponent.K2_SetRelativeLocation` _commode_drawer4 (`KismetMathLibrary.MakeVector` (`KismetMathLibrary.Lerp` (`self.BeginLocationX`) (`self.OpenAngleL`) _lerp_4) _relativelocation_y_3 _relativelocation_z_3) false false))))
          (:`B`
            (goto _label_4 :!via `Reverse`)))))
    (:`then_4`
      (if (`KismetStringLibrary.EqualEqual_StrStr` Name (`KismetSystemLibrary.GetObjectName` _commode_drawer_01))
        (`/Engine/EditorBlueprintResources/StandardMacros.FlipFlop`
          (:`A`
            (bind (_direction_5 _lerp_5) (`Timeline|Timeline_3` :!label _label_5)
              (:`Update`
                (`SceneComponent.K2_SetRelativeRotation` _commode_drawer_01 (`KismetMathLibrary.MakeRotator` 0.0 (`KismetMathLibrary.Lerp` 0.0 (`self.OpenAngleR`) _lerp_5)) false false))))
          (:`B`
            (goto _label_5 :!via `Reverse`)))))
    (:`then_5`
      (if (`KismetStringLibrary.EqualEqual_StrStr` Name (`KismetSystemLibrary.GetObjectName` _commode_drawer_02))
        (`/Engine/EditorBlueprintResources/StandardMacros.FlipFlop`
          (:`A`
            (bind (_direction_6 _lerp_6) (`Timeline|Timeline_4` :!label _label_6)
              (:`Update`
                (`SceneComponent.K2_SetRelativeRotation` _commode_drawer_02 (`KismetMathLibrary.MakeRotator` 0.0 (`KismetMathLibrary.Lerp` 0.0 (`self.OpenAngleR`) _lerp_6)) false false))))
          (:`B`
            (goto _label_6 :!via `Reverse`)))))))

(fn `UserConstructionScript`)