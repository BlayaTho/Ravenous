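; BP_KeyVictor is an interactable key pickup for a puzzle in Ravenous.
; On BeginPlay it caches the player's first-person character.
; Interacting sets the character's VictorKey flag, shows the key in the character's CaryItem child actor slot by assigning its own class, then destroys itself.
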(event `self.ReceiveBeginPlay`
  (bind _asbp_first_person_character (cast `/Game/Ravenous/Blueprints/Player/BP_FirstPersonCharacter` (`GameplayStatics.GetPlayerCharacter` 0)))
  (set `self.As BP First Person Character` _asbp_first_person_character))

(event `/Game/Ravenous/Blueprints/Interface/BPI_Interaction.Interact`
  (params (ForDoor :type Boolean) (ForLock :type Boolean) (Name :type String))
  (bind _as_bp_first_person_character (`self.As BP First Person Character`))
  (set `/Game/Ravenous/Blueprints/Player/BP_FirstPersonCharacter.VictorKey?` true _as_bp_first_person_character)
  (`ChildActorComponent.SetChildActorClass` (`/Game/Ravenous/Blueprints/Player/BP_FirstPersonCharacter.CaryItem` _as_bp_first_person_character) (`GameplayStatics.GetObjectClass` self))
  (`self.K2_DestroyActor`))

(fn `UserConstructionScript`)