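; Environmental sound Blueprint that plays ambient wood cracks and manages deep bass audio for a "way back" sequence.
; Construction gathers the children of Cracks, minus the first, and a self-repeating event plays RandomWoodCracks at one of them every 2–7 seconds.
; WayBackSoundManager swaps DeepBass for a fade track, then starts DeepBassWayBack after about 54 seconds unless Cinematiqueencours is set.
; Stopping it silences both way-back sounds and sets that flag.
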(event `self.ReceiveBeginPlay`
  (`self.PlaywoodCracks`))

(event `PlaywoodCracks`
  (`KismetSystemLibrary.Delay` (`KismetMathLibrary.RandomFloatInRange` 2.0 7.0))
  (`GameplayStatics.PlaySoundAtLocation` "/Game/Ravenous/Sound/Environnement/Woodcracks/RandomWoodCracks.RandomWoodCracks" (`SceneComponent.K2_GetComponentLocation` (`KismetArrayLibrary.Array_Random` (`self.Cracksarray`))) (struct) 1.0 1.0 0.0 "/Game/Ravenous/Sound/Environnement/Woodcracks/WoodCrackAtt.WoodCrackAtt" null null null)
  (`self.PlaywoodCracks`))

(event `WayBackSoundManager`
  (params (`Start?` :type Boolean))
  (bind _deepbasswayback (`self.DeepBassWayBack`))
  (if `Start?`
    (`AudioComponent.Play` (`self.DeepBassWayBackFade`) 0.0)
    (`AudioComponent.Stop` (`self.DeepBass`))
    (`KismetSystemLibrary.Delay` 53.684)
    (if (`self.cinematiqueencours`)
      (`AudioComponent.Stop` _deepbasswayback :!label _label)
      (`AudioComponent.Stop` (`self.DeepBassWayBackFade`))
      (set `self.cinematiqueencours` true)
      (else
        (`AudioComponent.Play` _deepbasswayback 0.0)))
    (else
      (goto _label))))

(fn `UserConstructionScript`
  (`KismetArrayLibrary.Array_Clear` (`self.Cracksarray`))
  (bind _output_get (set `self.Cracksarray` (`SceneComponent.GetChildrenComponents` (`self.Cracks`) false)))
  (`KismetArrayLibrary.Array_RemoveItem` _output_get (`|GetArrayItem` _output_get)))