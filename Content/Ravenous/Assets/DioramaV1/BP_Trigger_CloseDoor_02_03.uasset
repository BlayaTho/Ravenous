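; A trigger volume that changes the state of linked doors when the first-person player walks into it.
; On the first overlap by BP_FirstPersonCharacter, a DoOnce fires the door changes so they happen only once.
; It loops over four door reference lists to close and lock, close, unlock, or open each door.
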(event `self.CollisionComponent.OnComponentBeginOverlap`
  (params (OverlappedComponent :type "PrimitiveComponent Object Reference") (OtherActor :type "Actor Object Reference") (OtherComp :type "PrimitiveComponent Object Reference") (OtherBodyIndex :type Integer) (bFromSweep :type Boolean) (SweepResult :type "HitResult Structure (by ref)"))
  (cast `/Game/Ravenous/Core/Characters/Player/BP_FirstPersonCharacter` OtherActor)
  (`/Engine/EditorBlueprintResources/StandardMacros.DoOnce` false
    (:`Completed`
      (for _array_element (`self.DoorLockRefList`)
        (`/Game/Ravenous/Core/Interactables/BP_Door.Close&LockDoor` _array_element true))
      (for _array_element_2 (`self.DoorCloseRefList`)
        (`/Game/Ravenous/Core/Interactables/BP_Door.Close&LockDoor` _array_element_2 false))
      (for _array_element_3 (`self.DoorUnlockRefList`)
        (`/Game/Ravenous/Core/Interactables/BP_Door.UnlockDoor` _array_element_3))
      (for _array_element_4 (`self.DoorOpenRefList`)
        (`/Game/Ravenous/Core/Interactables/BP_Door.OpenDoor` _array_element_4 false)))))

(fn `UserConstructionScript`)