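; HidingDrawer_BP is a drawer prop with left and right doors that the player can open, apparently as a hiding spot.
; Its Interact event receives a component name and compares it to each door mesh to decide which door to swing.
; Each door has its own timeline that lerps its relative yaw outward to a right angle in opposite directions.
; Doors always play from the start, with no closing logic.
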(event `/Game/Ravenous/Core/Characters/Interface/BPI_Interaction.Interact`
  (params (ForDoor :type Boolean) (ForLock :type Boolean) (Name :type String))
  (`|ExecutionSequence`
    (:`then_0`
      (if (`KismetStringLibrary.EqualEqual_StrStr` Name (`KismetSystemLibrary.GetObjectName` (`self.TestHidingDrawer_Left_Door_MSH_StaticMeshComponent0`)))
        (bind (_direction _newtrack_0) (`Timeline|LeftDoorMovement` :!via `PlayFromStart`)
          (:`Update`
            (`SceneComponent.K2_SetRelativeRotation` (`self.TestHidingDrawer_Left_Door_MSH_StaticMeshComponent0`) (`KismetMathLibrary.MakeRotator` 0.0 0.0 (`KismetMathLibrary.Lerp` 0.0 90.0 _newtrack_0)) false false)))))
    (:`then_1`
      (if (`KismetStringLibrary.EqualEqual_StrStr` Name (`KismetSystemLibrary.GetObjectName` (`self.TestHidingDrawer_RightDoor_MSH_StaticMeshComponent0`)))
        (bind (_direction_2 _newtrack_0_2) (`Timeline|Timeline` :!via `PlayFromStart`)
          (:`Update`
            (`SceneComponent.K2_SetRelativeRotation` (`self.TestHidingDrawer_RightDoor_MSH_StaticMeshComponent0`) (`KismetMathLibrary.MakeRotator` 0.0 0.0 (`KismetMathLibrary.Lerp` 0.0 -90.0 _newtrack_0_2)) false false)))))))

(fn `UserConstructionScript`)