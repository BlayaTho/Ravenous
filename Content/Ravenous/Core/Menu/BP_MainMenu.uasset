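; Main menu actor that creates the W_MainMenu widget on BeginPlay, passes itself as owner, adds it to the viewport and shows the mouse cursor.
; Three OnOff events, for Play, Options and Quit, each use a FlipFlop to toggle that component's EmScale material parameter, switching its highlight on and off.
; A UI-only input mode call is present but never runs.
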(event `self.ReceiveBeginPlay`
  (bind _returnvalue (`|CreateWidget` "/Game/Ravenous/UI/Menu/W_MainMenu.W_MainMenu_C"))
  (bind _output_get (set `self.W_MainMenuRef` _returnvalue))
  (`/Game/Ravenous/UI/Menu/W_MainMenu.SetOwner` _output_get self)
  (`UserWidget.AddToViewport` _output_get 0)
  (set `PlayerController.bShowMouseCursor` true (`GameplayStatics.GetPlayerController` 0)))

(event `OnOff_Play`
  (bind _isa (`/Engine/EditorBlueprintResources/StandardMacros.FlipFlop`)
    (:`A`
      _)
    (:`B`
      _))
  (`MeshComponent.SetScalarParameterValueOnMaterials` (`self.Play`) "EmScale" (select `bool` _isa :`true` 10.0 :!type "Float (single-precision)")))

(event `OnOff_Options`
  (bind _isa (`/Engine/EditorBlueprintResources/StandardMacros.FlipFlop`)
    (:`A`
      _)
    (:`B`
      _))
  (`MeshComponent.SetScalarParameterValueOnMaterials` (`self.Options`) "EmScale" (select `bool` _isa :`true` 10.0 :!type "Float (single-precision)")))

(event `OnOff_Quit`
  (bind _isa (`/Engine/EditorBlueprintResources/StandardMacros.FlipFlop`)
    (:`A`
      _)
    (:`B`
      _))
  (`MeshComponent.SetScalarParameterValueOnMaterials` (`self.Quit`) "EmScale" (select `bool` _isa :`true` 10.0 :!type "Float (single-precision)")))

(fn `UserConstructionScript`)