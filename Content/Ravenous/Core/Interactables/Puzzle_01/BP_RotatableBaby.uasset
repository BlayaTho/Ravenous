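; BP_RotatableBaby is a puzzle interactable with a Key part that the player can pick up through the interact input.
; Interacting with the touched key hides it and shows a pickup screen; a later press through a gate dismisses it and hands a spawned BP_KeyBaby to the player.
; Endfonction resets the sequence, restoring the key if unclaimed.
; Tick shows the inspection widget only while an interactable part is touched.
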(event `self.ReceiveBeginPlay`
  ;[0.05208 0.05208 0.05208] Init Widget & Default Value
  (`parent.ReceiveBeginPlay`)
  (bind _asw_interaction_inspection (cast `/Game/Ravenous/UI/Widgets/W_InteractionInspection` (`WidgetComponent.GetUserWidgetObject` (`self.Widget`))))
  (set `self.W_InteractionKey` _asw_interaction_inspection)
  (set `self.InitialKeyLocation` (`SceneComponent.RelativeLocation` (`self.Key`))))

(event `EnhancedInput|/Game/Ravenous/Core/Characters/Player/Input/Actions/Player/IA_Interact`
  (params (ActionValue :type Boolean) (ElapsedSeconds :type "Float (double-precision)") (TriggeredSeconds :type "Float (double-precision)") (InputAction :type "InputAction Object Reference" :default "/Game/Ravenous/Core/Characters/Player/Input/Actions/Player/IA_Interact.IA_Interact"))
  ;[0.05208 0.05208 0.05208] Interaction With Key
  (:`Started`
    (`|ExecutionSequence`
      (:`then_0`
        (if (and (`self.TouchInteractebalePart?`) (`KismetStringLibrary.EqualEqual_StrStr` (`self.PartName`) "Key"))
          (`|ExecutionSequence`
            (:`then_0`
              (`/Engine/EditorBlueprintResources/StandardMacros.DoOnce` false :!label _label
                (:`Completed`
                  (`SceneComponent.SetVisibility` (`self.Key`) false true)
                  (`PrimitiveComponent.SetCollisionEnabled` (`self.Key`) "NoCollision")
                  ;;[1 1 1] PickUp Key Screen
                  (set `Widget.Visibility` "Collapsed" (`self.W_input`))
                  (`UserWidget.AddToViewport` (`self.W_PickUp`) 0)
                  (`KismetSystemLibrary.Delay` 0.05)
                  (set `self.bIsInWidget` true)
                  (goto _label_2 :!via `Open`))))
            (:`then_1`
              (`/Engine/EditorBlueprintResources/StandardMacros.Gate` true :!label _label_2
                (:`Exit`
                  (`/Engine/EditorBlueprintResources/StandardMacros.DoOnce` false
                    (:`Completed`
                      (set `self.bIsKeyPicked` true)
                      (`Widget.RemoveFromParent` (`self.W_PickUp`))
                      (set `Widget.Visibility` "Visible" (`self.W_input`))
                      (bind _returnvalue (`|SpawnActorFromClass` "/Game/Ravenous/Core/Interactables/Puzzle_01/BP_KeyBaby.BP_KeyBaby_C" (`KismetMathLibrary.MakeTransform` (0.0 0.0 0.0)) "Undefined" "MultiplyWithRoot" null null))
                      (`/Game/Ravenous/Core/Characters/Player/BP_FirstPersonCharacter.SetHandleItem` (`self.Player Ref`) _returnvalue)
                      (`KismetSystemLibrary.Delay` 0.1)
                      (set `self.bIsInWidget` false)))))))))
      (:`then_1`
        (goto _label_2)))))

(event `self.endfonction`
  ;[0.05208 0.05208 0.05208] Interaction With Key
  (`|ExecutionSequence`
    (:`then_0`
      (goto _label :!via `Reset`))
    (:`then_1`
      (if (not (`self.bIsKeyPicked`))
        (`SceneComponent.SetVisibility` (`self.Key`) true true)
        (`PrimitiveComponent.SetCollisionEnabled` (`self.Key`) "QueryOnly")))
    (:`then_2`
      (goto _label_2 :!via `Close`))))

(event `self.ReceiveTick`
  (params (DeltaSeconds :type "Float (single-precision)"))
  ;[0.05208 0.05208 0.05208] Set Widget Visibility
  (if (`self.TouchInteractebalePart?`)
    (`SceneComponent.SetHiddenInGame` (`self.Widget`) false false)
    (else
      (`SceneComponent.SetHiddenInGame` (`self.Widget`) true false))))

(fn `UserConstructionScript`
  (`parent.UserConstructionScript`))