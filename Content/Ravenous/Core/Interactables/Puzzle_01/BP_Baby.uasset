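; BP_Baby is an inspectable doll puzzle that hides Louis' bedroom key under its head.
; Its arm and head animation plays with audio on BeginPlay.
; Inspection input tilts the head open via Timeline, then picks up the key behind a gated pickup widget, replaces the player's held item and notifies the trigger manager of the nursery step.
; Tick shows head or key prompts according to the touched part and open state.
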(event `self.ReceiveBeginPlay`
  (`parent.ReceiveBeginPlay`)
  (`self.StartAnim`)
  (set `self.bCanUse` false)
  (set `self.DefaultHeadLocation` (`SceneComponent.RelativeLocation` (`self.Head`)))
  (set `self.DefaultRot` (`SceneComponent.RelativeRotation` (`self.Item`))))

(event `EnhancedInput|/Game/Ravenous/Core/Characters/Player/Input/Actions/Player/IA_InteractInspection`
  (params (ActionValue :type Boolean) (ElapsedSeconds :type "Float (double-precision)") (TriggeredSeconds :type "Float (double-precision)") (InputAction :type "InputAction Object Reference" :default "/Game/Ravenous/Core/Characters/Player/Input/Actions/Player/IA_InteractInspection.IA_InteractInspection"))
  (bind _player_ref (`self.Player Ref`))
  (bind _w_pickup (`self.W_PickUp`))
  (:`Started`
    ;[0.05208 0.05208 0.05208] Interaction With Head
    (`|ExecutionSequence`
      (:`then_0`
        (if (`self.TouchInteractebalePart?`)
          (`|ExecutionSequence`
            (:`then_0`
              (if (`KismetStringLibrary.EqualEqual_StrStr` (`self.PartName`) (`KismetSystemLibrary.GetObjectName` (`self.Head`)))
                (`/Engine/EditorBlueprintResources/StandardMacros.DoOnce` false
                  (:`Completed`
                    (`|ExecutionSequence`
                      (:`then_0`
                        (bind (_direction _lerp) (`Timeline|Timeline` :!via `PlayFromStart`)
                          (:`Update`
                            (`SceneComponent.K2_SetRelativeRotation` (`self.Head`) (`KismetMathLibrary.MakeRotator` 0.0 (`KismetMathLibrary.Lerp` -15.0 -50.0 _lerp)) false false))
                          (:`Finished`
                            (set `self.bIsHeadOpen` true)
                            (`PrimitiveComponent.SetCollisionEnabled` (`self.Head`) "NoCollision"))))
                      (:`then_1`
                        (`/Engine/EditorBlueprintResources/StandardMacros.DoOnce` false
                          (:`Completed`
                            (`GameplayStatics.PlaySoundAtLocation` "/Game/Ravenous/Sound/Doll/CrackDoll_Cue.CrackDoll_Cue" (`self.K2_GetActorLocation`) (struct) 1.0 1.0 0.0 null null null null)))))))))
            (:`then_1`
              (if (`self.bIsHeadOpen`)
                (if (`KismetStringLibrary.EqualEqual_StrStr` (`self.PartName`) (`KismetSystemLibrary.GetObjectName` (`self.LouisKey`)))
                  (`/Engine/EditorBlueprintResources/StandardMacros.DoOnce` false
                    (:`Completed`
                      ;[0.09166 0.4458 1] Completion Sound
                      (`GameplayStatics.PlaySoundAtLocation` "/Game/Ravenous/Sound/CompletionSound_Cue.CompletionSound_Cue" (`self.K2_GetActorLocation`) (struct) 1.0 1.0 0.0 null null null null)
                      (`SceneComponent.SetVisibility` (`self.LouisKey`) false true)
                      (`PrimitiveComponent.SetCollisionEnabled` (`self.LouisKey`) "NoCollision")
                      (set `Widget.Visibility` "Collapsed" (`self.W_input`))
                      (`/Game/Ravenous/UI/Widgets/W_PickUpItem.SetWidgetParameters` _w_pickup "/Game/Ravenous/UI/Widgets/CloseUp/LouisKeyPNG.LouisKeyPNG" "Louis' \nBedroom Key" (100.0 40.0))
                      (`UserWidget.AddToViewport` _w_pickup 0)
                      (`KismetSystemLibrary.Delay` 0.05)
                      (set `self.bIsInWidget` true)
                      (goto _label :!via `Open`)))))))))
      (:`then_1`
        (`/Engine/EditorBlueprintResources/StandardMacros.Gate` true :!label _label
          (:`Exit`
            (`/Engine/EditorBlueprintResources/StandardMacros.DoOnce` false
              (:`Completed`
                (set `self.bIsKeyPicked` true)
                (`Widget.RemoveFromParent` (`self.W_PickUp`))
                (set `Widget.Visibility` "Visible" (`self.W_input`))
                (bind _returnvalue (`|SpawnActorFromClass` "/Game/Ravenous/Core/Interactables/Bp_PickableItem.BP_PickableItem_C" (`KismetMathLibrary.MakeTransform` (0.0 0.0 0.0)) "Undefined" "MultiplyWithRoot" null null))
                (set `/Game/Ravenous/Core/Interactables/Bp_PickableItem.ItemType` "NewEnumerator4" _returnvalue)
                (`/Game/Ravenous/Core/Characters/Player/BP_FirstPersonCharacter.DestroyHeldItem` _player_ref)
                (`/Game/Ravenous/Core/Characters/Player/BP_FirstPersonCharacter.SetHandleItem` _player_ref _returnvalue)
                (`KismetSystemLibrary.DelayUntilNextTick`)
                (set `self.bIsInWidget` false)
                (`/Game/Ravenous/UI/Widgets/W_LouisText.DisplayText` (`/Game/Ravenous/Core/Characters/Player/BP_FirstPersonCharacter.W_LouisText` (`self.Player Ref`)) "05_LouisKey" 2.5 (struct :`R` 0.629016 :`G` 0.833333 :`B` 0.47309 :`A` 1.0))
                (`/Game/Ravenous/Core/Interactables/Trigger_Event/BP_TriggerMANAGER.NURSERY_Baby_Step` (`self.TriggerManagerRef`))
                (`AudioComponent.Stop` (`self.Audio`))
                (`self.SetActorEnableCollision` false)))))))))

(event `EnhancedInput|/Game/Ravenous/Core/Characters/Player/Input/Actions/Player/IA_LockView`
  (params (ActionValue :type Boolean) (ElapsedSeconds :type "Float (double-precision)") (TriggeredSeconds :type "Float (double-precision)") (InputAction :type "InputAction Object Reference" :default "/Game/Ravenous/Core/Characters/Player/Input/Actions/Player/IA_LockView.IA_LockView"))
  (:`Started`
    (goto _label)))

(event `self.ReceiveTick`
  (params (DeltaSeconds :type "Float (single-precision)"))
  ;[0.05208 0.05208 0.05208] Set Widget Visibility
  (if (`self.TouchInteractebalePart?`)
    (`|ExecutionSequence`
      (:`then_0`
        (if (and (`KismetStringLibrary.EqualEqual_StrStr` (`self.PartName`) (`KismetSystemLibrary.GetObjectName` (`self.Head`))) (not (`self.bIsHeadOpen`)))
          (`SceneComponent.SetHiddenInGame` (`self.WidgetHead`) false false)
          (else
            (`SceneComponent.SetHiddenInGame` (`self.WidgetHead`) true false))))
      (:`then_1`
        (if (and (`KismetStringLibrary.EqualEqual_StrStr` (`self.PartName`) (`KismetSystemLibrary.GetObjectName` (`self.LouisKey`))) (`self.bIsHeadOpen`))
          (`SceneComponent.SetHiddenInGame` (`self.WidgetKey`) false false)
          (else
            (`SceneComponent.SetHiddenInGame` (`self.WidgetKey`) true false)))))
    (else
      (`SceneComponent.SetHiddenInGame` (`self.WidgetHead`) true false)
      (`SceneComponent.SetHiddenInGame` (`self.WidgetKey`) true false))))

(event `StartAnim`
  ;[0.05208 0.05208 0.05208] Baby Anim (Arms + Head)
  (`AudioComponent.Play` (`self.Audio`) 0.0)
  (bind (_direction _armlerp _headlerp) (`Timeline|ArmMovement` :!via `PlayFromStart`)
    (:`Update`
      (`SceneComponent.K2_SetRelativeRotation` (`self.LeftArm`) (`KismetMathLibrary.MakeRotator` (`KismetMathLibrary.Lerp` -13.0 -70.0 _armlerp)) false false)
      (`SceneComponent.K2_SetRelativeRotation` (`self.RightArm`) (`KismetMathLibrary.MakeRotator` (`KismetMathLibrary.Lerp` -10.0 -77.0 _armlerp) 3.0) false false)
      ;;[1 1 1] HeadMovement
      (`SceneComponent.K2_SetRelativeRotation` (`self.Head`) (`KismetMathLibrary.MakeRotator` 0.0 (`KismetMathLibrary.Lerp` 0.0 -15.0 _headlerp)) false false))
    (:`Finished`
      (set `self.bCanUse` true))))

(fn `UserConstructionScript`
  (`parent.UserConstructionScript`))