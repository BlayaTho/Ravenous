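; BP_Cradle is an interactable cradle in Puzzle 01 that shows a line of Louis's text when the player interacts with it.
; The line displays only if CanDisplayText is set and the player holds no item or one of a different type than a specific enum value.
; It comes from a French or English string table chosen by the player's language flag.
; A DoOnce, reset after a short delay, prevents repeat spam.
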(event `/Game/Ravenous/Core/Characters/Interface/BPI_Interaction.Interact`
  (params (ForDoor :type Boolean) (ForLock :type Boolean) (Name :type String) (PlayerRef :type "/Game/Ravenous/Core/Characters/Player/BP_FirstPersonCharacter Object Reference"))
  (`/Engine/EditorBlueprintResources/StandardMacros.IsValid` PlayerRef
    (:`Is Valid`
      (`/Engine/EditorBlueprintResources/StandardMacros.IsValid` (`/Game/Ravenous/Core/Characters/Player/BP_FirstPersonCharacter.HeldItem` PlayerRef)
        (:`Is Valid`
          (if (not (`|EnumEquality` (`/Game/Ravenous/Core/Interactables/Bp_PickableItem.ItemType` (`/Game/Ravenous/Core/Characters/Player/BP_FirstPersonCharacter.HeldItem` PlayerRef)) "NewEnumerator6"))
            (if (`self.bCanDisplayText`) :!label _label
              (`/Engine/EditorBlueprintResources/StandardMacros.DoOnce` false :!label _label_2
                (:`Completed`
                  (`/Game/Ravenous/UI/Widgets/W_LouisText.DisplayText` (`/Game/Ravenous/Core/Characters/Player/BP_FirstPersonCharacter.W_LouisText` PlayerRef) (`KismetTextLibrary.TextFromStringTable` (select `bool` (`/Game/Ravenous/Core/Characters/Player/BP_FirstPersonCharacter.bIsInFrancais` PlayerRef) :`false` "/Game/Ravenous/Data/Texts/EN_en/ST_LouisText_EN.ST_LouisText_EN" :`true` "/Game/Ravenous/Data/Texts/FR_fr/ST_LouisText_FR.ST_LouisText_FR" :!type "Name") "03_LouisCradle") 1.75 (struct :`R` 0.629016 :`G` 0.833333 :`B` 0.47309 :`A` 1.0))
                  (`KismetSystemLibrary.Delay` 2.5)
                  (goto _label_2 :!via `Reset`))))))
        (:`Is Not Valid`
          (goto _label))))))

(fn `UserConstructionScript`)