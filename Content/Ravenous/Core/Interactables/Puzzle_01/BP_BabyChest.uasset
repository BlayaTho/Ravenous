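; BP_BabyChest is an interactable chest in Puzzle_01 whose lid toggles open and closed on Interact.
; A Timeline plays forward or reverses from its end based on IsOpen, lerping the Lid's relative pitch to swing it.
; A DoOnce gate ignores further interaction until the Timeline finishes.
; A closing sound plays at the chest's location once the lid has fully shut.
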(event `/Game/Ravenous/Core/Characters/Interface/BPI_Interaction.Interact`
  (params (ForDoor :type Boolean) (ForLock :type Boolean) (Name :type String) (PlayerRef :type "/Game/Ravenous/Core/Characters/Player/BP_FirstPersonCharacter Object Reference"))
  (`/Engine/EditorBlueprintResources/StandardMacros.DoOnce` false :!label _label
    (:`Completed`
      (if (`self.bIsOpen`)
        (bind _output_get (set `self.bIsOpen` false))
        (bind (_direction _openinglerp) (`Timeline|Timeline` :!via `ReverseFromEnd` :!label _label_2)
          (:`Update`
            (`SceneComponent.K2_SetRelativeRotation` (`self.Lid`) (`KismetMathLibrary.MakeRotator` 0.0 (`KismetMathLibrary.Lerp` 0.0 -75.0 _openinglerp)) false false))
          (:`Finished`
            (if _output_get
              (goto _label :!via `Reset`)
              (else
                (`GameplayStatics.PlaySoundAtLocation` "/Game/Ravenous/Sound/Drawer/ClosingCloset_Cue.ClosingCloset_Cue" (`self.K2_GetActorLocation`) (struct) 1.0 1.0 0.0 "/Game/Ravenous/Sound/Environnement/Woodcracks/LittleAtt.LittleAtt" null null null)
                (goto _label :!via `Reset`)))))
        (else
          (set `self.bIsOpen` true)
          (goto _label_2 :!via `PlayFromStart`))))))

(fn `UserConstructionScript`)