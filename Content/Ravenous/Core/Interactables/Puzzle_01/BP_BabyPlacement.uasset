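; Placement spot in the baby puzzle that accepts only the right baby pickable, swapping it for a spawned BP_Baby, while wrong ones shake their heads.
; Until solved, babies leaving the box can leave a NoneItem placeholder.
; If one exists on success, it is removed, remaining babies lock, and a timer flickers the light before a hint line and corridor spotlight change.
; A gated Tick turns a close-range widget toward the nearby player.
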(event `self.Box.OnComponentBeginOverlap`
  (params (OverlappedComponent :type "PrimitiveComponent Object Reference") (OtherActor :type "Actor Object Reference") (OtherComp :type "PrimitiveComponent Object Reference") (OtherBodyIndex :type Integer) (bFromSweep :type Boolean) (SweepResult :type "HitResult Structure (by ref)"))
  (bind _playerref (`self.PlayerRef`))
  (bind _asbp_pickable_item (cast `/Game/Ravenous/Core/Interactables/Bp_PickableItem` OtherActor))
  ;[0.05208 0.05208 0.05208] Check if it was the right baby
  (if (`/Game/Ravenous/Core/Interactables/Bp_PickableItem.bIsRightBaby` _asbp_pickable_item)
    (`|ExecutionSequence`
      (:`then_0`
        (bind _returnvalue (`|SpawnActorFromClass` "/Game/Ravenous/Core/Interactables/Puzzle_01/BP_Baby.BP_Baby_C" (`KismetMathLibrary.MakeTransform` (- (`self.K2_GetActorLocation` _asbp_pickable_item) (0.0 0.0 4.25)) (struct :`Yaw` 190.0)) "Undefined" "MultiplyWithRoot" null null))
        (set `/Game/Ravenous/Core/Interactables/Puzzle_01/BP_Baby.TriggerManagerRef` (`self.TriggerManager_Ref`) _returnvalue)
        ;[0.05208 0.05208 0.05208] Kill the baby
        (`self.K2_DestroyActor` _asbp_pickable_item)
        (`/Engine/EditorBlueprintResources/StandardMacros.IsValid` (stale `self.Box.OnComponentEndOverlap` _returnvalue)
          (:`Is Valid`
            ;[0.05208 0.05208 0.05208] Destroy Useless NoneItem
            (`self.K2_DestroyActor` (stale `self.Box.OnComponentEndOverlap` _returnvalue))
            (`KismetSystemLibrary.DelayUntilNextTick`)
            (`KismetArrayLibrary.Array_RemoveItem` (`self.BabyArr`) (`/Game/Ravenous/Core/Characters/Player/BP_FirstPersonCharacter.HeldItem` _playerref))
            (`/Game/Ravenous/Core/Characters/Player/BP_FirstPersonCharacter.DestroyHeldItem` _playerref)
            (bind _returnvalue_2 (`KismetSystemLibrary.K2_SetTimerDelegate` (delegate `OnOffLight`) 0.15 true))
            ;[0.05208 0.05208 0.05208] Lock All Baby
            (for _array_element (`self.BabyArr`)
              (set `/Game/Ravenous/Core/Interactables/Bp_PickableItem.bCanBePicked` false _array_element)
              (set `/Game/Ravenous/Core/Interactables/Bp_PickableItem.bShowUi` false _array_element))
            (set `/Game/Ravenous/Core/Interactables/Puzzle_01/BP_Cradle.bCanDisplayText` false (`self.Cradle_Ref`)))))
      (:`then_1`
        (goto _label :!via `Close`)))
    (else
      (`/Game/Ravenous/Core/Interactables/Bp_PickableItem.HeadShake` _asbp_pickable_item))))

(event `OnOffLight`
  (bind _lightcomponent (`Light.LightComponent` (`self.Light_Ref`)))
  (`SceneComponent.SetVisibility` _lightcomponent (not (`SceneComponent.bVisible` _lightcomponent)) false)
  (if (== (`self.LightTwitchNbr`) 11)
    (`KismetSystemLibrary.K2_ClearAndInvalidateTimerHandle` (stale `self.Box.OnComponentBeginOverlap` _returnvalue_2))
    (`/Engine/EditorBlueprintResources/StandardMacros.DoOnce` false
      (:`Completed`
        (`self.StartDialogue`)
        (`LightComponent.SetIntensity` (`SpotLight.SpotLightComponent` (`self.Spotlight_corridor_01REF`)) 10.0)))
    (else
      (`/Engine/EditorBlueprintResources/StandardMacros.IncrementInt` (`self.LightTwitchNbr`)))))

(event `self.Box.OnComponentEndOverlap`
  (params (OverlappedComponent :type "PrimitiveComponent Object Reference") (OtherActor :type "Actor Object Reference") (OtherComp :type "PrimitiveComponent Object Reference") (OtherBodyIndex :type Integer))
  (`/Engine/EditorBlueprintResources/StandardMacros.Gate` false :!label _label
    (:`Exit`
      (bind _asbp_pickable_item (cast `/Game/Ravenous/Core/Interactables/Bp_PickableItem` OtherActor))
      ;[0.05208 0.05208 0.05208] Spawn NoneItem if Last Baby to leave is the one who enter last == No Item in hand
      (if (`|EnumEquality` (`/Game/Ravenous/Core/Interactables/Bp_PickableItem.ItemType` _asbp_pickable_item) "NewEnumerator6")
        (if (`KismetStringLibrary.EqualEqual_StrStr` (`KismetSystemLibrary.GetDisplayName` (stale `self.Box.OnComponentBeginOverlap` OtherActor)) (`KismetSystemLibrary.GetDisplayName` _asbp_pickable_item))
          (bind _returnvalue (`|SpawnActorFromClass` "/Game/Ravenous/Core/Interactables/Puzzle_02/BP_NoneItem.BP_NoneItem_C" (`KismetMathLibrary.MakeTransform` (+ (`self.K2_GetActorLocation`) (0.0 0.0 10.0)) (struct :`Yaw` -90.0) (0.8 0.8 0.8)) "Undefined" "MultiplyWithRoot" null null)))))))

(event `StartDialogue`
  (`KismetSystemLibrary.Delay` 0.8)
  (`/Game/Ravenous/UI/Widgets/W_LouisText.DisplayText` (`/Game/Ravenous/Core/Characters/Player/BP_FirstPersonCharacter.W_LouisText` (`self.PlayerRef`)) "The baby seems to be hiding something in his head." (`self.Duration`) (struct :`R` 0.629016 :`G` 0.833333 :`B` 0.47309 :`A` 1.0)))

(event `self.ReceiveTick`
  (params (DeltaSeconds :type "Float (single-precision)"))
  ;[0.1146 0.1146 0.1146] Close Range Widget
  (`/Engine/EditorBlueprintResources/StandardMacros.Gate` true :!label _label_2
    (:`Exit`
      (`SceneComponent.K2_SetRelativeRotation` (`self.W_CloseRange`) (`KismetMathLibrary.MakeRotator` (.roll (`KismetMathLibrary.FindLookAtRotation` (`self.K2_GetActorLocation`) (`self.K2_GetActorLocation` (`self.PlayerRef`)))) (.pitch (`KismetMathLibrary.FindLookAtRotation` (`self.K2_GetActorLocation`) (`self.K2_GetActorLocation` (`self.PlayerRef`)))) (- (.yaw (`KismetMathLibrary.FindLookAtRotation` (`self.K2_GetActorLocation`) (`self.K2_GetActorLocation` (`self.PlayerRef`)))) 10.0)) false false)
      (`SceneComponent.SetVisibility` (`self.W_CloseRange`) true false))))

(event `self.PlayerCollider.OnComponentBeginOverlap`
  (params (OverlappedComponent :type "PrimitiveComponent Object Reference") (OtherActor :type "Actor Object Reference") (OtherComp :type "PrimitiveComponent Object Reference") (OtherBodyIndex :type Integer) (bFromSweep :type Boolean) (SweepResult :type "HitResult Structure (by ref)"))
  ;[0.1146 0.1146 0.1146] Close Range Widget
  (`|ExecutionSequence`
    (:`then_0`
      (`/Engine/EditorBlueprintResources/StandardMacros.DoOnce` false
        (:`Completed`
          (bind _asbp_first_person_character (cast `/Game/Ravenous/Core/Characters/Player/BP_FirstPersonCharacter` OtherActor))
          (set `self.PlayerRef` _asbp_first_person_character))))
    (:`then_1`
      _))
  (set `self.PlayerLoc` SweepResult_Location)
  (goto _label_2 :!via `Open`))

(event `self.PlayerCollider.OnComponentEndOverlap`
  (params (OverlappedComponent :type "PrimitiveComponent Object Reference") (OtherActor :type "Actor Object Reference") (OtherComp :type "PrimitiveComponent Object Reference") (OtherBodyIndex :type Integer))
  ;[0.1146 0.1146 0.1146] Close Range Widget
  (`SceneComponent.SetVisibility` (`self.W_CloseRange`) false false)
  (goto _label_2 :!via `Close`))

(fn `UserConstructionScript`)