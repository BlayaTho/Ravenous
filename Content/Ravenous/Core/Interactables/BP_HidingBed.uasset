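; Hiding-spot bed that lets the player slide underneath from the left, right or front and climb back out on a second interact.
; Side trigger overlaps gate Interact, and the named side picks the entry/exit reference point; construction removes disabled sides.
; Timelines lerp the player's location while input and collision are off, then level the view and allow pitch-limited camera-only control.
; Exiting restores standing state and full control; the yaw clamp is unconnected.
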(event `/Game/Ravenous/Core/Characters/Interface/BPI_Interaction.Interact`
  (params (ForDoor :type Boolean) (ForLock :type Boolean) (Name :type String) (PlayerRef :type "/Game/Ravenous/Core/Characters/Player/BP_FirstPersonCharacter Object Reference"))
  (bind _player_ref (`self.Player Ref`))
  (bind _player_ref_2 (`self.Player Ref`))
  (bind _player_ref_3 (`self.Player Ref`))
  (bind (_returnvalue_roll _returnvalue_pitch _returnvalue_yaw) (`KismetMathLibrary.BreakRotator` (`Pawn.GetControlRotation` (`self.Player Ref`))))
  (`/Engine/EditorBlueprintResources/StandardMacros.Gate` true :!label _label
    (:`Exit`
      (if (`KismetStringLibrary.EqualEqual_StrStr` Name (`KismetSystemLibrary.GetObjectName` (`self.RightSide`)))
        (set `self.HittedComponentRefPoint` (`self.DownRightRefPoint`))
        ;[0.1146 0.1146 0.1146] Set Player State
        (set `self.Player Ref` PlayerRef :!label _label_2)
        (switch `/Game/Ravenous/Data/E_MobilityState` (`/Game/Ravenous/Core/Characters/Player/BP_FirstPersonCharacter.MobilityState` (`self.Player Ref`))
          (:`NewEnumerator3`
            (set `/Game/Ravenous/Core/Characters/Player/BP_FirstPersonCharacter.MobilityState` "NewEnumerator0" (`self.Player Ref`) :!label _label_3)
            (`|ExecutionSequence`
              (:`then_0`
                ;[0.1146 0.1146 0.1146] Disable Player Input
                (`/Game/Ravenous/Core/Characters/Player/BP_FirstPersonPlayerController.DisablePlayer` (`/Game/Ravenous/Core/Characters/Player/BP_FirstPersonCharacter.PlayerControllerRef` _player_ref) _player_ref))
              (:`then_1`
                (`self.SetActorEnableCollision` (`self.Player Ref`) false)
                ;[0.1146 0.1146 0.1146] Prone Timeline
                (bind (_direction _newtrack_0) (`Timeline|ProneTimeline` :!via `PlayFromStart`)
                  (:`Update`
                    (`self.K2_SetActorLocation` (`self.Player Ref`) (`KismetMathLibrary.VLerp` (`self.K2_GetActorLocation` (`self.Player Ref`)) (`SceneComponent.K2_GetComponentLocation` (`self.HittedComponentRefPoint`)) _newtrack_0) false false))
                  (:`Finished`
                    ;[0.1146 0.1146 0.1146] Make Player Look Straight
                    (`Timeline|Timeline_1` :!via `PlayFromStart`
                      (:`Update`
                        (`Controller.SetControlRotation` (`GameplayStatics.GetPlayerController` 0) (`KismetMathLibrary.RInterpTo` (`Pawn.GetControlRotation` (`self.Player Ref`)) (`KismetMathLibrary.MakeRotator` 0.0 0.0 _returnvalue_yaw) (`GameplayStatics.GetWorldDeltaSeconds`) 5.0)))
                      (:`Finished`
                        ;[0.1146 0.1146 0.1146] Set Hide View
                        (set `PlayerCameraManager.ViewPitchMin` -20.0 (`GameplayStatics.GetPlayerCameraManager` 0))
                        (set `PlayerCameraManager.ViewPitchMax` 15.0 (`GameplayStatics.GetPlayerCameraManager` 0))
                        (`/Game/Ravenous/Core/Characters/Player/BP_FirstPersonPlayerController.EnablePlayer` (`/Game/Ravenous/Core/Characters/Player/BP_FirstPersonCharacter.PlayerControllerRef` _player_ref_3) _player_ref_3 true))))))
              (:`then_2`
                ;[0.1146 0.1146 0.1146] Hide Under Bed timeline
                (bind (_direction_2 _newtrack_0_2) (`Timeline|HideUnderBed` :!via `PlayFromStart`)
                  (:`Update`
                    (`self.K2_SetActorLocation` (`self.Player Ref`) (`KismetMathLibrary.VLerp` (`self.K2_GetActorLocation` (`self.Player Ref`)) (`SceneComponent.K2_GetComponentLocation` (`self.UnderBedRefPoint`)) _newtrack_0_2) false false))))
              (:`then_3`
                (goto _label :!via `Toggle`))))
          (:`NewEnumerator1`
            (goto _label_3))
          (:`NewEnumerator2`
            (goto _label_3))
          (:`NewEnumerator0`
            (`|ExecutionSequence`
              (:`then_0`
                ;[0.1146 0.1146 0.1146] Go Out Of Bed
                (bind (_direction_3 _newtrack_0_3) (`Timeline|Timeline` :!via `PlayFromStart`)
                  (:`Update`
                    (`self.K2_SetActorLocation` (`self.Player Ref`) (`KismetMathLibrary.VLerp` (`self.K2_GetActorLocation` (`self.Player Ref`)) (`SceneComponent.K2_GetComponentLocation` (`self.HittedComponentRefPoint`)) _newtrack_0_3) false false))
                  (:`Finished`
                    ;[0.1146 0.1146 0.1146] Stand Up Timeline
                    (bind (_direction_4 _newtrack_0_4) (`Timeline|Timeline_0` :!via `PlayFromStart`)
                      (:`Update`
                        (`self.K2_SetActorLocation` (`self.Player Ref`) (`KismetMathLibrary.VLerp` (`self.K2_GetActorLocation` (`self.Player Ref`)) (+ (`SceneComponent.K2_GetComponentLocation` (`self.HittedComponentRefPoint`)) (0.0 0.0 101.5)) _newtrack_0_4) false false))
                      (:`Finished`
                        ;[0.1146 0.1146 0.1146] Re-Enable Player's Input
                        (`self.SetActorEnableCollision` (`self.Player Ref`) true)
                        (set `/Game/Ravenous/Core/Characters/Player/BP_FirstPersonCharacter.MobilityState` "NewEnumerator3" (`self.Player Ref`))
                        (`/Game/Ravenous/Core/Characters/Player/BP_FirstPersonPlayerController.Set Default View` (`/Game/Ravenous/Core/Characters/Player/BP_FirstPersonCharacter.PlayerControllerRef` (`self.Player Ref`)))
                        (`/Game/Ravenous/Core/Characters/Player/BP_FirstPersonPlayerController.EnablePlayer` (`/Game/Ravenous/Core/Characters/Player/BP_FirstPersonCharacter.PlayerControllerRef` _player_ref_2) _player_ref_2 false)))))))))
        (elif (`KismetStringLibrary.EqualEqual_StrStr` Name (`KismetSystemLibrary.GetObjectName` (`self.LeftSide`)))
          (set `self.HittedComponentRefPoint` (`self.DownLeftRefPoint`))
          (goto _label_2)
          (elif (`KismetStringLibrary.EqualEqual_StrStr` Name (`KismetSystemLibrary.GetObjectName` (`self.FrontSide`)))
            (set `self.HittedComponentRefPoint` (`self.DownFrontRefPoint`))
            (goto _label_2)))))))

(event `self.TriggerLeftSide.OnComponentBeginOverlap`
  (params (OverlappedComponent :type "PrimitiveComponent Object Reference") (OtherActor :type "Actor Object Reference") (OtherComp :type "PrimitiveComponent Object Reference") (OtherBodyIndex :type Integer) (bFromSweep :type Boolean) (SweepResult :type "HitResult Structure (by ref)"))
  (goto _label :!via `Open`))

(event `self.TriggerRightSide.OnComponentBeginOverlap`
  (params (OverlappedComponent :type "PrimitiveComponent Object Reference") (OtherActor :type "Actor Object Reference") (OtherComp :type "PrimitiveComponent Object Reference") (OtherBodyIndex :type Integer) (bFromSweep :type Boolean) (SweepResult :type "HitResult Structure (by ref)"))
  (goto _label :!via `Open`))

(event `self.TriggerFrontSide.OnComponentBeginOverlap`
  (params (OverlappedComponent :type "PrimitiveComponent Object Reference") (OtherActor :type "Actor Object Reference") (OtherComp :type "PrimitiveComponent Object Reference") (OtherBodyIndex :type Integer) (bFromSweep :type Boolean) (SweepResult :type "HitResult Structure (by ref)"))
  (goto _label :!via `Open`))

(event `self.TriggerLeftSide.OnComponentEndOverlap`
  (params (OverlappedComponent :type "PrimitiveComponent Object Reference") (OtherActor :type "Actor Object Reference") (OtherComp :type "PrimitiveComponent Object Reference") (OtherBodyIndex :type Integer))
  (goto _label :!via `Close`))

(event `self.TriggerRightSide.OnComponentEndOverlap`
  (params (OverlappedComponent :type "PrimitiveComponent Object Reference") (OtherActor :type "Actor Object Reference") (OtherComp :type "PrimitiveComponent Object Reference") (OtherBodyIndex :type Integer))
  (goto _label :!via `Close`))

(event `self.TriggerFrontSide.OnComponentEndOverlap`
  (params (OverlappedComponent :type "PrimitiveComponent Object Reference") (OtherActor :type "Actor Object Reference") (OtherComp :type "PrimitiveComponent Object Reference") (OtherBodyIndex :type Integer))
  (goto _label :!via `Close`))

(fn `UserConstructionScript`
  (bind (_returnvalue_roll _returnvalue_pitch _returnvalue_yaw) (`KismetMathLibrary.BreakRotator` (`self.K2_GetActorRotation`)))
  (`|ExecutionSequence`
    (:`then_0`
      (if (not (`self.bHasLeftSide`))
        (`ActorComponent.K2_DestroyComponent` (`self.TriggerLeftSide`))
        (`ActorComponent.K2_DestroyComponent` (`self.LeftSide`))
        (`ActorComponent.K2_DestroyComponent` (`self.DownLeftRefPoint`))))
    (:`then_1`
      (if (not (`self.bHasRightSide`))
        (`ActorComponent.K2_DestroyComponent` (`self.TriggerRightSide`))
        (`ActorComponent.K2_DestroyComponent` (`self.DownRightRefPoint`))
        (`ActorComponent.K2_DestroyComponent` (`self.RightSide`))))
    (:`then_2`
      (if (not (`self.bHasFrontSide`))
        (`ActorComponent.K2_DestroyComponent` (`self.TriggerFrontSide`))
        (`ActorComponent.K2_DestroyComponent` (`self.FrontSide`))
        (`ActorComponent.K2_DestroyComponent` (`self.DownFrontRefPoint`))))
    (:`then_3`
      (set `self.YawMedianValue` _returnvalue_yaw))))