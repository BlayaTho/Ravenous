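; Interactable hallway wall drawer whose door stays locked until the player supplies the missing handle.
; When locked, a held item of the required type is consumed to reveal the handle, unlock it and play sounds, while empty hands trigger a throttled, localized hint.
; Once unlocked, interactions alternately swing the door open and closed through a FlipFlop-driven timeline, gated by a DoOnce until the motion finishes.
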(event `/Game/Ravenous/Core/Characters/Interface/BPI_Interaction.Interact`
  (params (ForDoor :type Boolean) (ForLock :type Boolean) (Name :type String) (PlayerRef :type "/Game/Ravenous/Core/Characters/Player/BP_FirstPersonCharacter Object Reference"))
  (bind _helditem (`/Game/Ravenous/Core/Characters/Player/BP_FirstPersonCharacter.HeldItem` PlayerRef))
  (`/Engine/EditorBlueprintResources/StandardMacros.IsValid` PlayerRef
    (:`Is Valid`
      (if (`self.bIsLock`)
        (`/Engine/EditorBlueprintResources/StandardMacros.IsValid` _helditem
          (:`Is Valid`
            (if (`|EnumEquality` (`/Game/Ravenous/Core/Interactables/Bp_PickableItem.ItemType` _helditem) "NewEnumerator1")
              (`/Game/Ravenous/Core/Characters/Player/BP_FirstPersonCharacter.DestroyHeldItem` PlayerRef)
              (set `self.bIsLock` false)
              (`SceneComponent.SetVisibility` (`self.S_WallShelfHandle_`) true false)
              (`GameplayStatics.PlaySoundAtLocation` "/Game/Ravenous/Sound/Player/GrabItem/PlacingObject_Cue.PlacingObject_Cue" (`self.K2_GetActorLocation`) (struct) 1.0 1.0 0.0 null null null null)
              ;[0.09166 0.4458 1] Completion Sound
              (`GameplayStatics.PlaySoundAtLocation` "/Game/Ravenous/Sound/CompletionSound_Cue.CompletionSound_Cue" (`self.K2_GetActorLocation`) (struct) 1.0 1.0 0.0 null null null null)))
          (:`Is Not Valid`
            (`/Engine/EditorBlueprintResources/StandardMacros.DoOnce` false :!label _label
              (:`Completed`
                (`/Game/Ravenous/UI/Widgets/W_LouisText.DisplayText` (`/Game/Ravenous/Core/Characters/Player/BP_FirstPersonCharacter.W_LouisText` PlayerRef) (`KismetTextLibrary.TextFromStringTable` (select `/Game/Ravenous/Data/E_Language` (`/Game/Ravenous/Core/Characters/Player/BP_FirstPersonCharacter.Language` PlayerRef) :`NewEnumerator0` "/Game/Ravenous/Data/Texts/EN_en/ST_LouisText_EN.ST_LouisText_EN" :`NewEnumerator1` "/Game/Ravenous/Data/Texts/FR_fr/ST_LouisText_FR.ST_LouisText_FR" :`NewEnumerator2` "/Game/Ravenous/Data/Texts/KR_kr/ST_LouisText_KR.ST_LouisText_KR" :!type "Name") "13_WallDrawer") 2.5 (struct :`R` 0.629016 :`G` 0.833333 :`B` 0.47309 :`A` 1.0))
                (`KismetSystemLibrary.Delay` 2.5)
                (goto _label :!via `Reset`)))))
        (else
          (`/Engine/EditorBlueprintResources/StandardMacros.DoOnce` false :!label _label_2
            (:`Completed`
              (`/Engine/EditorBlueprintResources/StandardMacros.FlipFlop`
                (:`A`
                  (bind (_direction _rotationlerp) (`Timeline|Door Rotation` :!via `PlayFromStart` :!label _label_3)
                    (:`Update`
                      (`SceneComponent.K2_SetRelativeRotation` (`self.S_WallShelfDoorNoHandle_`) (`KismetMathLibrary.MakeRotator` 0.0 0.0 (`KismetMathLibrary.Lerp` 0.0 120.0 _rotationlerp)) false false))
                    (:`Finished`
                      (goto _label_2 :!via `Reset`))))
                (:`B`
                  (goto _label_3 :!via `ReverseFromEnd`))))))))))

(fn `UserConstructionScript`)