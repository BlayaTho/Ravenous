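; BP_BabyKey is an interactable baby key the player can pick up.
; Interact input on the touched key part hides it and shows a pickup widget through a DoOnce, while a Gate controls marking it picked and collapsing that widget.
; Endfonction resets the DoOnce, closes the Gate and restores the key if it is not picked.
; Tick shows the interaction widget only while an interactable part is touched.
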(event `self.ReceiveBeginPlay`
  ;[0.05208 0.05208 0.05208] Init Widget & Default Value
  (`parent.ReceiveBeginPlay`)
  (bind _asw_interaction_inspection (cast `/Game/Ravenous/UI/Widgets/W_InteractionInspection` (`WidgetComponent.GetUserWidgetObject` (`self.Widget`))))
  (set `self.W_InteractionKey` _asw_interaction_inspection)
  (set `self.InitialKeyLocation` (`SceneComponent.RelativeLocation` (`self.Key`)))
  (bind _returnvalue (`|CreateWidget` "/Game/Ravenous/UI/Widgets/W_PickUpItem.W_PickUpItem_C"))
  (bind _output_get (set `self.W_PickUp` _returnvalue))
  (`UserWidget.AddToViewport` _output_get 0))

(event `EnhancedInput|/Game/Ravenous/Core/Characters/Player/Input/Actions/Player/IA_Interact`
  (params (ActionValue :type Boolean) (ElapsedSeconds :type "Float (double-precision)") (TriggeredSeconds :type "Float (double-precision)") (InputAction :type "InputAction Object Reference" :default "/Game/Ravenous/Core/Characters/Player/Input/Actions/Player/IA_Interact.IA_Interact"))
  ;[0.05208 0.05208 0.05208] Interaction With Key
  (:`Started`
    (if (and (`self.TouchInteractebalePart?`) (`KismetStringLibrary.EqualEqual_StrStr` (`self.PartName`) "Key"))
      (`|ExecutionSequence`
        (:`then_0`
          (`/Engine/EditorBlueprintResources/StandardMacros.DoOnce` false :!label _label
            (:`Completed`
              (`SceneComponent.SetVisibility` (`self.Key`) false true)
              (`PrimitiveComponent.SetCollisionEnabled` (`self.Key`) "NoCollision")
              (set `Widget.Visibility` "SelfHitTestInvisible" (`self.W_PickUp`)))))
        (:`then_1`
          ;[1 1 1] PickUp Key Screen
          (`/Engine/EditorBlueprintResources/StandardMacros.Gate` true :!label _label_2
            (:`Exit`
              (set `self.bIsKeyPicked` true)
              (set `Widget.Visibility` "Collapsed" (`self.W_PickUp`))
              (`KismetSystemLibrary.PrintString` "Key PickedUP"))))))))

(event `self.endfonction`
  ;[0.05208 0.05208 0.05208] Interaction With Key
  (`|ExecutionSequence`
    (:`then_0`
      (goto _label :!via `Reset`))
    (:`then_1`
      (if (not (`self.bIsKeyPicked`))
        (`SceneComponent.SetVisibility` (`self.Key`) true true)
        (`PrimitiveComponent.SetCollisionEnabled` (`self.Key`) "QueryOnly")))
    (:`then_2`
      (goto _label_2 :!via `Close`))))

(event `self.ReceiveTick`
  (params (DeltaSeconds :type "Float (single-precision)"))
  ;[0.05208 0.05208 0.05208] Set Widget Visibility
  (if (`self.TouchInteractebalePart?`)
    (`SceneComponent.SetHiddenInGame` (`self.Widget`) false false)
    (else
      (`SceneComponent.SetHiddenInGame` (`self.Widget`) true false))))

(fn `UserConstructionScript`
  (`parent.UserConstructionScript`))