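; BP_Meuble is an interactable piece of furniture with three desk drawers that slide open and closed.
; The Interact event receives a name and compares it to each drawer component's object name to pick the drawer.
; Each drawer has its own FlipFlop and timeline, alternating play and reverse to lerp its relative X between shared BeginLocationX and OpenAngle values, which act as positions despite the latter's name.
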(event `/Game/Ravenous/Core/Characters/Interface/BPI_Interaction.Interact`
  (params (ForDoor :type Boolean) (ForLock :type Boolean) (Name :type String))
  (bind _desk_drawer1 (`self.desk_drawer1`))
  (bind _desk_drawer3 (`self.desk_drawer3`))
  (bind _desk_drawer2 (`self.desk_drawer2`))
  (bind (_relativelocation_x _relativelocation_y _relativelocation_z) (`KismetMathLibrary.BreakVector` (`SceneComponent.RelativeLocation` _desk_drawer3)))
  (bind (_relativelocation_x_2 _relativelocation_y_2 _relativelocation_z_2) (`KismetMathLibrary.BreakVector` (`SceneComponent.RelativeLocation` _desk_drawer2)))
  (bind (_relativelocation_x_3 _relativelocation_y_3 _relativelocation_z_3) (`KismetMathLibrary.BreakVector` (`SceneComponent.RelativeLocation` _desk_drawer1)))
  (`|ExecutionSequence`
    (:`then_0`
      (if (`KismetStringLibrary.EqualEqual_StrStr` Name (`KismetSystemLibrary.GetObjectName` _desk_drawer1))
        (`/Engine/EditorBlueprintResources/StandardMacros.FlipFlop`
          (:`A`
            (bind (_direction _lerp) (`Timeline|Timeline_1` :!label _label)
              (:`Update`
                (`SceneComponent.K2_SetRelativeLocation` _desk_drawer1 (`KismetMathLibrary.MakeVector` (`KismetMathLibrary.Lerp` (`self.BeginLocationX`) (`self.OpenAngle`) _lerp) _relativelocation_y_3 _relativelocation_z_3) false false))))
          (:`B`
            (goto _label :!via `Reverse`)))))
    (:`then_1`
      (if (`KismetStringLibrary.EqualEqual_StrStr` Name (`KismetSystemLibrary.GetObjectName` _desk_drawer2))
        (`/Engine/EditorBlueprintResources/StandardMacros.FlipFlop`
          (:`A`
            (bind (_direction_2 _lerp_2) (`Timeline|Timeline` :!label _label_2)
              (:`Update`
                (`SceneComponent.K2_SetRelativeLocation` _desk_drawer2 (`KismetMathLibrary.MakeVector` (`KismetMathLibrary.Lerp` (`self.BeginLocationX`) (`self.OpenAngle`) _lerp_2) _relativelocation_y_2 _relativelocation_z_2) false false))))
          (:`B`
            (goto _label_2 :!via `Reverse`)))))
    (:`then_2`
      (if (`KismetStringLibrary.EqualEqual_StrStr` Name (`KismetSystemLibrary.GetObjectName` _desk_drawer3))
        (`/Engine/EditorBlueprintResources/StandardMacros.FlipFlop`
          (:`A`
            (bind (_direction_3 _lerp_3) (`Timeline|Timeline_0` :!label _label_3)
              (:`Update`
                (`SceneComponent.K2_SetRelativeLocation` _desk_drawer3 (`KismetMathLibrary.MakeVector` (`KismetMathLibrary.Lerp` (`self.BeginLocationX`) (`self.OpenAngle`) _lerp_3) _relativelocation_y _relativelocation_z) false false))))
          (:`B`
            (goto _label_3 :!via `Reverse`)))))))

(fn `UserConstructionScript`)