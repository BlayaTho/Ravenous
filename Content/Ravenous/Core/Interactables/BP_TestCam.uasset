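; BP_TestCam is an interactable camera that lets the player look through it at a room, then return to their own view.
; Interact blends the view target to the actor over a cubic curve and hands input from player to camera.
; Lock View or Interact input reverses the switch, with an InMotion flag and short delay blocking retriggers during blends.
; Timer-driven view toggling and lock-view widget logic remain unwired.
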(event `self.ReceiveBeginPlay`
  ;[1 0 0 1 56] CACA DE THOMAS
)

(event `self.ReceiveTick`
  (params (DeltaSeconds :type "Float (single-precision)"))
  ;[1 0 0 1 56] CACA DE THOMAS
)

(event `ARA`
  ;[1 0 0 1 56] CACA DE THOMAS
  (`PlayerController.SetViewTargetWithBlend` (`GameplayStatics.GetPlayerController` 0) self 0.5 "VTBlend_Cubic" 0.0 false))

(event `STOP`
  ;[1 0 0 1 56] CACA DE THOMAS
  (`PlayerController.SetViewTargetWithBlend` (`GameplayStatics.GetPlayerController` 0) (`self.As BP First Person Character`) 0.5 "VTBlend_Cubic" 0.0 false))

(event `/Game/Ravenous/Core/Characters/Interface/BPI_Interaction.Interact`
  (params (ForDoor :type Boolean) (ForLock :type Boolean) (Name :type String) (PlayerRef :type "/Game/Ravenous/Core/Characters/Player/BP_FirstPersonCharacter Object Reference"))
  ;[0.05208 0.05208 0.05208] Look At Room
  (if (not (`self.bInMotion`))
    (set `self.Player Ref` PlayerRef)
    (`self.SetCameraView`)
    (`KismetSystemLibrary.Delay` 0.6)
    (set `self.bInMotion` false)))

(event `EnhancedInput|/Game/Ravenous/Core/Characters/Player/Input/Actions/Player/IA_LockView`
  (params (ActionValue :type Boolean) (ElapsedSeconds :type "Float (double-precision)") (TriggeredSeconds :type "Float (double-precision)") (InputAction :type "InputAction Object Reference" :default "/Game/Ravenous/Core/Characters/Player/Input/Actions/Player/IA_LockView.IA_LockView"))
  ;[0.05208 0.05208 0.05208] Leave
  (:`Started`
    (if (not (`self.bInMotion`)) :!label _label
      (`self.Leave`)
      (`KismetSystemLibrary.Delay` 0.6)
      (set `self.bInMotion` false))))

(event `EnhancedInput|/Game/Ravenous/Core/Characters/Player/Input/Actions/Player/IA_Interact`
  (params (ActionValue :type Boolean) (ElapsedSeconds :type "Float (double-precision)") (TriggeredSeconds :type "Float (double-precision)") (InputAction :type "InputAction Object Reference" :default "/Game/Ravenous/Core/Characters/Player/Input/Actions/Player/IA_Interact.IA_Interact"))
  ;[0.05208 0.05208 0.05208] Leave
  (:`Started`
    (goto _label)))

(fn `EnableInputs`
  (bind _player_ref (`self.Player Ref`))
  (bind _playercontrollerref (`/Game/Ravenous/Core/Characters/Player/BP_FirstPersonCharacter.PlayerControllerRef` _player_ref))
  (`self.DisableInput` (select `bool` (`self.bInInteraction`) :`false` self :`true` _player_ref :!type "Actor Object Reference") _playercontrollerref)
  (`self.EnableInput` (select `bool` (`self.bInInteraction`) :`false` (`self.Player Ref`) :`true` self :!type "Actor Object Reference") _playercontrollerref))

(fn `Leave`
  (`self.SetCameraView`)
  (`self.EnableInputs`))

(fn `SetCameraView`
  (bind _player_ref (`self.Player Ref`))
  (set `self.bInMotion` true)
  (`PlayerController.SetViewTargetWithBlend` (`/Game/Ravenous/Core/Characters/Player/BP_FirstPersonCharacter.PlayerControllerRef` _player_ref) (select `bool` (`self.bInInteraction`) :`false` self :`true` _player_ref :!type "Actor Object Reference") 0.5 "VTBlend_Cubic" 0.0 false)
  (set `self.bInInteraction` (not (`self.bInInteraction`)))
  (`self.EnableInputs`))

(fn `UserConstructionScript`)