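; Trigger volume that plays a Lucy dialogue line once when the first-person player enters, through its own W_LucyDialogue widget created at BeginPlay.
; It can also knock a door and show Lucy's light, while a timeline eases the player's view toward a focus door.
; It passes itself to the widget and exposes callbacks for slow door opening and light-off.
; IsActive gates collision at construction, and it can self-destroy on exit or door opening.
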(event `self.ReceiveBeginPlay`
  (bind _returnvalue (`|CreateWidget` "/Game/Ravenous/UI/Widgets/W_LucyDialogue.W_LucyDialogue_C"))
  (bind _output_get (set `self.W_LucyDialogue` _returnvalue))
  (`UserWidget.AddToViewport` _output_get 0))

(event `self.TriggerBox.OnComponentBeginOverlap`
  (params (OverlappedComponent :type "PrimitiveComponent Object Reference") (OtherActor :type "Actor Object Reference") (OtherComp :type "PrimitiveComponent Object Reference") (OtherBodyIndex :type Integer) (bFromSweep :type Boolean) (SweepResult :type "HitResult Structure (by ref)"))
  (bind _doorreftofocus (`self.DoorRefToFocus`))
  (bind _doortoknock (`self.DoorToKnock`))
  (bind _asbp_first_person_character (cast `/Game/Ravenous/Core/Characters/Player/BP_FirstPersonCharacter` OtherActor))
  (`/Engine/EditorBlueprintResources/StandardMacros.DoOnce` false
    (:`Completed`
      (`|ExecutionSequence`
        (:`then_0`
          (`/Game/Ravenous/UI/Widgets/W_LucyDialogue.StartDialogue` (`self.W_LucyDialogue`) (`self.TextToDisplay`) (`self.Duration`) self)
          (`/Engine/EditorBlueprintResources/StandardMacros.IsValid` _doortoknock
            (:`Is Valid`
              (`/Game/Ravenous/Core/Interactables/BP_Door.DoorKnock` _doortoknock))
            (:`Is Not Valid`
              _))
          (`/Engine/EditorBlueprintResources/StandardMacros.IsValid` (`self.LucyLight`)
            (:`Is Valid`
              (`SceneComponent.SetVisibility` (`RectLight.RectLightComponent` (`self.LucyLight`)) true false))))
        (:`then_1`
          (`Timeline|RotHead` :!via `PlayFromStart`
            (:`Update`
              (`Controller.SetControlRotation` (`/Game/Ravenous/Core/Characters/Player/BP_FirstPersonCharacter.PlayerControllerRef` _asbp_first_person_character) (`KismetMathLibrary.RInterpTo` (`Pawn.GetControlRotation` _asbp_first_person_character) (`KismetMathLibrary.FindLookAtRotation` (`SceneComponent.K2_GetComponentLocation` (`/Game/Ravenous/Core/Characters/Player/BP_FirstPersonCharacter.FirstPersonCamera` _asbp_first_person_character)) (- (`self.K2_GetActorLocation` _doorreftofocus) (* (`self.GetActorRightVector` _doorreftofocus) 95.0))) (`GameplayStatics.GetWorldDeltaSeconds`) 15.0)))))))))

(event `self.TriggerBox.OnComponentEndOverlap`
  (params (OverlappedComponent :type "PrimitiveComponent Object Reference") (OtherActor :type "Actor Object Reference") (OtherComp :type "PrimitiveComponent Object Reference") (OtherBodyIndex :type Integer))
  (cast `/Game/Ravenous/Core/Characters/Player/BP_FirstPersonCharacter` OtherActor)
  (if (`self.bShouldKHS`)
    (`self.K2_DestroyActor`)))

(fn `CallSlowOpening`
  (`/Engine/EditorBlueprintResources/StandardMacros.IsValid` (`self.DoorToOpen`)
    (:`Is Valid`
      (`/Game/Ravenous/Core/Interactables/BP_Door.SlowOpening` (`self.DoorToOpen`) 1.0)
      (`self.K2_DestroyActor`))))

(fn `CallTurnOffLight`
  (if (`self.bShouldTurnOffLight`)
    (`SceneComponent.SetVisibility` (`RectLight.RectLightComponent` (`self.LucyLight`)) false false)))

(fn `UserConstructionScript`
  (if (`self.bIsActive`)
    (`PrimitiveComponent.SetCollisionEnabled` (`self.TriggerBox`) "QueryOnly")
    (else
      (`PrimitiveComponent.SetCollisionEnabled` (`self.TriggerBox`) "NoCollision"))))