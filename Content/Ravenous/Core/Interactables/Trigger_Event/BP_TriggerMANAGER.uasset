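; Level trigger manager that scripts Ravenous's narrative beats, from the opening cinematic to the alpha's closing credits.
; ChangeTriggersState maps a step index to Lucy dialogue, flickering lights or salon monster and dollhouse sequences, while separate step functions and overlap events unlock later rooms, triggers and puzzles.
; During the monster encounter, Tick plays the salon sequence once the player faces the door handle, using a distance-scaled yaw tolerance and a pitch check.
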(event `self.ReceiveBeginPlay`
  (bind _playerref (`self.PlayerRef`))
  ;[0.05208 0.05208 0.05208] Init
  (bind _asbp_first_person_character (cast `/Game/Ravenous/Core/Characters/Player/BP_FirstPersonCharacter` (`GameplayStatics.GetPlayerCharacter` 0)))
  (set `self.PlayerRef` _asbp_first_person_character)
  (`self.SetActorEnableCollision` (`self.ShowDoll_Ref`) false)
  (`MovieSceneSequencePlayer.Play` (`LevelSequenceActor.SequencePlayer` (`self.LSRef`)))
  (`KismetSystemLibrary.DelayUntilNextTick`)
  (`/Game/Ravenous/Core/Characters/Player/BP_FirstPersonPlayerController.DisablePlayer` (`/Game/Ravenous/Core/Characters/Player/BP_FirstPersonCharacter.PlayerControllerRef` _playerref) _playerref))

(event `EndCinematiqueDébut`
  (`/Game/Ravenous/Core/Characters/Player/BP_FirstPersonCharacter.StartingThePlayer` (`self.PlayerRef`)))

(event `ChangeTriggersState`
  (params (NarrativeStep :type Integer))
  (bind _output_get (set `self.NarrativeStep` NarrativeStep))
  (switch `int` _output_get
    (:`0`
      (`self.CORRIDOR_FirstMetWithLucy_Step`))
    (:`1`
      ;[0.09166 0.4458 1] LightFlickering Sound
      (`GameplayStatics.PlaySound2D` "/Game/Ravenous/Sound/Light/LightFlickering_Cue.LightFlickering_Cue" 1.0 1.0 0.0 null null)
      ;[0.05208 0.05208 0.05208] Make Lights Flick
      (for _array_element (`self.SalonLightRef`)
        (bind _asbp_lamp_ (cast `/Game/Ravenous/Core/Environnement/BP_Lamp_` _array_element)
          (:`then`
            (`/Game/Ravenous/Core/Environnement/BP_Lamp_.LightFlickering` _asbp_lamp_ false true))
          (:`CastFailed`
            (bind _asbp_lamp_wall (cast `/Game/Ravenous/Core/Environnement/BP_Lamp_Wall` _array_element))
            (`/Game/Ravenous/Core/Environnement/BP_Lamp_Wall.LightFlickering` _asbp_lamp_wall false true)))))
    (:`2`
      (`self.SALON_PlayerMetMonster_Step`))
    (:`3`
      (`self.SALON_OpenDollHouse_Step`))
    (:`4`
      (`self.SALON_End_Step`))))

(event `self.ReceiveTick`
  (params (DeltaSeconds :type "Float (single-precision)"))
  (if (`self.bShouldCheckForPlayerRotation`)
    (if (`self.MONSTER_IsPlayerLookingInrightDirection`)
      (`MovieSceneSequencePlayer.Play` (`LevelSequenceActor.SequencePlayer` (`self.LSA_Salon`)))
      (set `self.bShouldCheckForPlayerRotation` false))))

(event `self.Trigger_Act1_0304.OnComponentEndOverlap`
  (params (OverlappedComponent :type "PrimitiveComponent Object Reference") (OtherActor :type "Actor Object Reference") (OtherComp :type "PrimitiveComponent Object Reference") (OtherBodyIndex :type Integer))
  ;[0.05208 0.05208 0.05208] Enable First Lucy's Dialogue
  (cast `/Game/Ravenous/Core/Characters/Player/BP_FirstPersonCharacter` OtherActor)
  (`/Engine/EditorBlueprintResources/StandardMacros.DoOnce` false
    (:`Completed`
      (`self.ChangeTriggersState` 0)
      (`ActorComponent.K2_DestroyComponent` (`self.Trigger_Act1_0304`)))))

(event `CORRIDOR_PostCadena`
  (`AudioComponent.Play` (`self.Audio_PreSalon`) 0.0))

(event `self.Trigger_EndAlphaV02.OnComponentBeginOverlap`
  (params (OverlappedComponent :type "PrimitiveComponent Object Reference") (OtherActor :type "Actor Object Reference") (OtherComp :type "PrimitiveComponent Object Reference") (OtherBodyIndex :type Integer) (bFromSweep :type Boolean) (SweepResult :type "HitResult Structure (by ref)"))
  ;[1 0 0] ALPHA
  (bind _asbp_first_person_character (cast `/Game/Ravenous/Core/Characters/Player/BP_FirstPersonCharacter` OtherActor))
  (`/Engine/EditorBlueprintResources/StandardMacros.DoOnce` false
    (:`Completed`
      (`/Game/Ravenous/Core/Characters/Player/BP_FirstPersonPlayerController.DisablePlayer` (`/Game/Ravenous/Core/Characters/Player/BP_FirstPersonCharacter.PlayerControllerRef` _asbp_first_person_character) _asbp_first_person_character)
      (`Timeline|LookAt`
        (:`Update`
          (`Controller.SetControlRotation` (`/Game/Ravenous/Core/Characters/Player/BP_FirstPersonCharacter.PlayerControllerRef` _asbp_first_person_character) (`KismetMathLibrary.RInterpTo` (`Pawn.GetControlRotation` _asbp_first_person_character) (`KismetMathLibrary.FindLookAtRotation` (`SceneComponent.K2_GetComponentLocation` (`/Game/Ravenous/Core/Characters/Player/BP_FirstPersonCharacter.FirstPersonCamera` _asbp_first_person_character)) (`KismetMathLibrary.MakeVector` 3400.0 -1285.0 100.0)) (`GameplayStatics.GetWorldDeltaSeconds`) 15.0)))
        (:`Finished`
          (bind _w_dot (`/Game/Ravenous/Core/Characters/Player/BP_FirstPersonCharacter.W_Dot` _asbp_first_person_character))
          (`UserWidget.PlayAnimationForward` _w_dot (`/Game/Ravenous/UI/Widgets/W_Dot.FadeDot` _w_dot) 2.5 false :!label _label)
          (bind _returnvalue (`|CreateWidget` "/Game/Ravenous/UI/Menu/W_Credits.W_Credits_C"))
          (`UserWidget.AddToViewport` _returnvalue 0)
          (`/Game/Ravenous/UI/Menu/W_Credits.StartCredits` _returnvalue true (`/Game/Ravenous/Core/Characters/Player/BP_FirstPersonCharacter.PlayerControllerRef` (`self.PlayerRef`)) null))))))

(event `EndAlpha`
  ;[1 0 0] ALPHA
  (goto _label))

(event `LouisBedroomStep`
  (bind _dialoguetrigger (`self.DialogueTrigger`))
  (bind _output (`|GetArrayItem` _dialoguetrigger (`KismetArrayLibrary.Array_LastIndex` _dialoguetrigger)))
  ;[0.1146 0.1146 0.1146] Enable Lucy's Dialogue after Doing Puzzle In LouisBedroom
  (`/Game/Ravenous/UI/Widgets/W_LouisText.DisplayText` (`/Game/Ravenous/Core/Characters/Player/BP_FirstPersonCharacter.W_LouisText` (`self.PlayerRef`)) "06_PuzzleLouisRoom" 1.5 (struct :`R` 0.85098 :`G` 1.0 :`B` 0.737255 :`A` 1.0))
  (`KismetSystemLibrary.Delay` 2.0)
  (`PrimitiveComponent.SetCollisionEnabled` (`/Game/Ravenous/Core/Interactables/Trigger_Event/BP_Trigger_LucyDialogue.TriggerBox` _output) "QueryOnly")
  (`SceneComponent.SetVisibility` (`RectLight.RectLightComponent` (`/Game/Ravenous/Core/Interactables/Trigger_Event/BP_Trigger_LucyDialogue.LucyLight` _output)) true false)
  (`PrimitiveComponent.SetCollisionEnabled` (`self.Trigger_Act2_03`) "QueryAndPhysics")
  (`/Game/Ravenous/Core/Interactables/Trigger_Event/BP_Trigger_MonsterOut.EnableTrigger` (`|GetArrayItem` (`self.TriggerMonsterArr`) 1)))

(event `self.Trigger_Act2_03.OnComponentBeginOverlap`
  (params (OverlappedComponent :type "PrimitiveComponent Object Reference") (OtherActor :type "Actor Object Reference") (OtherComp :type "PrimitiveComponent Object Reference") (OtherBodyIndex :type Integer) (bFromSweep :type Boolean) (SweepResult :type "HitResult Structure (by ref)"))
  (if (== OtherActor (`self.PlayerRef`))
    (`/Engine/EditorBlueprintResources/StandardMacros.DoOnce` false
      (:`Completed`
        ;[0.1146 0.1146 0.1146] Add Monster Sound At 15.5sec
        (`KismetSystemLibrary.Delay` 24.0)
        (`self.SetActorEnableCollision` (`self.OpenDoorTriggerRef`) true)
        (set `/Game/Ravenous/Core/Interactables/BP_Cadenas.bCanEnterCode` true (`self.Cadena_Ref`))))))

(fn `CORRIDOR_FirstMetWithLucy_Step`
  (`PrimitiveComponent.SetCollisionEnabled` (`/Game/Ravenous/Core/Interactables/Trigger_Event/BP_Trigger_LucyDialogue.TriggerBox` (`|GetArrayItem` (`self.DialogueTrigger`))) "QueryOnly")
  (`PrimitiveComponent.SetCollisionEnabled` (`/Game/Ravenous/Core/Interactables/Trigger_Event/BP_Trigger_LucyDialogue.TriggerBox` (`|GetArrayItem` (`self.DialogueTrigger`) 1)) "QueryOnly"))

(fn `MONSTER_IsPlayerLookingInrightDirection`
  (returns (ReturnValue :type Boolean))
  (bind _playerref (`self.PlayerRef`))
  (bind (_returnvalue_x _returnvalue_y) (`KismetMathLibrary.BreakVector` (`self.K2_GetActorLocation` (`self.PlayerRef`))))
  (bind (_returnvalue_x_2 _returnvalue_y_2) (`KismetMathLibrary.BreakVector` (`SceneComponent.K2_GetComponentLocation` (`/Game/Ravenous/Core/Interactables/BP_Door.S_DoorHandle_` (`self.DoorRef`)))))
  (bind (_returnvalue_roll _returnvalue_pitch) (`KismetMathLibrary.BreakRotator` (`SceneComponent.K2_GetComponentRotation` (`/Game/Ravenous/Core/Characters/Player/BP_FirstPersonCharacter.FirstPersonCamera` (`self.PlayerRef`)))))
  (bind (_returnvalue_roll_2 _returnvalue_pitch_2 _returnvalue_yaw) (`KismetMathLibrary.BreakRotator` (`KismetMathLibrary.FindRelativeLookAtRotation` (`KismetMathLibrary.MakeTransform` (`self.K2_GetActorLocation` _playerref) (`self.K2_GetActorRotation` _playerref)) (`SceneComponent.K2_GetComponentLocation` (`/Game/Ravenous/Core/Interactables/BP_Door.S_DoorHandle_` (`self.DoorRef`))))))
  (return (and (`KismetMathLibrary.NearlyEqual_FloatFloat` _returnvalue_yaw 0.0 (`KismetMathLibrary.MapRangeClamped` (`KismetMathLibrary.Vector_Distance` (`KismetMathLibrary.MakeVector` _returnvalue_x _returnvalue_y) (`KismetMathLibrary.MakeVector` _returnvalue_x_2 _returnvalue_y_2)) 0.0 800.0 2.25 40.0)) (`KismetMathLibrary.NearlyEqual_FloatFloat` _returnvalue_pitch 0.0 15.0))))

(fn `NURSERY_Baby_Step`
  (`/Game/Ravenous/Core/Interactables/Trigger_Event/BP_Trigger_MonsterOut.EnableTrigger` (`|GetArrayItem` (`self.TriggerMonsterArr`)))
  (`self.SetActorEnableCollision` (`self.CloseDoorPostBaby_Ref`) true)
  (`/Game/Ravenous/Core/Interactables/BP_Door.SlowOpening` (`self.Door_Ref`) 1.0))

(fn `Parents_Step`
  (bind _parentsdoorref (`self.ParentsDoorRef`))
  (`/Game/Ravenous/Core/Interactables/BP_Door.UnlockDoor` _parentsdoorref)
  (set `/Game/Ravenous/Core/Interactables/BP_Door.bHasSequencer` true _parentsdoorref))

(fn `SALON_End_Step`
  ;[0.05208 0.05208 0.05208] Unlock Door
  (`/Game/Ravenous/Core/Interactables/BP_Door.SlowOpening` (`self.DoorRef`) -1.0)
  ;[0.05208 0.05208 0.05208] Destroy Monster
  (`self.K2_DestroyActor` (`self.Monstre_Ref`)))

(fn `SALON_OpenDollHouse_Step`
  (`/Game/Ravenous/Core/Interactables/Puzzle_03/BP_TestMaison.OpenDollSalon` (`self.DollHouse_Ref`)))

(fn `SALON_PlayerMetMonster_Step`
  (bind _showdoll_ref (`self.ShowDoll_Ref`))
  (`self.SetActorHiddenInGame` (`self.Monstre_Ref`) false)
  (set `self.bShouldCheckForPlayerRotation` true)
  (`/Game/Ravenous/Core/Interactables/BP_Door.SlowOpening` (`self.DoorRef`) -1.0)
  (`self.SetActorHiddenInGame` _showdoll_ref false)
  (`self.SetActorEnableCollision` _showdoll_ref true)
  (`self.SetActorEnableCollision` (`self.CloseTrigger`) true))

(fn `UserConstructionScript`)