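; BP_Trigger_MonsterOut is a one-shot level trigger that plays a monster scare sequence and then removes the monster.
; Its collision stays off until EnableTrigger turns it on and unhides the referenced monster and light.
; A player overlap or ForcePlayAnim plays the referenced Level Sequence once through a DoOnce, then destroys the monster five seconds later.
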(event `self.ReceiveBeginPlay`
  (`self.SetActorEnableCollision` false))

(event `EnableTrigger`
  ;[0.1146 0.1146 0.1146] Enable Trigger
  (`self.SetActorEnableCollision` true)
  (`self.SetActorHiddenInGame` (`self.MonsterRef`) false)
  (`self.SetActorHiddenInGame` (`self.LightRef`) false))

(event `self.TriggerBox.OnComponentBeginOverlap`
  (params (OverlappedComponent :type "PrimitiveComponent Object Reference") (OtherActor :type "Actor Object Reference") (OtherComp :type "PrimitiveComponent Object Reference") (OtherBodyIndex :type Integer) (bFromSweep :type Boolean) (SweepResult :type "HitResult Structure (by ref)"))
  ;[0.1146 0.1146 0.1146] On Overlap With Player
  (cast `/Game/Ravenous/Core/Characters/Player/BP_FirstPersonCharacter` OtherActor)
  (`/Engine/EditorBlueprintResources/StandardMacros.DoOnce` false :!label _label
    (:`Completed`
      (`MovieSceneSequencePlayer.Play` (`LevelSequenceActor.SequencePlayer` (`self.LSRef`)))
      (`KismetSystemLibrary.Delay` 5.0)
      (`self.K2_DestroyActor` (`self.MonsterRef`)))))

(event `ForcePlayAnim`
  ;[0.1146 0.1146 0.1146] On Overlap With Player
  (goto _label))

(fn `UserConstructionScript`)