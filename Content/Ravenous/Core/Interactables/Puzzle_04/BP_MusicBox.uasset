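; Inspectable music box for Puzzle_04 that hides Lucy's key in a drawer.
; Using the required held item on it plays music and a Timeline that winds the key, slides the drawer open, then loops spinning the doll.
; Taking Lucy's key shows a pickup widget; a Gate waits for input before handing over the item and advancing the trigger manager.
; Tick toggles contextual prompts, while IsOn2ndMap auto-plays the animation with collision disabled.
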(event `self.ReceiveBeginPlay`
  (bind (_defaultdrawerloc_x _defaultdrawerloc_y _defaultdrawerloc_z) (`KismetMathLibrary.BreakVector` (`self.DefaultDrawerLoc`)))
  (`parent.ReceiveBeginPlay`)
  (set `self.DefaultRot` (`SceneComponent.RelativeRotation` (`self.Item`)))
  (set `self.DefaultDrawerLoc` (`SceneComponent.RelativeLocation` (`self.S_MusicBoxDrawer`)))
  (`PrimitiveComponent.SetCollisionEnabled` (`self.LucyKeyCollider`) "NoCollision")
  (set `self.UseScale` (0.35 0.35 0.35))
  (bind _returnvalue (`|CreateWidget` "/Game/Ravenous/UI/Widgets/W_PickUpItem.W_PickUpItem_C"))
  (set `self.W_PickUp` _returnvalue)
  (if (`self.bIsOn2ndMap`)
    (`self.SetActorEnableCollision` false)
    ;[1 1 1] Clef Rot
    (bind (_direction _rotlerp _loclerp) (`Timeline|Timeline` :!via `PlayFromStart` :!label _label)
      (:`Update`
        (if (not (`self.bIsDrawerOpen`))
          (`SceneComponent.K2_SetRelativeRotation` (`self.Key_0`) (`KismetMathLibrary.RLerp` (struct) (struct :`Roll` 260.0) _rotlerp) false false)
          (`SceneComponent.K2_SetRelativeLocation` (`self.S_MusicBoxDrawer`) (`KismetMathLibrary.VLerp` (`self.DefaultDrawerLoc`) (`KismetMathLibrary.MakeVector` _defaultdrawerloc_x -6.5 _defaultdrawerloc_z) _loclerp) false false)
          (`SceneComponent.K2_SetRelativeRotation` (`self.S_Doll`) (`KismetMathLibrary.MakeRotator` 0.0 0.0 (`KismetMathLibrary.Lerp` 0.0 180.0 _rotlerp)) false false)
          (else
            (`SceneComponent.K2_AddRelativeRotation` (`self.S_Doll`) (`KismetMathLibrary.MakeRotator` 0.0 0.0 (`KismetMathLibrary.RandomFloatInRange` 1.75 2.25)) false false))))
      (:`Finished`
        (`|ExecutionSequence`
          (:`then_0`
            (`/Engine/EditorBlueprintResources/StandardMacros.DoOnce` false
              (:`Completed`
                (set `self.bIsDrawerOpen` true)
                (`PrimitiveComponent.SetCollisionEnabled` (`self.LucyKeyCollider`) "QueryOnly"))))
          (:`then_1`
            (goto _label :!via `PlayFromStart`)))))))

(event `EnhancedInput|/Game/Ravenous/Core/Characters/Player/Input/Actions/Player/IA_InteractInspection`
  (params (ActionValue :type Boolean) (ElapsedSeconds :type "Float (double-precision)") (TriggeredSeconds :type "Float (double-precision)") (InputAction :type "InputAction Object Reference" :default "/Game/Ravenous/Core/Characters/Player/Input/Actions/Player/IA_InteractInspection.IA_InteractInspection"))
  (:`Started`
    (`|ExecutionSequence`
      (:`then_0`
        (`/Engine/EditorBlueprintResources/StandardMacros.IsValid` (`/Game/Ravenous/Core/Characters/Player/BP_FirstPersonCharacter.HeldItem` (`self.Player Ref`))
          (:`Is Valid`
            (if (and (and (`self.TouchInteractebalePart?`) (`KismetStringLibrary.EqualEqual_StrStr` (`self.PartName`) (`KismetSystemLibrary.GetObjectName` (`self.Collider`)))) (`|EnumEquality` (`/Game/Ravenous/Core/Interactables/Bp_PickableItem.ItemType` (`/Game/Ravenous/Core/Characters/Player/BP_FirstPersonCharacter.HeldItem` (`self.Player Ref`))) "NewEnumerator10"))
              (`/Engine/EditorBlueprintResources/StandardMacros.DoOnce` false
                (:`Completed`
                  (`/Game/Ravenous/Core/Characters/Player/BP_FirstPersonCharacter.DestroyHeldItem` (`self.Player Ref`))
                  (`SceneComponent.SetHiddenInGame` (`self.Key_0`) false false)
                  (`AudioComponent.Play` (`self.Music_Box_Cue`) 0.0)
                  (goto _label :!via `PlayFromStart`)))))
          (:`Is Not Valid`
            (if (and (and (`self.TouchInteractebalePart?`) (`KismetStringLibrary.EqualEqual_StrStr` (`self.PartName`) (`KismetSystemLibrary.GetObjectName` (`self.LucyKeyCollider`)))) (`self.bIsDrawerOpen`))
              (`/Engine/EditorBlueprintResources/StandardMacros.DoOnce` false
                (:`Completed`
                  (`ActorComponent.K2_DestroyComponent` (`self.MSH_LucyKey_0`))
                  (set `Widget.Visibility` "Collapsed" (`/Game/Ravenous/Core/Characters/Player/BP_FirstPersonCharacter.W_inputInteraction` (`self.Player Ref`)))
                  (`/Game/Ravenous/UI/Widgets/W_PickUpItem.SetWidgetParameters` (`self.W_PickUp`) "/Game/Ravenous/UI/Widgets/CloseUp/LucyKeyPNG.LucyKeyPNG" (select `bool` (`/Game/Ravenous/Core/Characters/Player/BP_FirstPersonCharacter.bIsInFrancais` (`self.Player Ref`)) :`false` "" :`true` "" :!type "Object Object Reference") (120.0 60.0))
                  (set `Widget.Visibility` "Visible" (`self.W_PickUp`))
                  (`UserWidget.AddToViewport` (`self.W_PickUp`) 0)
                  (`KismetSystemLibrary.Delay` 0.05)
                  (set `self.bIsInWidget` true)
                  (goto _label_2 :!via `Open`)))))))
      (:`then_1`
        (`/Engine/EditorBlueprintResources/StandardMacros.Gate` true :!label _label_2
          (:`Exit`
            (`/Engine/EditorBlueprintResources/StandardMacros.DoOnce` false
              (:`Completed`
                (set `self.bIsKeyPicked` true)
                (`Widget.RemoveFromParent` (`self.W_PickUp`))
                (set `Widget.Visibility` "Visible" (`/Game/Ravenous/Core/Characters/Player/BP_FirstPersonCharacter.W_inputInteraction` (`self.Player Ref`)))
                (`/Game/Ravenous/Core/Characters/Player/BP_FirstPersonCharacter.SetHandleItem` (`self.Player Ref`) (`self.LucyKeyRef`))
                (`/Game/Ravenous/Core/Interactables/Trigger_Event/BP_TriggerMANAGER.PARENTS_Step` (`self.TriggerManagerRef`))
                (`KismetSystemLibrary.DelayUntilNextTick`)
                (set `self.bIsInWidget` false)
                (set `self.bCanUse` false)
                (`self.SetActorEnableCollision` false)))))))))

(event `self.ReceiveTick`
  (params (DeltaSeconds :type "Float (single-precision)"))
  ;[0.05208 0.05208 0.05208] Widget Show / Dismiss
  (`|ExecutionSequence`
    (:`then_0`
      (if (and (and (`/Game/Ravenous/Core/Characters/Player/BP_FirstPersonCharacter.bInspecting?` (`self.Player Ref`)) (and (not (`self.bIsDrawerOpen`)) (`KismetStringLibrary.EqualEqual_StrStr` (`self.PartName`) (`KismetSystemLibrary.GetObjectName` (`self.Collider`))))) (`KismetSystemLibrary.IsValid` (`/Game/Ravenous/Core/Characters/Player/BP_FirstPersonCharacter.HeldItem` (`self.Player Ref`))))
        (`SceneComponent.SetHiddenInGame` (`self.WidgetKey`) false false)
        (else
          (`SceneComponent.SetHiddenInGame` (`self.WidgetKey`) true false))))
    (:`then_1`
      (if (and (and (`/Game/Ravenous/Core/Characters/Player/BP_FirstPersonCharacter.bInspecting?` (`self.Player Ref`)) (and (`self.bIsDrawerOpen`) (`KismetStringLibrary.EqualEqual_StrStr` (`self.PartName`) (`KismetSystemLibrary.GetObjectName` (`self.LucyKeyCollider`))))) (not (`self.bIsKeyPicked`)))
        (`SceneComponent.SetHiddenInGame` (`self.WidgetKey1`) false false)
        (else
          (`SceneComponent.SetHiddenInGame` (`self.WidgetKey1`) true false))))))

(event `StopMusicBox`
  (`AudioComponent.Stop` (`self.Music_Box_Cue`)))

(event `EnhancedInput|/Game/Ravenous/Core/Characters/Player/Input/Actions/Player/IA_LockView`
  (params (ActionValue :type Boolean) (ElapsedSeconds :type "Float (double-precision)") (TriggeredSeconds :type "Float (double-precision)") (InputAction :type "InputAction Object Reference" :default "/Game/Ravenous/Core/Characters/Player/Input/Actions/Player/IA_LockView.IA_LockView"))
  (:`Started`
    (goto _label_2)))

(fn `UserConstructionScript`
  (`parent.UserConstructionScript`))