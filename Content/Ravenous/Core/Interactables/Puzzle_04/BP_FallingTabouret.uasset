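; BP_FallingTabouret is a Puzzle 04 prop, a stool that tips over as a one-time scare.
; StartFall passes a DoOnce, waits briefly, then plays a timeline that lerps the mesh's relative rotation toward a 90-degree yaw.
; The Screamer04Cue audio component plays the fall slam sound as the timeline starts, while an older play-sound-at-location call is left disconnected.
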(event `StartFall`
  (`/Engine/EditorBlueprintResources/StandardMacros.DoOnce` false
    (:`Completed`
      (`KismetSystemLibrary.Delay` 0.35)
      (`|ExecutionSequence`
        (:`then_0`
          (bind (_direction _rotlerp) (`Timeline|TabouretFall` :!via `PlayFromStart`)
            (:`Update`
              (`SceneComponent.K2_SetRelativeRotation` (`self.MSH`) (`KismetMathLibrary.RLerp` (struct) (struct :`Pitch` 90.0) _rotlerp) false false))))
        (:`then_1`
          ;[0.09166 0.4458 1] FallSlam Sound
          (`AudioComponent.Play` (`self.Screamer_04_Cue`) 0.0))))))

(fn `UserConstructionScript`)