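; Hiding drawer interactable: interacting with either door while in range puts the player inside or lets them back out.
; Timelines swing the doors, turn the view and slide the player, with input disabled during each move.
; Inside, only camera look is enabled, yaw-clamped around the drawer's construction-time facing, and the player's MobilityState becomes Hiding.
; EnnemyGrabsPlayer only swings the doors open.
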(event `/Game/Ravenous/Core/Characters/Interface/BPI_Interaction.Interact`
  (params (ForDoor :type Boolean) (ForLock :type Boolean) (Name :type String) (PlayerRef :type "/Game/Ravenous/Core/Characters/Player/BP_FirstPersonCharacter Object Reference"))
  (bind _player_ref (`self.Player Ref`))
  (bind _player_ref_2 (`self.Player Ref`))
  (bind _player_ref_3 (`self.Player Ref`))
  (bind _player_ref_4 (`self.Player Ref`))
  (bind _player_ref_5 (`self.Player Ref`))
  (bind _player_ref_6 (`self.Player Ref`))
  (bind (_returnvalue_x _returnvalue_y _returnvalue_z) (`KismetMathLibrary.BreakVector` (`self.K2_GetActorLocation` _player_ref)))
  (bind (_returnvalue_x_2 _returnvalue_y_2) (`KismetMathLibrary.BreakVector` (`SceneComponent.K2_GetComponentLocation` (`self.OutDrawerPointRef`))))
  (bind (_returnvalue_x_3 _returnvalue_y_3) (`KismetMathLibrary.BreakVector` (`SceneComponent.K2_GetComponentLocation` (`self.OutDrawerPointRef`))))
  (bind (_returnvalue_x_4 _returnvalue_y_4 _returnvalue_z_2) (`KismetMathLibrary.BreakVector` (`self.K2_GetActorLocation` _player_ref_2)))
  (bind (_returnvalue_x_5 _returnvalue_y_5) (`KismetMathLibrary.BreakVector` (`SceneComponent.K2_GetComponentLocation` (`self.InsideRefPoint`))))
  (bind (_returnvalue_x_6 _returnvalue_y_6 _returnvalue_z_3) (`KismetMathLibrary.BreakVector` (`SceneComponent.K2_GetComponentLocation` (`/Game/Ravenous/Core/Characters/Player/BP_FirstPersonCharacter.FirstPersonCamera` (`self.Player Ref`)))))
  (bind (_returnvalue_x_7 _returnvalue_y_7 _returnvalue_z_4) (`KismetMathLibrary.BreakVector` (`SceneComponent.K2_GetComponentLocation` (`/Game/Ravenous/Core/Characters/Player/BP_FirstPersonCharacter.FirstPersonCamera` (`self.Player Ref`)))))
  (bind (_returnvalue_x_8 _returnvalue_y_8 _returnvalue_z_5) (`KismetMathLibrary.BreakVector` (`SceneComponent.K2_GetComponentLocation` (`/Game/Ravenous/Core/Characters/Player/BP_FirstPersonCharacter.FirstPersonCamera` (`self.Player Ref`)))))
  (`/Engine/EditorBlueprintResources/StandardMacros.Gate` true :!label _label
    (:`Exit`
      (set `self.Player Ref` PlayerRef)
      (if (or (`KismetStringLibrary.EqualEqual_StrStr` Name (`KismetSystemLibrary.GetObjectName` (`self.S_TestHidingDrawer_Left_Door`))) (`KismetStringLibrary.EqualEqual_StrStr` Name (`KismetSystemLibrary.GetObjectName` (`self.S_TestHidingDrawer_RightDoor`))))
        (switch `/Game/Ravenous/Data/E_MobilityState` (`/Game/Ravenous/Core/Characters/Player/BP_FirstPersonCharacter.MobilityState` (`self.Player Ref`))
          (:`NewEnumerator3`
            (`|ExecutionSequence` :!label _label_2
              (:`then_0`
                ;[0.05208 0.05208 0.05208] Disable Player's Input While Hiding Movement
                (`/Game/Ravenous/Core/Characters/Player/BP_FirstPersonPlayerController.DisablePlayer` (`/Game/Ravenous/Core/Characters/Player/BP_FirstPersonCharacter.PlayerControllerRef` _player_ref_3) _player_ref_3)
                ;[0.05208 0.05208 0.05208] Make Player Look Between Doors
                (`Timeline|Timeline_0` :!via `PlayFromStart`
                  (:`Update`
                    (`Controller.SetControlRotation` (`GameplayStatics.GetPlayerController` 0) (`KismetMathLibrary.RInterpTo` (`Pawn.GetControlRotation` (`self.Player Ref`)) (`KismetMathLibrary.FindLookAtRotation` (`KismetMathLibrary.MakeVector` _returnvalue_x_8 _returnvalue_y_8 _returnvalue_z_5) (`KismetMathLibrary.MakeVector` _returnvalue_x_5 _returnvalue_y_5 _returnvalue_z_5)) (`GameplayStatics.GetWorldDeltaSeconds`) 5.0)))))
              (:`then_1`
                (`PrimitiveComponent.SetCollisionEnabled` (`self.S_TestHidingDrawer_Left_Door`) "QueryOnly")
                (`PrimitiveComponent.SetCollisionEnabled` (`self.S_TestHidingDrawer_RightDoor`) "QueryOnly")
                ;[0.05208 0.05208 0.05208] Doors Movement
                (bind (_direction _newtrack_0) (`Timeline|DoorMovement` :!via `PlayFromStart` :!label _label_3)
                  (:`Update`
                    (`SceneComponent.K2_SetRelativeRotation` (`self.S_TestHidingDrawer_Left_Door`) (`KismetMathLibrary.MakeRotator` 0.0 0.0 (`KismetMathLibrary.Lerp` 0.0 80.0 _newtrack_0)) false false)
                    (`SceneComponent.K2_SetRelativeRotation` (`self.S_TestHidingDrawer_RightDoor`) (`KismetMathLibrary.MakeRotator` 0.0 0.0 (`KismetMathLibrary.Lerp` 0.0 -80.0 _newtrack_0)) false false))
                  (:`Finished`
                    (switch `ETimelineDirection` _direction
                      (:`Forward`
                        (`|ExecutionSequence`
                          (:`then_0`
                            ;[0.05208 0.05208 0.05208] Player In Locker
                            (bind (_direction_2 _playermovementvalue) (`Timeline|PlayerIn`)
                              (:`Update`
                                (bind _returnvalue (`KismetMathLibrary.TLerp` (`KismetMathLibrary.MakeTransform` (`self.K2_GetActorLocation` (`self.Player Ref`))) (`KismetMathLibrary.MakeTransform` (`SceneComponent.K2_GetComponentLocation` (`self.InsideRefPoint`))) _playermovementvalue))
                                (`self.K2_SetActorLocation` _player_ref_2 (`KismetMathLibrary.MakeVector` (.x (.location _returnvalue)) (.y (.location _returnvalue)) _returnvalue_z_2) false false))))
                          (:`then_1`
                            ;[0.05208 0.05208 0.05208] Make Player Look Outside Drawer
                            (`Timeline|LookAtRightDirection` :!via `PlayFromStart`
                              (:`Update`
                                (`Controller.SetControlRotation` (`GameplayStatics.GetPlayerController` 0) (`KismetMathLibrary.RInterpTo` (`Pawn.GetControlRotation` (`self.Player Ref`)) (`KismetMathLibrary.FindLookAtRotation` (`KismetMathLibrary.MakeVector` _returnvalue_x_6 _returnvalue_y_6 _returnvalue_z_3) (`KismetMathLibrary.MakeVector` _returnvalue_x_2 _returnvalue_y_2 _returnvalue_z_3)) (`GameplayStatics.GetWorldDeltaSeconds`) 3.5)))
                              (:`Finished`
                                ;[0.05208 0.05208 0.05208] Enable Look Input
                                (`/Game/Ravenous/Core/Characters/Player/BP_FirstPersonPlayerController.EnablePlayer` (`/Game/Ravenous/Core/Characters/Player/BP_FirstPersonCharacter.PlayerControllerRef` _player_ref_4) _player_ref_4 true)
                                (set `PlayerCameraManager.ViewPitchMin` -70.0 (`GameplayStatics.GetPlayerCameraManager` 0))
                                ;;[0.05208 0.05208 0.05208] Find Right Rotator To Lock View
                                (set `PlayerCameraManager.ViewYawMin` (- (`self.YawMedianValue`) 30.0) (`GameplayStatics.GetPlayerCameraManager` 0))
                                (set `PlayerCameraManager.ViewYawMax` (+ (`self.YawMedianValue`) 30.0) (`GameplayStatics.GetPlayerCameraManager` 0))
                                (set `/Game/Ravenous/Core/Characters/Player/BP_FirstPersonCharacter.MobilityState` "NewEnumerator0" (`self.Player Ref`))
                                (set `self.bIsPlayerInside` true)
                                (set `/Game/Ravenous/Core/Characters/Player/BP_FirstPersonCharacter.HideOutPointRef` (`SceneComponent.K2_GetComponentLocation` (`self.OutDrawerPointRef`)) (`self.Player Ref`)))))
                          (:`then_2`
                            (goto _label_3 :!via `ReverseFromEnd`))))))))))
          (:`NewEnumerator1`
            (goto _label_2))
          (:`NewEnumerator2`
            (goto _label_2))
          (:`NewEnumerator0`
            (`|ExecutionSequence`
              (:`then_0`
                ;[0.05208 0.05208 0.05208] Disable Player's Input While Hiding Movement
                (`/Game/Ravenous/Core/Characters/Player/BP_FirstPersonPlayerController.DisablePlayer` (`/Game/Ravenous/Core/Characters/Player/BP_FirstPersonCharacter.PlayerControllerRef` _player_ref_5) _player_ref_5)
                ;[0.05208 0.05208 0.05208] Doors Movement
                (bind (_direction_3 _newtrack_0_2) (`Timeline|DoorsMovement` :!via `PlayFromStart` :!label _label_4)
                  (:`Update`
                    (`SceneComponent.K2_SetRelativeRotation` (`self.S_TestHidingDrawer_Left_Door`) (`KismetMathLibrary.MakeRotator` 0.0 0.0 (`KismetMathLibrary.Lerp` 0.0 80.0 _newtrack_0_2)) false false)
                    (`SceneComponent.K2_SetRelativeRotation` (`self.S_TestHidingDrawer_RightDoor`) (`KismetMathLibrary.MakeRotator` 0.0 0.0 (`KismetMathLibrary.Lerp` 0.0 -80.0 _newtrack_0_2)) false false))))
              (:`then_1`
                ;[0.05208 0.05208 0.05208] Make Player Look Between Doors
                (`Timeline|Timeline` :!via `PlayFromStart`
                  (:`Update`
                    (`Controller.SetControlRotation` (`GameplayStatics.GetPlayerController` 0) (`KismetMathLibrary.RInterpTo` (`Pawn.GetControlRotation` (`self.Player Ref`)) (`KismetMathLibrary.FindLookAtRotation` (`KismetMathLibrary.MakeVector` _returnvalue_x_7 _returnvalue_y_7 _returnvalue_z_4) (`KismetMathLibrary.MakeVector` _returnvalue_x_3 _returnvalue_y_3 _returnvalue_z_4)) (`GameplayStatics.GetWorldDeltaSeconds`) 10.0)))
                  (:`Finished`
                    ;[0.05208 0.05208 0.05208] Player Out Locker
                    (bind (_direction_4 _playermovementvalue_2) (`Timeline|PlayerOut` :!via `PlayFromStart`)
                      (:`Update`
                        (bind _returnvalue_2 (`KismetMathLibrary.TLerp` (`KismetMathLibrary.MakeTransform` (`self.K2_GetActorLocation` (`self.Player Ref`))) (`KismetMathLibrary.MakeTransform` (`SceneComponent.K2_GetComponentLocation` (`self.OutDrawerPointRef`))) _playermovementvalue_2))
                        (`self.K2_SetActorLocation` _player_ref (`KismetMathLibrary.MakeVector` (.x (.location _returnvalue_2)) (.y (.location _returnvalue_2)) _returnvalue_z) false false))
                      (:`Finished`
                        (`|ExecutionSequence`
                          (:`then_0`
                            (set `/Game/Ravenous/Core/Characters/Player/BP_FirstPersonCharacter.MobilityState` "NewEnumerator3" (`self.Player Ref`))
                            ;[0.05208 0.05208 0.05208] Set Default Camera View
                            (`/Game/Ravenous/Core/Characters/Player/BP_FirstPersonPlayerController.SetDefaultView` (`/Game/Ravenous/Core/Characters/Player/BP_FirstPersonCharacter.PlayerControllerRef` (`self.Player Ref`)))
                            ;[0.05208 0.05208 0.05208] Re Enable Players Input
                            (`/Game/Ravenous/Core/Characters/Player/BP_FirstPersonPlayerController.EnablePlayer` (`/Game/Ravenous/Core/Characters/Player/BP_FirstPersonCharacter.PlayerControllerRef` _player_ref_6) _player_ref_6 false)
                            (set `self.bIsPlayerInside` false))
                          (:`then_1`
                            (goto _label_4 :!via `ReverseFromEnd`)))))))))))))))

(event `self.InteractRange.OnComponentBeginOverlap`
  (params (OverlappedComponent :type "PrimitiveComponent Object Reference") (OtherActor :type "Actor Object Reference") (OtherComp :type "PrimitiveComponent Object Reference") (OtherBodyIndex :type Integer) (bFromSweep :type Boolean) (SweepResult :type "HitResult Structure (by ref)"))
  (goto _label :!via `Open`))

(event `self.InteractRange.OnComponentEndOverlap`
  (params (OverlappedComponent :type "PrimitiveComponent Object Reference") (OtherActor :type "Actor Object Reference") (OtherComp :type "PrimitiveComponent Object Reference") (OtherBodyIndex :type Integer))
  (goto _label :!via `Close`))

(event `EnnemyGrabsPlayer`
  ;[0.05208 0.05208 0.05208] Doors Opening Movement
  (bind (_direction _newtrack_0) (`Timeline|Timeline_1` :!via `PlayFromStart`)
    (:`Update`
      (`SceneComponent.K2_SetRelativeRotation` (`self.S_TestHidingDrawer_Left_Door`) (`KismetMathLibrary.MakeRotator` 0.0 0.0 (`KismetMathLibrary.Lerp` 0.0 80.0 _newtrack_0)) false false)
      (`SceneComponent.K2_SetRelativeRotation` (`self.S_TestHidingDrawer_RightDoor`) (`KismetMathLibrary.MakeRotator` 0.0 0.0 (`KismetMathLibrary.Lerp` 0.0 -80.0 _newtrack_0)) false false))))

(fn `GetLookingRotator`)

(fn `UserConstructionScript`
  (bind (_returnvalue_roll _returnvalue_pitch _returnvalue_yaw) (`KismetMathLibrary.BreakRotator` (`self.K2_GetActorRotation`)))
  (set `self.YawMedianValue` _returnvalue_yaw))