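; Inspectable doll for Puzzle 03 whose head the player can detach to obtain the candle head item.
; Tick shows a gamepad-aware prompt widget during inspection when the focused part is the capsule and the head is still attached.
; The inspection-interact input fires once, playing a timeline that twists and lifts the head with a crack sound.
; When it finishes, the head hides, the player receives the item, inspection exits and collision turns off.
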(event `self.ReceiveBeginPlay`
  (`parent.ReceiveBeginPlay`)
  (set `self.DefaultRot` (`SceneComponent.RelativeRotation` (`self.Item`)))
  (set `self.DefaultHeadLoc` (`SceneComponent.RelativeLocation` (`self.S_LouisHead`))))

(event `EnhancedInput|/Game/Ravenous/Core/Characters/Player/Input/Actions/Player/IA_InteractInspection`
  (params (ActionValue :type Boolean) (ElapsedSeconds :type "Float (double-precision)") (TriggeredSeconds :type "Float (double-precision)") (InputAction :type "InputAction Object Reference" :default "/Game/Ravenous/Core/Characters/Player/Input/Actions/Player/IA_InteractInspection.IA_InteractInspection"))
  (bind _s_louishead (`self.S_LouisHead`))
  (bind _defaultheadloc (`self.DefaultHeadLoc`))
  (:`Started`
    (`/Engine/EditorBlueprintResources/StandardMacros.DoOnce` false
      (:`Completed`
        (set `self.bCanLeave` false)
        (set `self.IsHeadPicked` true)
        (bind (_direction _rotlerp _loclerp) (`Timeline|Head Anim` :!via `PlayFromStart`)
          (:`Update`
            (`|ExecutionSequence`
              (:`then_0`
                (`SceneComponent.K2_SetRelativeRotation` _s_louishead (`KismetMathLibrary.RLerp` (struct) (struct :`Pitch` -50.0) _rotlerp) false false)
                (`SceneComponent.K2_SetRelativeLocation` _s_louishead (`KismetMathLibrary.VLerp` _defaultheadloc (+ _defaultheadloc (0.0 0.0 35.0)) _loclerp) false false))
              (:`then_1`
                (`/Engine/EditorBlueprintResources/StandardMacros.DoOnce` false
                  (:`Completed`
                    (`KismetSystemLibrary.Delay` 0.1)
                    (`GameplayStatics.PlaySoundAtLocation` "/Game/Ravenous/Sound/Doll/CrackDoll_Cue.CrackDoll_Cue" (`self.K2_GetActorLocation`) (struct) 1.0 1.0 0.0 null null null null))))))
          (:`Finished`
            (`SceneComponent.SetVisibility` (`self.S_LouisHead`) false false)
            (`/Game/Ravenous/Core/Characters/Player/BP_FirstPersonCharacter.SetHandleItem` (`self.Player Ref`) (`self.CandleHeadRef`))
            (`self.ExitObject`)
            (`self.SetActorEnableCollision` false)))))))

(event `self.ReceiveTick`
  (params (DeltaSeconds :type "Float (single-precision)"))
  (if (`/Game/Ravenous/Core/Characters/Player/BP_FirstPersonCharacter.bInspecting?` (`self.Player Ref`))
    (`|ExecutionSequence`
      (:`then_0`
        (`/Engine/EditorBlueprintResources/StandardMacros.DoOnce` false :!label _label
          (:`Completed`
            (bind _asw_interaction_inspection (cast `/Game/Ravenous/UI/Widgets/W_InteractionInspection` (`WidgetComponent.GetWidget` (`self.WidgetHead`))))
            (`/Game/Ravenous/UI/Widgets/W_InteractionInspection.Set Ui Input` _asw_interaction_inspection (`/Game/Ravenous/Core/Characters/Player/BP_FirstPersonCharacter.bIsUsingGamePad` (`self.Player Ref`))))))
      (:`then_1`
        _))
    ;[0.05208 0.05208 0.05208] Set Widget Visibility
    (if (and (not (`self.IsHeadPicked`)) (`KismetStringLibrary.EqualEqual_StrStr` (`self.PartName`) (`KismetSystemLibrary.GetObjectName` (`self.Capsule`))) (not (`/Game/Ravenous/Core/Characters/Player/BP_FirstPersonCharacter.bCanInspect?` (`self.Player Ref`))))
      (`SceneComponent.SetHiddenInGame` (`self.WidgetHead`) false false)
      (else
        (`SceneComponent.SetHiddenInGame` (`self.WidgetHead`) true false :!label _label_2)))
    (else
      (`|ExecutionSequence`
        (:`then_0`
          (goto _label :!via `Reset`))
        (:`then_1`
          (goto _label_2))))))

(fn `UserConstructionScript`
  (`parent.UserConstructionScript`)
  (`SceneComponent.SetVisibility` (`self.PointLight`) (`self.bHasLight?`) false))