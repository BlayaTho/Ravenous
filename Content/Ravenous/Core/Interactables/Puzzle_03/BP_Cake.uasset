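; BP_Cake is an interactable puzzle cake that takes three candles (Louis, Lucy, Mom) from the player.
; Interacting with a held candle reveals the mesh matching its CandleIndex and destroys the item; the first interaction also displays a Louis text line.
; Once all candles are placed, it advances the trigger manager's state.
; Until then, an overlap-controlled gate on Tick shows a close-range widget facing the player.
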(event `self.ReceiveBeginPlay`
  ;[0.05208 0.05208 0.05208] Init
  (bind _asbp_first_person_character (cast `/Game/Ravenous/Core/Characters/Player/BP_FirstPersonCharacter` (`GameplayStatics.GetPlayerCharacter` 0)))
  (set `self.PlayerRef` _asbp_first_person_character))

(event `CheckCandles`
  (if (not (`KismetArrayLibrary.Array_Contains` (`self.IsCandlePlaced`)))
    (`KismetSystemLibrary.PrintString` "Door Unlocked")
    (set `self.bIsAllGood` true)
    (`/Game/Ravenous/Core/Interactables/Trigger_Event/BP_TriggerMANAGER.ChangeTriggersState` (`self.TriggerManagerRef`) 4)
    (else
      (`KismetSystemLibrary.PrintString` "Still needs Head(s)"))))

(event `/Game/Ravenous/Core/Characters/Interface/BPI_Interaction.Interact`
  (params (ForDoor :type Boolean) (ForLock :type Boolean) (Name :type String) (PlayerRef :type "/Game/Ravenous/Core/Characters/Player/BP_FirstPersonCharacter Object Reference"))
  (bind _candleindex (`/Game/Ravenous/Core/Interactables/Bp_PickableItem.CandleIndex` (`/Game/Ravenous/Core/Characters/Player/BP_FirstPersonCharacter.HeldItem` PlayerRef)))
  (`|ExecutionSequence`
    (:`then_0`
      (`/Engine/EditorBlueprintResources/StandardMacros.IsValid` (`/Game/Ravenous/Core/Characters/Player/BP_FirstPersonCharacter.HeldItem` PlayerRef)
        (:`Is Valid`
          (if (`|EnumEquality` (`/Game/Ravenous/Core/Interactables/Bp_PickableItem.ItemType` (`/Game/Ravenous/Core/Characters/Player/BP_FirstPersonCharacter.HeldItem` PlayerRef)) "NewEnumerator9")
            (`SceneComponent.SetVisibility` (select `int` _candleindex :`0` (`self.FirstCandleLouis`) :`1` (`self.ScndCandleLucy`) :`2` (`self.ThirdCandleMom`) :!type "SceneComponent Object Reference") true true)
            (`KismetArrayLibrary.Array_Set` (`self.IsCandlePlaced`) _candleindex true)
            (`self.CheckCandles`)
            (`/Game/Ravenous/Core/Characters/Player/BP_FirstPersonCharacter.DestroyHeldItem` PlayerRef)))))
    (:`then_1`
      (`/Engine/EditorBlueprintResources/StandardMacros.DoOnce` false
        (:`Completed`
          (`/Game/Ravenous/UI/Widgets/W_LouisText.DisplayText` (`/Game/Ravenous/Core/Characters/Player/BP_FirstPersonCharacter.W_LouisText` PlayerRef) "08_SalonDadsDoll" 1.5))))))

(event `self.ReceiveTick`
  (params (DeltaSeconds :type "Float (single-precision)"))
  ;[0.1146 0.1146 0.1146] Close Range Widget
  (if (not (`self.bIsAllGood`))
    (`/Engine/EditorBlueprintResources/StandardMacros.Gate` true :!label _label
      (:`Exit`
        (`SceneComponent.K2_SetRelativeRotation` (`self.W_CloseRange`) (`KismetMathLibrary.FindLookAtRotation` (`self.K2_GetActorLocation`) (`self.K2_GetActorLocation` (`self.PlayerRef`))) false false)
        (`SceneComponent.SetVisibility` (`self.W_CloseRange`) true false)))
    (else
      (`SceneComponent.SetVisibility` (`self.W_CloseRange`) false false))))

(event `self.PlayerDetect.OnComponentBeginOverlap`
  (params (OverlappedComponent :type "PrimitiveComponent Object Reference") (OtherActor :type "Actor Object Reference") (OtherComp :type "PrimitiveComponent Object Reference") (OtherBodyIndex :type Integer) (bFromSweep :type Boolean) (SweepResult :type "HitResult Structure (by ref)"))
  ;[0.1146 0.1146 0.1146] Close Range Widget
  (if (and (== OtherActor (`self.PlayerRef`)) (not (`self.bIsAllGood`)))
    (set `self.PlayerLoc` SweepResult_Location)
    (goto _label :!via `Open`)))

(event `self.PlayerDetect.OnComponentEndOverlap`
  (params (OverlappedComponent :type "PrimitiveComponent Object Reference") (OtherActor :type "Actor Object Reference") (OtherComp :type "PrimitiveComponent Object Reference") (OtherBodyIndex :type Integer))
  ;[0.1146 0.1146 0.1146] Close Range Widget
  (if (== OtherActor (`self.PlayerRef`))
    (`SceneComponent.SetVisibility` (`self.W_CloseRange`) false false)
    (goto _label :!via `Close`)))

(fn `UserConstructionScript`)