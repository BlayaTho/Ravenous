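; Louis doll interactable for Puzzle 03, whose head can be removed once to give the player a candle head item.
; The first inspection-interact input plays a timeline that rotates and raises the head mesh from its cached position.
; When the timeline finishes, the mesh is hidden and the candle head reference becomes the player's handle item.
; Tick toggles the head prompt widget from the player's CanInspect flag, keeping it hidden after pickup.
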(event `self.ReceiveBeginPlay`
  (`parent.ReceiveBeginPlay`)
  (set `self.DefaultRot` (`SceneComponent.RelativeRotation` (`self.Item`)))
  (set `self.DefaultHeadLoc` (`SceneComponent.RelativeLocation` (`self.S_LouisHead`))))

(event `EnhancedInput|/Game/Ravenous/Core/Characters/Player/Input/Actions/Player/IA_InteractInspection`
  (params (ActionValue :type Boolean) (ElapsedSeconds :type "Float (double-precision)") (TriggeredSeconds :type "Float (double-precision)") (InputAction :type "InputAction Object Reference" :default "/Game/Ravenous/Core/Characters/Player/Input/Actions/Player/IA_InteractInspection.IA_InteractInspection"))
  (bind _s_louishead (`self.S_LouisHead`))
  (bind _defaultheadloc (`self.DefaultHeadLoc`))
  (:`Started`
    (`/Engine/EditorBlueprintResources/StandardMacros.DoOnce` false
      (:`Completed`
        (set `self.IsHeadPicked` true)
        (bind (_direction _rotlerp _loclerp) (`Timeline|Head Anim` :!via `PlayFromStart`)
          (:`Update`
            (`SceneComponent.K2_SetRelativeRotation` _s_louishead (`KismetMathLibrary.RLerp` (struct) (struct :`Pitch` -50.0) _rotlerp) false false)
            (`SceneComponent.K2_SetRelativeLocation` _s_louishead (`KismetMathLibrary.VLerp` _defaultheadloc (+ _defaultheadloc (0.0 0.0 35.0)) _loclerp) false false))
          (:`Finished`
            (`SceneComponent.SetVisibility` (`self.S_LouisHead`) false false)
            (`/Game/Ravenous/Core/Characters/Player/BP_FirstPersonCharacter.SetHandleItem` (`self.Player Ref`) (`self.CandleHeadRef`))))))))

(event `self.ReceiveTick`
  (params (DeltaSeconds :type "Float (single-precision)"))
  ;[0.05208 0.05208 0.05208] Set Widget Visibility
  (if (not (`self.IsHeadPicked`))
    (`SceneComponent.SetHiddenInGame` (`self.WidgetHead`) (`/Game/Ravenous/Core/Characters/Player/BP_FirstPersonCharacter.bCanInspect?` (`self.Player Ref`)) false)
    (else
      (`SceneComponent.SetHiddenInGame` (`self.WidgetHead`) true false))))

(fn `UserConstructionScript`
  (`parent.UserConstructionScript`))