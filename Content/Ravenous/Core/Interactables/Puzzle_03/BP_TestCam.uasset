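; BP_TestCam is an interactable fixed camera in Puzzle_03 that lets the player look at a room from its viewpoint.
; Interact blends the view target to it and hands over input; lock-view or interact input blends back, with a delayed InMotion flag blocking re-triggers mid-blend.
; Look input rotates the camera in clamped steps within narrow yaw and pitch limits.
; Timer-based view switching and lock-view widget logic are left disconnected.
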(event `self.ReceiveBeginPlay`
  ;[1 0 0 1 56] THOMAS
)

(event `ARA`
  ;[1 0 0 1 56] THOMAS
  (`PlayerController.SetViewTargetWithBlend` (`GameplayStatics.GetPlayerController` 0) self 0.5 "VTBlend_Cubic" 0.0 false))

(event `STOP`
  ;[1 0 0 1 56] THOMAS
  (`PlayerController.SetViewTargetWithBlend` (`GameplayStatics.GetPlayerController` 0) (`self.As BP First Person Character`) 0.5 "VTBlend_Cubic" 0.0 false))

(event `/Game/Ravenous/Core/Characters/Interface/BPI_Interaction.Interact`
  (params (ForDoor :type Boolean) (ForLock :type Boolean) (Name :type String) (PlayerRef :type "/Game/Ravenous/Core/Characters/Player/BP_FirstPersonCharacter Object Reference"))
  ;[0.05208 0.05208 0.05208] Look At Room
  (if (not (`self.bInMotion`))
    (set `self.Player Ref` PlayerRef)
    (`self.SetCameraView`)
    (`KismetSystemLibrary.Delay` 0.6)
    (set `self.bInMotion` false)))

(event `EnhancedInput|/Game/Ravenous/Core/Characters/Player/Input/Actions/Player/IA_LockView`
  (params (ActionValue :type Boolean) (ElapsedSeconds :type "Float (double-precision)") (TriggeredSeconds :type "Float (double-precision)") (InputAction :type "InputAction Object Reference" :default "/Game/Ravenous/Core/Characters/Player/Input/Actions/Player/IA_LockView.IA_LockView"))
  ;[0.05208 0.05208 0.05208] Leave
  (:`Started`
    (if (not (`self.bInMotion`)) :!label _label
      (`self.Leave`)
      (`KismetSystemLibrary.Delay` 0.6)
      (set `self.bInMotion` false))))

(event `EnhancedInput|/Game/Ravenous/Core/Characters/Player/Input/Actions/Player/IA_Interact`
  (params (ActionValue :type Boolean) (ElapsedSeconds :type "Float (double-precision)") (TriggeredSeconds :type "Float (double-precision)") (InputAction :type "InputAction Object Reference" :default "/Game/Ravenous/Core/Characters/Player/Input/Actions/Player/IA_Interact.IA_Interact"))
  ;[0.05208 0.05208 0.05208] Leave
  (:`Started`
    (goto _label)))

(event `EnhancedInput|/Game/Ravenous/Core/Characters/Player/Input/Actions/Player/IA_Look`
  (params (ActionValue :type "Vector2D Structure") (ElapsedSeconds :type "Float (double-precision)") (TriggeredSeconds :type "Float (double-precision)") (InputAction :type "InputAction Object Reference" :default "/Game/Ravenous/Core/Characters/Player/Input/Actions/Player/IA_Look.IA_Look"))
  (bind _returnvalue (* ActionValue_X 0.5))
  (bind _returnvalue_2 (* (* ActionValue_Y 0.5) -1.0))
  (:`Triggered`
    (`|ExecutionSequence`
      (:`then_0`
        (if (`self.CanMoveTo+X` _returnvalue)
          (`SceneComponent.K2_AddRelativeRotation` (`self.Camera`) (`KismetMathLibrary.MakeRotator` 0.0 0.0 (`KismetMathLibrary.FClamp` _returnvalue -3.0 3.0)) false false :!label _label_2)))
      (:`then_1`
        (if (`self.CanMoveTo-X` _returnvalue)
          (goto _label_2)))
      (:`then_2`
        (if (`self.CanMoveTo+Y` _returnvalue_2)
          (`SceneComponent.K2_AddRelativeRotation` (`self.Camera`) (`KismetMathLibrary.MakeRotator` 0.0 (`KismetMathLibrary.FClamp` _returnvalue_2 -3.0 3.0)) false false :!label _label_3)))
      (:`then_3`
        (if (`self.CanMoveTo-Y` _returnvalue_2)
          (goto _label_3))))))

(fn `CanMoveTo+X`
  (params (A :type "Float (double-precision)"))
  (returns (ReturnValue :type Boolean))
  (bind (_relativerotation_roll _relativerotation_pitch _relativerotation_yaw) (`KismetMathLibrary.BreakRotator` (`SceneComponent.RelativeRotation` (`self.Camera`))))
  (return (and (> A 0.0) (<= _relativerotation_yaw 12.5))))

(fn `CanMoveTo+Y`
  (params (A :type "Float (double-precision)"))
  (returns (ReturnValue :type Boolean))
  (bind (_relativerotation_roll _relativerotation_pitch) (`KismetMathLibrary.BreakRotator` (`SceneComponent.RelativeRotation` (`self.Camera`))))
  (return (and (> A 0.0) (<= _relativerotation_pitch 10.0))))

(fn `CanMoveTo-X`
  (params (A :type "Float (double-precision)"))
  (returns (ReturnValue :type Boolean))
  (bind (_relativerotation_roll _relativerotation_pitch _relativerotation_yaw) (`KismetMathLibrary.BreakRotator` (`SceneComponent.RelativeRotation` (`self.Camera`))))
  (return (and (< A 0.0) (>= _relativerotation_yaw -7.5))))

(fn `CanMoveTo-Y`
  (params (A :type "Float (double-precision)"))
  (returns (ReturnValue :type Boolean))
  (bind (_relativerotation_roll _relativerotation_pitch) (`KismetMathLibrary.BreakRotator` (`SceneComponent.RelativeRotation` (`self.Camera`))))
  (return (and (< A 0.0) (>= _relativerotation_pitch -7.5))))

(fn `EnableInputs`
  (bind _player_ref (`self.Player Ref`))
  (bind _playercontrollerref (`/Game/Ravenous/Core/Characters/Player/BP_FirstPersonCharacter.PlayerControllerRef` _player_ref))
  (`self.DisableInput` (select `bool` (`self.bInInteraction`) :`false` self :`true` _player_ref :!type "Actor Object Reference") _playercontrollerref)
  (`self.EnableInput` (select `bool` (`self.bInInteraction`) :`false` (`self.Player Ref`) :`true` self :!type "Actor Object Reference") _playercontrollerref))

(fn `Leave`
  (`self.SetCameraView`)
  (`self.EnableInputs`))

(fn `SetCameraView`
  (bind _player_ref (`self.Player Ref`))
  (set `self.bInMotion` true)
  (`PlayerController.SetViewTargetWithBlend` (`/Game/Ravenous/Core/Characters/Player/BP_FirstPersonCharacter.PlayerControllerRef` _player_ref) (select `bool` (`self.bInInteraction`) :`false` self :`true` _player_ref :!type "Actor Object Reference") 0.5 "VTBlend_Cubic" 0.0 false)
  (set `self.bInInteraction` (not (`self.bInInteraction`)))
  (`self.EnableInputs`))

(fn `UserConstructionScript`)