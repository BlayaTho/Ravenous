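; Pickable item actor for Ravenous, configured by an ItemType enum covering keys, handle, tale page, baby doll, phone and candle heads.
; The construction script sets each type's mesh, adding a child head component for the baby.
; Interact hands the item to the player with a sound, with extra conditions or triggers for some types.
; HeadShake swings the baby's head, then opens a Tick-fed gate so it tracks the player.
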(event `self.ReceiveBeginPlay`
  (bind _asbp_first_person_character (cast `/Game/Ravenous/Core/Characters/Player/BP_FirstPersonCharacter` (`GameplayStatics.GetPlayerCharacter` 0)))
  (set `self.Player Ref` _asbp_first_person_character))

(event `/Game/Ravenous/Core/Characters/Interface/BPI_Interaction.Interact`
  (params (ForDoor :type Boolean) (ForLock :type Boolean) (Name :type String) (PlayerRef :type "/Game/Ravenous/Core/Characters/Player/BP_FirstPersonCharacter Object Reference"))
  (bind _tabouretref (`self.TabouretRef`))
  (bind _output_get (set `self.Player Ref` PlayerRef))
  (switch `/Game/Ravenous/Data/E_PickableItemList` (`self.ItemType`)
    (:`NewEnumerator0`
      (`/Game/Ravenous/Core/Characters/Player/BP_FirstPersonCharacter.SetHandleItem` (`self.Player Ref`) self :!label _label)
      ;[0.09166 0.4458 1] PickUp Sound
      (`GameplayStatics.PlaySoundAtLocation` "/Game/Ravenous/Sound/Player/GrabItem_Cue.GrabItem_Cue" (`self.K2_GetActorLocation` _output_get) (struct) 1.0 1.0 0.0 null null null null))
    (:`NewEnumerator4`
      (goto _label))
    (:`NewEnumerator1`
      (goto _label))
    (:`NewEnumerator2`
      (if (not (`/Game/Ravenous/Core/Interactables/Puzzle_02/BP_CodeDisplayer.bIsDisplaying` (`self.CodeDisplayerRef`)))
        (goto _label)))
    (:`NewEnumerator6`
      (if (`self.bCanBePicked`)
        (goto _label)))
    (:`NewEnumerator7`
      (goto _label))
    (:`NewEnumerator8`
      (goto _label))
    (:`NewEnumerator9`
      (goto _label))
    (:`NewEnumerator10`
      (`/Engine/EditorBlueprintResources/StandardMacros.IsValid` _tabouretref
        (:`Is Valid`
          (`/Game/Ravenous/Core/Interactables/Puzzle_04/BP_FallingTabouret.StartFall` _tabouretref)
          (goto _label))))))

(event `HeadShake`
  (bind (_returnvalue_roll _returnvalue_pitch _returnvalue_yaw) (`KismetMathLibrary.BreakRotator` (`self.K2_GetActorRotation`)))
  (bind (_returnvalue_roll_2 _returnvalue_pitch_2 _returnvalue_yaw_2) (`KismetMathLibrary.BreakRotator` (`KismetMathLibrary.FindLookAtRotation` (`SceneComponent.K2_GetComponentLocation` (`SceneComponent.GetChildComponent` (`self.StaticMesh`) 0)) (`self.K2_GetActorLocation` (`self.Player Ref`)))))
  ;[0.05208 0.05208 0.05208] Baby HeadShake
  (`/Engine/EditorBlueprintResources/StandardMacros.IsValid` (`SceneComponent.GetChildComponent` (`self.StaticMesh`) 0)
    (:`Is Valid`
      (`|ExecutionSequence`
        (:`then_0`
          (bind (_direction _lerprotation) (`Timeline|Timeline` :!via `PlayFromStart`)
            (:`Update`
              (`SceneComponent.K2_SetRelativeRotation` (`SceneComponent.GetChildComponent` (`self.StaticMesh`) 0) (`KismetMathLibrary.MakeRotator` 0.0 0.0 (`KismetMathLibrary.Lerp` -50.0 50.0 _lerprotation)) false false))
            (:`Finished`
              (goto _label_2 :!via `Open`))))
        (:`then_1`
          (goto _label_2 :!via `Close`))))))

(event `self.ReceiveTick`
  (params (DeltaSeconds :type "Float (single-precision)"))
  (bind (_returnvalue_roll _returnvalue_pitch _returnvalue_yaw) (`KismetMathLibrary.BreakRotator` (`self.K2_GetActorRotation`)))
  (bind (_returnvalue_roll_2 _returnvalue_pitch_2 _returnvalue_yaw_2) (`KismetMathLibrary.BreakRotator` (`KismetMathLibrary.FindLookAtRotation` (`SceneComponent.K2_GetComponentLocation` (`SceneComponent.GetChildComponent` (`self.StaticMesh`) 0)) (`self.K2_GetActorLocation` (`self.Player Ref`)))))
  ;[0.05208 0.05208 0.05208] Make Baby Head Rota
  (if (`|EnumEquality` (`self.ItemType`) "NewEnumerator6")
    (`/Engine/EditorBlueprintResources/StandardMacros.Gate` false :!label _label_2
      (:`Exit`
        (`SceneComponent.K2_SetRelativeRotation` (`SceneComponent.GetChildComponent` (`self.StaticMesh`) 0) (`KismetMathLibrary.MakeRotator` 0.0 0.0 (- (- _returnvalue_yaw_2 _returnvalue_yaw) 90.0)) false false)))))

(fn `UserConstructionScript`
  (bind _staticmesh (`self.StaticMesh`))
  (bind _staticmesh_2 (`self.StaticMesh`))
  (bind _staticmesh_3 (`self.StaticMesh`))
  (switch `/Game/Ravenous/Data/E_PickableItemList` (`self.ItemType`)
    (:`NewEnumerator0`
      (`StaticMeshComponent.SetStaticMesh` _staticmesh_3 "/Game/Ravenous/Assets/Prototype_PreProd/SM_Key.SM_Key")
      (`SceneComponent.SetRelativeScale3D` _staticmesh_3 (1.0 1.0 1.0)))
    (:`NewEnumerator4`
      (`StaticMeshComponent.SetStaticMesh` _staticmesh_2 "/Game/Ravenous/Art/KeyWithTag/S_Key_.S_Key_")
      (`SceneComponent.SetRelativeScale3D` _staticmesh_2 (2.0 2.0 2.0)))
    (:`NewEnumerator1`
      (`StaticMeshComponent.SetStaticMesh` (`self.StaticMesh`) "/Game/Ravenous/Assets/AlphaV02/S_WallShelf_/S_WallShelfHandle_.S_WallShelfHandle_"))
    (:`NewEnumerator2`
      (`StaticMeshComponent.SetStaticMesh` (`self.StaticMesh`) "/Game/Ravenous/Art/LouisBedroom/Drawing/S_PaperDraw.S_PaperDraw")
      (`PrimitiveComponent.SetMaterial` (`self.StaticMesh`) 0 (select `int` (`self.DefaultValue`) :`0` "/Game/Ravenous/Art/LouisBedroom/Drawing/M_Drawing_Inst01.M_Drawing_Inst01" :`1` "/Game/Ravenous/Art/LouisBedroom/Drawing/M_Drawing_Inst02.M_Drawing_Inst02" :`2` "/Game/Ravenous/Art/LouisBedroom/Drawing/M_Drawing_Inst03.M_Drawing_Inst03" :`3` "/Game/Ravenous/Art/LouisBedroom/Drawing/M_Drawing_Inst04.M_Drawing_Inst04" :!type "MaterialInterface Object Reference")))
    (:`NewEnumerator6`
      (`StaticMeshComponent.SetStaticMesh` (`self.StaticMesh`) "/Game/Ravenous/Art/Nursery/Baby/S_PlasticBaby01.S_PlasticBaby01")
      (bind _returnvalue (`AddComponent|NODE_AddStaticMeshComponent-1` :`RelativeTransform` (`KismetMathLibrary.MakeTransform` (0.0 1.0 9.0))))
      (`SceneComponent.K2_AttachToComponent` _returnvalue (`self.StaticMesh`) "None" "KeepRelative" "KeepRelative" "KeepRelative" true))
    (:`NewEnumerator7`
      (`StaticMeshComponent.SetStaticMesh` (`self.StaticMesh`) "/Game/Ravenous/Art/Salon/Props/S_Phone/phone_lp.phone_lp")
      (`SceneComponent.K2_SetRelativeLocation` (`self.StaticMesh`) (0.0 4.75 -9.5) false false))
    (:`NewEnumerator8`
      (`StaticMeshComponent.SetStaticMesh` (`self.StaticMesh`) "/Game/Ravenous/Art/Salon/Props/S_PendulumKey_/S_KeyPendulum_.S_KeyPendulum_"))
    (:`NewEnumerator9`
      (`StaticMeshComponent.SetStaticMesh` (`self.StaticMesh`) (select `int` (`self.CandleIndex`) :`0` "/Game/Ravenous/Art/Salon/dolls/Doll_Lucy/S_Doll_LucyHead.S_Doll_LucyHead" :`1` "/Game/Ravenous/Art/Salon/dolls/Doll_Lucy/S_Doll_LucyHead.S_Doll_LucyHead" :`2` "/Game/Ravenous/Art/Salon/dolls/Doll_Mother/S_Doll_MotherHead.S_Doll_MotherHead" :!type "StaticMesh Object Reference")))
    (:`NewEnumerator10`
      (`StaticMeshComponent.SetStaticMesh` (`self.StaticMesh`) "/Game/Ravenous/Art/ParentBedroom/MusicBox/S_MusicBoxKey.S_MusicBoxKey"))
    (:`NewEnumerator11`
      (`StaticMeshComponent.SetStaticMesh` _staticmesh "/Game/Ravenous/Assets/Prototype_PreProd/SM_BabyKey_PH.SM_BabyKey_PH")
      (`SceneComponent.SetRelativeScale3D` _staticmesh (0.5 0.5 0.5)))))