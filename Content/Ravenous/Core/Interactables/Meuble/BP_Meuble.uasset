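; Interactable furniture piece (meuble) with three drawers that slide open and closed individually.
; Interact switches on the drawer name, flips its entry in DrawerStateArr and plays or reverses that drawer's timeline to lerp relative X toward OpenAngle, a distance despite its name.
; A DoOnce per drawer blocks re-triggering until the timeline finishes.
; The construction script pre-opens drawers flagged in the array; its HasProps branch is empty.
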(event `/Game/Ravenous/Core/Characters/Interface/BPI_Interaction.Interact`
  (params (ForDoor :type Boolean) (ForLock :type Boolean) (Name :type String) (PlayerRef :type "/Game/Ravenous/Core/Characters/Player/BP_FirstPersonCharacter Object Reference"))
  (bind _sm_drawer_01 (`self.SM_Drawer_01`))
  (bind _sm_drawer_03 (`self.SM_Drawer_03`))
  (bind _sm_drawer_02 (`self.SM_Drawer_02`))
  (bind _output (`|GetArrayItem` (`self.DrawerStateArr`) 2))
  (bind _output_2 (`|GetArrayItem` (`self.DrawerStateArr`) 0))
  (bind _output_3 (`|GetArrayItem` (`self.DrawerStateArr`) 1))
  (bind (_relativelocation_x _relativelocation_y _relativelocation_z) (`KismetMathLibrary.BreakVector` (`SceneComponent.RelativeLocation` _sm_drawer_03)))
  (bind (_relativelocation_x_2 _relativelocation_y_2 _relativelocation_z_2) (`KismetMathLibrary.BreakVector` (`SceneComponent.RelativeLocation` _sm_drawer_01)))
  (bind (_relativelocation_x_3 _relativelocation_y_3 _relativelocation_z_3) (`KismetMathLibrary.BreakVector` (`SceneComponent.RelativeLocation` _sm_drawer_02)))
  (switch `string` Name
    (:`SM_Drawer_01`
      (`/Engine/EditorBlueprintResources/StandardMacros.DoOnce` false :!label _label
        (:`Completed`
          (`KismetArrayLibrary.Array_Set` (`self.DrawerStateArr`) 0 (not _output_2))
          (if _output_2
            (bind (_direction _translationlerp) (`Timeline|Timeline_2` :!via `PlayFromStart` :!label _label_2)
              (:`Update`
                (`SceneComponent.K2_SetRelativeLocation` _sm_drawer_01 (`KismetMathLibrary.MakeVector` (`KismetMathLibrary.Lerp` 63.0 (`self.OpenAngle`) _translationlerp) _relativelocation_y_2 _relativelocation_z_2) false false))
              (:`Finished`
                (goto _label :!via `Reset`)))
            (else
              (goto _label_2 :!via `ReverseFromEnd`))))))
    (:`SM_Drawer_02`
      (`/Engine/EditorBlueprintResources/StandardMacros.DoOnce` false :!label _label_3
        (:`Completed`
          (`KismetArrayLibrary.Array_Set` (`self.DrawerStateArr`) 1 (not _output_3))
          (if _output_3
            (bind (_direction_2 _translationlerp_2) (`Timeline|Timeline_1` :!via `PlayFromStart` :!label _label_4)
              (:`Update`
                (`SceneComponent.K2_SetRelativeLocation` _sm_drawer_02 (`KismetMathLibrary.MakeVector` (`KismetMathLibrary.Lerp` 63.0 (`self.OpenAngle`) _translationlerp_2) _relativelocation_y_3 _relativelocation_z_3) false false))
              (:`Finished`
                (goto _label_3 :!via `Reset`)))
            (else
              (goto _label_4 :!via `ReverseFromEnd`))))))
    (:`SM_Drawer_03`
      (`/Engine/EditorBlueprintResources/StandardMacros.DoOnce` false :!label _label_5
        (:`Completed`
          (`KismetArrayLibrary.Array_Set` (`self.DrawerStateArr`) 2 (not _output))
          (if _output
            (bind (_direction_3 _translationlerp_3) (`Timeline|Timeline` :!via `PlayFromStart` :!label _label_6)
              (:`Update`
                (`SceneComponent.K2_SetRelativeLocation` _sm_drawer_03 (`KismetMathLibrary.MakeVector` (`KismetMathLibrary.Lerp` 63.0 (`self.OpenAngle`) _translationlerp_3) _relativelocation_y _relativelocation_z) false false))
              (:`Finished`
                (goto _label_5 :!via `Reset`)))
            (else
              (goto _label_6 :!via `ReverseFromEnd`))))))))

(fn `UserConstructionScript`
  (bind _sm_drawer_02 (`self.SM_Drawer_02`))
  (bind _sm_drawer_03 (`self.SM_Drawer_03`))
  (bind _sm_drawer_01 (`self.SM_Drawer_01`))
  (bind (_relativelocation_x _relativelocation_y _relativelocation_z) (`KismetMathLibrary.BreakVector` (`SceneComponent.RelativeLocation` _sm_drawer_03)))
  (bind (_relativelocation_x_2 _relativelocation_y_2 _relativelocation_z_2) (`KismetMathLibrary.BreakVector` (`SceneComponent.RelativeLocation` _sm_drawer_02)))
  (bind (_relativelocation_x_3 _relativelocation_y_3 _relativelocation_z_3) (`KismetMathLibrary.BreakVector` (`SceneComponent.RelativeLocation` _sm_drawer_01)))
  (`|ExecutionSequence`
    (:`then_0`
      (for (_array_element _array_index) (`self.DrawerStateArr`)
        (if _array_element
          (switch `int` _array_index
            (:`0`
              (`SceneComponent.K2_SetRelativeLocation` _sm_drawer_01 (`KismetMathLibrary.MakeVector` (`self.OpenAngle`) _relativelocation_y_3 _relativelocation_z_3) false false))
            (:`1`
              (`SceneComponent.K2_SetRelativeLocation` _sm_drawer_02 (`KismetMathLibrary.MakeVector` (`self.OpenAngle`) _relativelocation_y_2 _relativelocation_z_2) false false))
            (:`2`
              (`SceneComponent.K2_SetRelativeLocation` _sm_drawer_03 (`KismetMathLibrary.MakeVector` (`self.OpenAngle`) _relativelocation_y _relativelocation_z) false false))))))
    (:`then_1`
      (if (`self.bHasProps`)
        _))))