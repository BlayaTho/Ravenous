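; BP_LargeDresser is a large dresser furniture Blueprint with configurable doors, drawers and glass doors, filed under the game's interactables.
; Its Construction Script checks one boolean per part and destroys that component when the flag is off, so each instance can have its own layout.
; Parts cover two numbered sets of left and right doors and drawers, plus a glass door pair.
; The event graph holds no active logic.
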(fn `UserConstructionScript`
  (`|ExecutionSequence`
    (:`then_0`
      (`|ExecutionSequence`
        (:`then_0`
          (if (not (`self.bHasLeft_01_Door`))
            (`ActorComponent.K2_DestroyComponent` (`self.Door_Left_01`))))
        (:`then_1`
          (if (not (`self.bHasRight_01_Door`))
            (`ActorComponent.K2_DestroyComponent` (`self.Door_Right_01`))))
        (:`then_2`
          (if (not (`self.bHasLeft_01_Drawer`))
            (`ActorComponent.K2_DestroyComponent` (`self.Drawer_Left_01`))))
        (:`then_3`
          (if (not (`self.bHasRight_01_Drawer`))
            (`ActorComponent.K2_DestroyComponent` (`self.Drawer_Right_01`))))
        (:`then_4`
          (if (not (`self.bHasLeftGlassDoor`))
            (`ActorComponent.K2_DestroyComponent` (`self.GlassDoor_Left`))))
        (:`then_5`
          (if (not (`self.bHasRightGlassDoor`))
            (`ActorComponent.K2_DestroyComponent` (`self.GlassDoor_Right`))))))
    (:`then_1`
      (`|ExecutionSequence`
        (:`then_0`
          (if (not (`self.bHasLeft_02_Door`))
            (`ActorComponent.K2_DestroyComponent` (`self.Door_Left_02`))))
        (:`then_1`
          (if (not (`self.bHasRight_02_Door`))
            (`ActorComponent.K2_DestroyComponent` (`self.Door_Right_02`))))
        (:`then_2`
          (if (not (`self.bHasLeft_02_Drawer`))
            (`ActorComponent.K2_DestroyComponent` (`self.Drawer_Left_02`))))
        (:`then_3`
          (if (not (`self.bHasRight_02_Drawer`))
            (`ActorComponent.K2_DestroyComponent` (`self.Drawer_Right_02`))))))))