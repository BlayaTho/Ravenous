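; Interactable furniture piece with six drawer meshes that open and close: the first two pitch open, the other four slide along local X.
; Interact receives a component name, flips that drawer's entry in DrawerStateArr and plays its Timeline forward or in reverse to lerp the motion.
; A DoOnce per drawer blocks re-triggering until the Timeline finishes.
; The construction script poses drawers flagged as open in the array.
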(event `self.Interact`
  (params (ForDoor :type Boolean) (ForLock :type Boolean) (Name :type String) (PlayerRef :type "/Game/Ravenous/Core/Characters/Player/BP_FirstPersonCharacter Object Reference"))
  (bind _output (`|GetArrayItem` (`self.DrawerStateArr`) 2))
  (bind _output_2 (`|GetArrayItem` (`self.DrawerStateArr`) 3))
  (bind _output_3 (`|GetArrayItem` (`self.DrawerStateArr`) 0))
  (bind _output_4 (`|GetArrayItem` (`self.DrawerStateArr`) 5))
  (bind _output_5 (`|GetArrayItem` (`self.DrawerStateArr`) 1))
  (bind _output_6 (`|GetArrayItem` (`self.DrawerStateArr`) 4))
  (bind (_relativelocation_x _relativelocation_y _relativelocation_z) (`KismetMathLibrary.BreakVector` (`SceneComponent.RelativeLocation` (`self.SM_Drawer_04`))))
  (bind (_relativelocation_x_2 _relativelocation_y_2 _relativelocation_z_2) (`KismetMathLibrary.BreakVector` (`SceneComponent.RelativeLocation` (`self.SM_Drawer_06`))))
  (bind (_relativelocation_x_3 _relativelocation_y_3 _relativelocation_z_3) (`KismetMathLibrary.BreakVector` (`SceneComponent.RelativeLocation` (`self.SM_Drawer_05`))))
  (bind (_relativelocation_x_4 _relativelocation_y_4 _relativelocation_z_4) (`KismetMathLibrary.BreakVector` (`SceneComponent.RelativeLocation` (`self.SM_Drawer_03`))))
  (switch `string` Name
    (:`SM_Drawer_01`
      (`/Engine/EditorBlueprintResources/StandardMacros.DoOnce` false :!label _label
        (:`Completed`
          (`KismetArrayLibrary.Array_Set` (`self.DrawerStateArr`) 0 (not _output_3))
          (if _output_3
            (bind (_direction _rotationlerp) (`Timeline|Timeline_3` :!via `PlayFromStart` :!label _label_2)
              (:`Update`
                (`SceneComponent.K2_SetRelativeRotation` (`self.SM_Drawer_01`) (`KismetMathLibrary.MakeRotator` 0.0 (`KismetMathLibrary.Lerp` 0.0 (`self.OpenAngleR`) _rotationlerp)) false false))
              (:`Finished`
                (goto _label :!via `Reset`)))
            (else
              (goto _label_2 :!via `ReverseFromEnd`))))))
    (:`SM_Drawer_02`
      (`/Engine/EditorBlueprintResources/StandardMacros.DoOnce` false :!label _label_3
        (:`Completed`
          (`KismetArrayLibrary.Array_Set` (`self.DrawerStateArr`) 1 (not _output_5))
          (if _output_5
            (bind (_direction_2 _rotationlerp_2) (`Timeline|Timeline_1` :!via `PlayFromStart` :!label _label_4)
              (:`Update`
                (`SceneComponent.K2_SetRelativeRotation` (`self.SM_Drawer_02`) (`KismetMathLibrary.MakeRotator` 0.0 (`KismetMathLibrary.Lerp` 0.0 (`self.OpenAngleR`) _rotationlerp_2)) false false))
              (:`Finished`
                (goto _label_3 :!via `Reset`)))
            (else
              (goto _label_4 :!via `ReverseFromEnd`))))))
    (:`SM_Drawer_03`
      (`/Engine/EditorBlueprintResources/StandardMacros.DoOnce` false :!label _label_5
        (:`Completed`
          (`KismetArrayLibrary.Array_Set` (`self.DrawerStateArr`) 2 (not _output))
          (if _output
            (bind (_direction_3 _translationlerp) (`Timeline|Timeline` :!via `PlayFromStart` :!label _label_6)
              (:`Update`
                (`SceneComponent.K2_SetRelativeLocation` (`self.SM_Drawer_03`) (`KismetMathLibrary.MakeVector` (`KismetMathLibrary.Lerp` (`self.BeginLocationX`) (`self.OpenAngleL`) _translationlerp) _relativelocation_y_4 _relativelocation_z_4) false false))
              (:`Finished`
                (goto _label_5 :!via `Reset`)))
            (else
              (goto _label_6 :!via `ReverseFromEnd`))))))
    (:`SM_Drawer_04`
      (`/Engine/EditorBlueprintResources/StandardMacros.DoOnce` false :!label _label_7
        (:`Completed`
          (`KismetArrayLibrary.Array_Set` (`self.DrawerStateArr`) 3 (not _output_2))
          (if _output_2
            (bind (_direction_4 _translationlerp_2) (`Timeline|Timeline_0` :!via `PlayFromStart` :!label _label_8)
              (:`Update`
                (`SceneComponent.K2_SetRelativeLocation` (`self.SM_Drawer_04`) (`KismetMathLibrary.MakeVector` (`KismetMathLibrary.Lerp` (`self.BeginLocationX`) (`self.OpenAngleL`) _translationlerp_2) _relativelocation_y _relativelocation_z) false false))
              (:`Finished`
                (goto _label_7 :!via `Reset`)))
            (else
              (goto _label_8 :!via `ReverseFromEnd`))))))
    (:`SM_Drawer_05`
      (`/Engine/EditorBlueprintResources/StandardMacros.DoOnce` false :!label _label_9
        (:`Completed`
          (`KismetArrayLibrary.Array_Set` (`self.DrawerStateArr`) 4 (not _output_6))
          (if _output_6
            (bind (_direction_5 _translationlerp_3) (`Timeline|Timeline_2` :!via `PlayFromStart` :!label _label_10)
              (:`Update`
                (`SceneComponent.K2_SetRelativeLocation` (`self.SM_Drawer_05`) (`KismetMathLibrary.MakeVector` (`KismetMathLibrary.Lerp` (`self.BeginLocationX`) (`self.OpenAngleL`) _translationlerp_3) _relativelocation_y_3 _relativelocation_z_3) false false))
              (:`Finished`
                (goto _label_9 :!via `Reset`)))
            (else
              (goto _label_10 :!via `ReverseFromEnd`))))))
    (:`SM_Drawer_06`
      (`/Engine/EditorBlueprintResources/StandardMacros.DoOnce` false :!label _label_11
        (:`Completed`
          (`KismetArrayLibrary.Array_Set` (`self.DrawerStateArr`) 5 (not _output_4))
          (if _output_4
            (bind (_direction_6 _translationlerp_4) (`Timeline|Timeline_4` :!via `PlayFromStart` :!label _label_12)
              (:`Update`
                (`SceneComponent.K2_SetRelativeLocation` (`self.SM_Drawer_06`) (`KismetMathLibrary.MakeVector` (`KismetMathLibrary.Lerp` (`self.BeginLocationX`) (`self.OpenAngleL`) _translationlerp_4) _relativelocation_y_2 _relativelocation_z_2) false false))
              (:`Finished`
                (goto _label_11 :!via `Reset`)))
            (else
              (goto _label_12 :!via `ReverseFromEnd`))))))))

(fn `UserConstructionScript`
  (bind _sm_drawer_03 (`self.SM_Drawer_03`))
  (bind _sm_drawer_04 (`self.SM_Drawer_04`))
  (bind _sm_drawer_05 (`self.SM_Drawer_05`))
  (bind _sm_drawer_06 (`self.SM_Drawer_06`))
  (bind (_relativelocation_x _relativelocation_y _relativelocation_z) (`KismetMathLibrary.BreakVector` (`SceneComponent.RelativeLocation` _sm_drawer_06)))
  (bind (_relativelocation_x_2 _relativelocation_y_2 _relativelocation_z_2) (`KismetMathLibrary.BreakVector` (`SceneComponent.RelativeLocation` _sm_drawer_04)))
  (bind (_relativelocation_x_3 _relativelocation_y_3 _relativelocation_z_3) (`KismetMathLibrary.BreakVector` (`SceneComponent.RelativeLocation` _sm_drawer_05)))
  (bind (_relativelocation_x_4 _relativelocation_y_4 _relativelocation_z_4) (`KismetMathLibrary.BreakVector` (`SceneComponent.RelativeLocation` _sm_drawer_03)))
  (for (_array_element _array_index) (`self.DrawerStateArr`)
    (if _array_element
      (switch `int` _array_index
        (:`0`
          (`SceneComponent.K2_SetRelativeRotation` (`self.SM_Drawer_01`) (`KismetMathLibrary.MakeRotator` 0.0 (`self.OpenAngleR`)) false false))
        (:`1`
          (`SceneComponent.K2_SetRelativeRotation` (`self.SM_Drawer_02`) (`KismetMathLibrary.MakeRotator` 0.0 (`self.OpenAngleR`)) false false))
        (:`2`
          (`SceneComponent.K2_SetRelativeLocation` _sm_drawer_03 (`KismetMathLibrary.MakeVector` (`self.OpenAngleL`) _relativelocation_y_4 _relativelocation_z_4) false false))
        (:`3`
          (`SceneComponent.K2_SetRelativeLocation` _sm_drawer_04 (`KismetMathLibrary.MakeVector` (`self.OpenAngleL`) _relativelocation_y_2 _relativelocation_z_2) false false))
        (:`4`
          (`SceneComponent.K2_SetRelativeLocation` _sm_drawer_05 (`KismetMathLibrary.MakeVector` (`self.OpenAngleL`) _relativelocation_y_3 _relativelocation_z_3) false false))
        (:`5`
          (`SceneComponent.K2_SetRelativeLocation` _sm_drawer_06 (`KismetMathLibrary.MakeVector` (`self.OpenAngleL`) _relativelocation_y _relativelocation_z) false false))))))