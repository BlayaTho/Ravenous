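; BP_Meuble4 is a modular furniture actor, filed under interactables, with optional left and right doors, drawers and glass doors.
; Its Construction Script checks a Has flag for each of these six parts and destroys the matching component when the flag is false.
; The event graph holds only disabled placeholder events, so the Blueprint's graphs add no runtime behavior.
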(fn `UserConstructionScript`
  (`|ExecutionSequence`
    (:`then_0`
      (if (not (`self.bHasLeftDoor`))
        (`ActorComponent.K2_DestroyComponent` (`self.Door_Left`))))
    (:`then_1`
      (if (not (`self.bHasRightDoor`))
        (`ActorComponent.K2_DestroyComponent` (`self.Door_Right`))))
    (:`then_2`
      (if (not (`self.bHasLeftDrawer`))
        (`ActorComponent.K2_DestroyComponent` (`self.Drawer_Left`))))
    (:`then_3`
      (if (not (`self.bHasRightDrawer`))
        (`ActorComponent.K2_DestroyComponent` (`self.Drawer_Right`))))
    (:`then_4`
      (if (not (`self.bHasLeftGlassDoor`))
        (`ActorComponent.K2_DestroyComponent` (`self.GlassDoor_Left`))))
    (:`then_5`
      (if (not (`self.bHasRightGlassDoor`))
        (`ActorComponent.K2_DestroyComponent` (`self.GlassDoor_Right`))))))