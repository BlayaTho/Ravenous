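; BP_Drawer is an interactable furniture drawer or door, with a configurable mesh, that can be locked and can hold a handle or pendulum key.
; BeginPlay attaches those items to the mesh; Interact toggles a timeline, either rotating the mesh or sliding the actor forward with sound.
; DoOnce gates block input mid-animation, and a matching held item is consumed to unlock.
; The slide distance is hardcoded, ignoring the construction script's TranslationValue.
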(event `self.ReceiveBeginPlay`
  (set `self.DefaultLoc` (`self.K2_GetActorLocation`))
  (set `self.DefaultRot` (`self.K2_GetActorRotation`))
  (`|ExecutionSequence`
    (:`then_0`
      (if (`self.bHasHandleInIt`)
        (bind _returnvalue (`AddComponent|NODE_AddChildActorComponent-0` :`bManualAttachment` true :`RelativeTransform` (`KismetMathLibrary.MakeTransform` (15.0 15.0 37.5) (struct :`Yaw` 35.0))))
        (`SceneComponent.K2_AttachToComponent` _returnvalue (`self.StaticMesh`) "None" "KeepRelative" "KeepRelative" "KeepRelative" true)))
    (:`then_1`
      (if (`self.bHasPendulumKeyInIt`)
        (bind _returnvalue_2 (`AddComponent|NODE_AddChildActorComponent-1` :`bManualAttachment` true :`RelativeTransform` (`KismetMathLibrary.MakeTransform` (30.0 6.5 63.5) (struct :`Yaw` 35.0))))
        (`SceneComponent.K2_AttachToComponent` _returnvalue_2 (`self.StaticMesh`) "None" "KeepRelative" "KeepRelative" "KeepRelative" true)))))

(event `/Game/Ravenous/Core/Characters/Interface/BPI_Interaction.Interact`
  (params (ForDoor :type Boolean) (ForLock :type Boolean) (Name :type String) (PlayerRef :type "/Game/Ravenous/Core/Characters/Player/BP_FirstPersonCharacter Object Reference"))
  (bind _helditem (`/Game/Ravenous/Core/Characters/Player/BP_FirstPersonCharacter.HeldItem` PlayerRef))
  (bind (_defaultrot_roll _defaultrot_pitch) (`KismetMathLibrary.BreakRotator` (`self.DefaultRot`)))
  (bind (_defaultrot_roll_2 _defaultrot_pitch_2 _defaultrot_yaw) (`KismetMathLibrary.BreakRotator` (`self.DefaultRot`)))
  (bind _defaultloc (`self.DefaultLoc`))
  (if (not (`self.bIsLock`))
    (if (or (`self.bShouldRotateZ`) (`self.bShouldRotateY`))
      ;[0.05208 0.05208 0.05208] Open / Close Drawer ROTATION
      (`/Engine/EditorBlueprintResources/StandardMacros.DoOnce` false :!label _label
        (:`Completed`
          (`/Engine/EditorBlueprintResources/StandardMacros.FlipFlop`
            (:`A`
              (bind (_direction _lerpvalue) (`Timeline|Timeline` :!via `PlayFromStart` :!label _label_2)
                (:`Update`
                  (if (`self.bShouldRotateY`)
                    (`SceneComponent.K2_SetRelativeRotation` (`self.StaticMesh`) (`KismetMathLibrary.MakeRotator` _defaultrot_roll_2 (`KismetMathLibrary.Lerp` 0.0 (`self.RotationValue`) _lerpvalue) _defaultrot_yaw) false false)
                    (else
                      (`SceneComponent.K2_SetRelativeRotation` (`self.StaticMesh`) (`KismetMathLibrary.MakeRotator` _defaultrot_roll _defaultrot_pitch (`KismetMathLibrary.Lerp` 0.0 -90.0 _lerpvalue)) false false))))
                (:`Finished`
                  (goto _label :!via `Reset`))))
            (:`B`
              (goto _label_2 :!via `ReverseFromEnd`)))))
      (else
        (`/Engine/EditorBlueprintResources/StandardMacros.DoOnce` false :!label _label_3
          (:`Completed`
            ;[0.05208 0.05208 0.05208] Open / Close Drawer TRANSLATION
            ;;[0.09166 0.4458 1] DrawerOpening Sound
            (`GameplayStatics.PlaySoundAtLocation` "/Game/Ravenous/Sound/Drawer/DrawerOpening_Cue.DrawerOpening_Cue" (`self.K2_GetActorLocation`) (struct) 1.0 1.0 0.0 null null null null)
            (`/Engine/EditorBlueprintResources/StandardMacros.FlipFlop`
              (:`A`
                (bind (_direction_2 _lerpvalue_2) (`Timeline|DrawerMovement` :!via `PlayFromStart` :!label _label_4)
                  (:`Update`
                    (`self.K2_SetActorLocation` (`KismetMathLibrary.VLerp` _defaultloc (+ _defaultloc (* (`self.GetActorForwardVector`) 20.0)) _lerpvalue_2)))
                  (:`Finished`
                    (goto _label_3 :!via `Reset`))))
              (:`B`
                (goto _label_4 :!via `ReverseFromEnd`)))))))
    (else
      (`/Engine/EditorBlueprintResources/StandardMacros.IsValid` _helditem
        (:`Is Valid`
          (if (`|EnumEquality` (`/Game/Ravenous/Core/Interactables/Bp_PickableItem.ItemType` _helditem) "NewEnumerator8")
            (`/Game/Ravenous/Core/Characters/Player/BP_FirstPersonCharacter.DestroyHeldItem` PlayerRef)
            (set `self.bIsLock` false)
            (else
              (`KismetSystemLibrary.PrintString` "It's Lock" :!label _label_5))))
        (:`Is Not Valid`
          (goto _label_5))))))

(fn `UserConstructionScript`
  (`StaticMeshComponent.SetStaticMesh` (`self.StaticMesh`) (`self.DrawerMesh`))
  (if (== (`self.DrawerMesh`) "/Game/Ravenous/Art/Salon/Meubles/S_ConsoleTable_/S_ConsoleTable_Drawer_.S_ConsoleTable_Drawer_")
    (set `self.TranslationValue` 15.0)
    (else
      (if (== (`self.DrawerMesh`) "/Game/Ravenous/Assets/DioramaV2/Pendulum/S_Pendulum_Door_.S_Pendulum_Door_")
        _
        (else
          _))
      (set `self.TranslationValue` 25.0))))