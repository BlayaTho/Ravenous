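; BP_MovableObject is an interactable toy prop in Puzzle_02 that moves back and forth between two poses when used.
; The construction script applies the configurable mesh, and Interact plays a rolling sound and alternates a timeline forward and in reverse via FlipFlop.
; The duck mesh slides sideways, while other meshes lift slightly and rotate.
; A DoOnce gate blocks further interaction until the timeline finishes.
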(event `/Game/Ravenous/Core/Characters/Interface/BPI_Interaction.Interact`
  (params (ForDoor :type Boolean) (ForLock :type Boolean) (Name :type String) (PlayerRef :type "/Game/Ravenous/Core/Characters/Player/BP_FirstPersonCharacter Object Reference"))
  (`/Engine/EditorBlueprintResources/StandardMacros.DoOnce` false :!label _label
    (:`Completed`
      (`AudioComponent.Play` (`self.RollingToy_Cue`) 0.0)
      (`/Engine/EditorBlueprintResources/StandardMacros.FlipFlop`
        (:`A`
          (bind (_direction _lerptrans) (`Timeline|Timeline` :!via `PlayFromStart` :!label _label_2)
            (:`Update`
              (if (== (`self.ObjectMesh`) "/Game/Ravenous/Art/Salon/Props/S_Duck_/S_Duck_lp.S_Duck_lp")
                (`SceneComponent.K2_SetRelativeLocation` (`self.Object`) (`KismetMathLibrary.VLerp` (0.0 0.0 0.0) (0.0 35.0 0.0) _lerptrans) false false)
                (else
                  (`SceneComponent.K2_SetRelativeLocationAndRotation` (`self.Object`) (`KismetMathLibrary.VLerp` (0.0 0.0 0.0) (0.0 0.0 1.5) _lerptrans) (`KismetMathLibrary.RLerp` (struct) (struct :`Pitch` 35.0) _lerptrans) false false))))
            (:`Finished`
              (goto _label :!via `Reset`))))
        (:`B`
          (goto _label_2 :!via `ReverseFromEnd`))))))

(fn `UserConstructionScript`
  (`StaticMeshComponent.SetStaticMesh` (`self.Object`) (`self.ObjectMesh`)))