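; BP_Panda is an inspectable panda puzzle object whose two arms are opened to release a tale page.
; Tick shows an arm's prompt widget while that part is touched, and IA_Interact toggles that arm's rotation through FlipFlop-driven timelines gated by resettable DoOnce nodes.
; With both arms open, the interact input swaps TalePage for the paper actor, disables collision and exits inspection.
; EndFunction re-triggers both arm toggles.
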(event `self.ReceiveBeginPlay`
  (bind _relativerotation_roll (`KismetMathLibrary.BreakRotator` (`SceneComponent.RelativeRotation` (`self.ArmD`))))
  (`parent.ReceiveBeginPlay`)
  (set `self.bCanUse` true)
  (set `self.DefaultArmRotation` _relativerotation_roll)
  (set `self.DefaultRot` (`SceneComponent.RelativeRotation` (`self.Item`))))

(event `self.ReceiveTick`
  (params (DeltaSeconds :type "Float (single-precision)"))
  ;[0.05208 0.05208 0.05208] Set Widget Visibility
  (if (`self.TouchInteractebalePart?`)
    (`|ExecutionSequence`
      (:`then_0`
        (if (`KismetStringLibrary.EqualEqual_StrStr` (`self.PartName`) (`KismetSystemLibrary.GetObjectName` (`self.ArmD`)))
          (`SceneComponent.SetHiddenInGame` (`self.WidgetArmD`) false false)))
      (:`then_1`
        (if (`KismetStringLibrary.EqualEqual_StrStr` (`self.PartName`) (`KismetSystemLibrary.GetObjectName` (`self.ArmL`)))
          (`SceneComponent.SetHiddenInGame` (`self.WidgetArmL`) false false))))
    (else
      (`SceneComponent.SetHiddenInGame` (`self.WidgetArmD`) true false)
      (`SceneComponent.SetHiddenInGame` (`self.WidgetArmL`) true false))))

(event `EnhancedInput|/Game/Ravenous/Core/Characters/Player/Input/Actions/Player/IA_Interact`
  (params (ActionValue :type Boolean) (ElapsedSeconds :type "Float (double-precision)") (TriggeredSeconds :type "Float (double-precision)") (InputAction :type "InputAction Object Reference" :default "/Game/Ravenous/Core/Characters/Player/Input/Actions/Player/IA_Interact.IA_Interact"))
  (:`Started`
    (`|ExecutionSequence`
      (:`then_0`
        (if (`self.TouchInteractebalePart?`)
          (`|ExecutionSequence`
            (:`then_0`
              (if (`KismetStringLibrary.EqualEqual_StrStr` (`self.PartName`) (`KismetSystemLibrary.GetObjectName` (`self.ArmD`)))
                (`/Engine/EditorBlueprintResources/StandardMacros.DoOnce` false :!label _label
                  (:`Completed`
                    (`/Engine/EditorBlueprintResources/StandardMacros.FlipFlop` :!label _label_2
                      (:`A`
                        (set `self.bIsArmDOpen` true)
                        (bind (_direction _lerp) (`Timeline|Timeline` :!via `PlayFromStart` :!label _label_3)
                          (:`Update`
                            (`SceneComponent.K2_SetRelativeRotation` (`self.ArmD`) (`KismetMathLibrary.MakeRotator` (`KismetMathLibrary.Lerp` (`self.DefaultArmRotation`) -25.0 _lerp)) false false))
                          (:`Finished`
                            (switch `ETimelineDirection` _direction
                              (:`Forward`
                                (set `self.bIsArmDOpen` true)
                                (goto _label :!via `Reset`))
                              (:`Backward`
                                (set `self.bIsArmDOpen` false)
                                (goto _label :!via `Reset`))))))
                      (:`B`
                        (set `self.bIsArmDOpen` false)
                        (goto _label_3 :!via `ReverseFromEnd`)))))))
            (:`then_1`
              (if (`KismetStringLibrary.EqualEqual_StrStr` (`self.PartName`) (`KismetSystemLibrary.GetObjectName` (`self.ArmL`)))
                (`/Engine/EditorBlueprintResources/StandardMacros.DoOnce` false :!label _label_4
                  (:`Completed`
                    (`/Engine/EditorBlueprintResources/StandardMacros.FlipFlop` :!label _label_5
                      (:`A`
                        (set `self.bIsArmLOpen` true)
                        (bind (_direction_2 _lerp_2) (`Timeline|Timeline_0` :!via `PlayFromStart` :!label _label_6)
                          (:`Update`
                            (`SceneComponent.K2_SetRelativeRotation` (`self.ArmL`) (`KismetMathLibrary.MakeRotator` (`KismetMathLibrary.Lerp` (`self.DefaultArmRotation`) -25.0 _lerp_2)) false false))
                          (:`Finished`
                            (switch `ETimelineDirection` _direction_2
                              (:`Forward`
                                (set `self.bIsArmLOpen` true)
                                (goto _label_4 :!via `Reset`))
                              (:`Backward`
                                (set `self.bIsArmLOpen` false)
                                (goto _label_4 :!via `Reset`))))))
                      (:`B`
                        (set `self.bIsArmLOpen` false)
                        (goto _label_6 :!via `ReverseFromEnd`))))))))))
      (:`then_1`
        (if (and (`self.bIsArmDOpen`) (`self.bIsArmLOpen`))
          (`/Engine/EditorBlueprintResources/StandardMacros.DoOnce` false
            (:`Completed`
              (set `self.bIsPaperPicked` false)
              (`Widget.RemoveFromParent` (`self.W_PickUp`))
              (set `Widget.Visibility` "Visible" (`self.W_input`))
              (`self.K2_SetActorLocation` (`self.PaperRef`) (`SceneComponent.K2_GetComponentLocation` (`self.TalePage`)) false false)
              (`self.K2_AttachToComponent` (`self.PaperRef`) (`self.Item`) "None" "KeepWorld" "KeepRelative" "KeepRelative" true)
              (`ActorComponent.K2_DestroyComponent` (`self.TalePage`))
              (`KismetSystemLibrary.Delay` 0.2)
              (`self.SetActorEnableCollision` false)
              (set `self.bCanUse` false)
              (`self.ExitObject`))))))))

(event `EndFunction`
  (`|ExecutionSequence`
    (:`then_0`
      (goto _label :!via `Reset`))
    (:`then_1`
      (goto _label_2))
    (:`then_2`
      (goto _label_4 :!via `Reset`))
    (:`then_3`
      (goto _label_5))))

(fn `UserConstructionScript`
  (`parent.UserConstructionScript`))