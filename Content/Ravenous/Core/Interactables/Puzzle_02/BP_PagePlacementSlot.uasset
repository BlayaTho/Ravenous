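; Page placement slot for Puzzle 02 that checks whether the correct pickable item sits in it.
; Box overlaps filter by item type, compare DefaultValue to RightValue and report to CodeDisplayerRef, ignoring new placements while it displays.
; Removing the last detected item, matched by display name, spawns a scaled-down BP_NoneItem and clears the slot's correct state.
; A player trigger toggles the close-range widget, which Tick hides during code display.
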(event `self.ReceiveTick`
  (params (DeltaSeconds :type "Float (single-precision)"))
  (if (`/Game/Ravenous/Core/Interactables/Puzzle_02/BP_CodeDisplayer.bIsDisplaying` (`self.CodeDisplayerRef`))
    (`SceneComponent.SetHiddenInGame` (`self.W_CloseRange`) true false)))

(event `self.Box.OnComponentBeginOverlap`
  (params (OverlappedComponent :type "PrimitiveComponent Object Reference") (OtherActor :type "Actor Object Reference") (OtherComp :type "PrimitiveComponent Object Reference") (OtherBodyIndex :type Integer) (bFromSweep :type Boolean) (SweepResult :type "HitResult Structure (by ref)"))
  (bind _asbp_pickable_item (cast `/Game/Ravenous/Core/Interactables/Bp_PickableItem` OtherActor))
  (if (`|EnumEquality` (`/Game/Ravenous/Core/Interactables/Bp_PickableItem.ItemType` _asbp_pickable_item) "NewEnumerator2")
    (if (not (`/Game/Ravenous/Core/Interactables/Puzzle_02/BP_CodeDisplayer.bIsDisplaying` (`self.CodeDisplayerRef`)))
      (`/Game/Ravenous/Core/Interactables/Puzzle_02/BP_CodeDisplayer.SetRightSlot` (`self.CodeDisplayerRef`) (`self.RightValue`) (== (`/Game/Ravenous/Core/Interactables/Bp_PickableItem.DefaultValue` _asbp_pickable_item) (`self.RightValue`))))))

(event `self.Box.OnComponentEndOverlap`
  (params (OverlappedComponent :type "PrimitiveComponent Object Reference") (OtherActor :type "Actor Object Reference") (OtherComp :type "PrimitiveComponent Object Reference") (OtherBodyIndex :type Integer))
  (bind _asbp_pickable_item (cast `/Game/Ravenous/Core/Interactables/Bp_PickableItem` OtherActor))
  (if (`|EnumEquality` (`/Game/Ravenous/Core/Interactables/Bp_PickableItem.ItemType` _asbp_pickable_item) "NewEnumerator2")
    (if (`KismetStringLibrary.EqualEqual_StrStr` (`KismetSystemLibrary.GetDisplayName` (stale `self.Box.OnComponentBeginOverlap` _asbp_pickable_item)) (`KismetSystemLibrary.GetDisplayName` _asbp_pickable_item))
      (bind _returnvalue (`|SpawnActorFromClass` "/Game/Ravenous/Core/Interactables/Puzzle_02/BP_NoneItem.BP_NoneItem_C" (`KismetMathLibrary.MakeTransform` (`self.K2_GetActorLocation`)) "Undefined" "MultiplyWithRoot" null null))
      (`self.SetActorScale3D` _returnvalue (0.4 0.4 0.4))
      (`/Game/Ravenous/Core/Interactables/Puzzle_02/BP_CodeDisplayer.SetRightSlot` (`self.CodeDisplayerRef`) (`self.RightValue`) false))))

(event `self.PlayerDetect.OnComponentBeginOverlap`
  (params (OverlappedComponent :type "PrimitiveComponent Object Reference") (OtherActor :type "Actor Object Reference") (OtherComp :type "PrimitiveComponent Object Reference") (OtherBodyIndex :type Integer) (bFromSweep :type Boolean) (SweepResult :type "HitResult Structure (by ref)"))
  (cast `/Game/Ravenous/Core/Characters/Player/BP_FirstPersonCharacter` OtherActor)
  (`SceneComponent.SetVisibility` (`self.W_CloseRange`) true false))

(event `self.PlayerDetect.OnComponentEndOverlap`
  (params (OverlappedComponent :type "PrimitiveComponent Object Reference") (OtherActor :type "Actor Object Reference") (OtherComp :type "PrimitiveComponent Object Reference") (OtherBodyIndex :type Integer))
  (cast `/Game/Ravenous/Core/Characters/Player/BP_FirstPersonCharacter` OtherActor)
  (`SceneComponent.SetVisibility` (`self.W_CloseRange`) false false))

(fn `UserConstructionScript`)