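; BP_NoneItem is a Puzzle_02 interactable that passes itself to the player's SetHandleItem when used with a qualifying held item.
; Interact checks the player's HeldItem and, when HasBlackList is set, proceeds only if its type equals WhiteListedItem, so that flag acts as a whitelist.
; BeginPlay creates a W_LucyDialogue widget, stores it as WText and adds it to the viewport.
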(event `self.ReceiveBeginPlay`
  (bind _returnvalue (`|CreateWidget` "/Game/Ravenous/UI/Widgets/W_LucyDialogue.W_LucyDialogue_C"))
  (bind _output_get (set `self.W_Text` _returnvalue))
  (`UserWidget.AddToViewport` _output_get 0))

(event `/Game/Ravenous/Core/Characters/Interface/BPI_Interaction.Interact`
  (params (ForDoor :type Boolean) (ForLock :type Boolean) (Name :type String) (PlayerRef :type "/Game/Ravenous/Core/Characters/Player/BP_FirstPersonCharacter Object Reference"))
  (bind _helditem (`/Game/Ravenous/Core/Characters/Player/BP_FirstPersonCharacter.HeldItem` PlayerRef))
  (if (not (== _helditem null))
    (if (`self.bHasBlackList`)
      (if (`|EnumEquality` (`/Game/Ravenous/Core/Interactables/Bp_PickableItem.ItemType` _helditem) (`self.WhiteListedItem`))
        (bind _output_get (set `self.Player_Ref` PlayerRef :!label _label))
        (`/Game/Ravenous/Core/Characters/Player/BP_FirstPersonCharacter.SetHandleItem` _output_get self))
      (else
        (goto _label)))))

(fn `UserConstructionScript`)