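; BP_PlacementSlot is a puzzle slot that checks items placed in its box trigger for a linked chest.
; While the chest is closed, an overlapping pickable of the required type reports whether its value matches the slot's RightValue, which also serves as the slot index.
; When the last overlapped item leaves, identified by display name, the slot spawns a scaled-down BP_NoneItem at its own location.
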(event `self.Box.OnComponentBeginOverlap`
  (params (OverlappedComponent :type "PrimitiveComponent Object Reference") (OtherActor :type "Actor Object Reference") (OtherComp :type "PrimitiveComponent Object Reference") (OtherBodyIndex :type Integer) (bFromSweep :type Boolean) (SweepResult :type "HitResult Structure (by ref)"))
  (bind _asbp_pickable_item (cast `/Game/Ravenous/Core/Interactables/BP_PickableItem` OtherActor))
  (if (`|EnumEquality` (`/Game/Ravenous/Core/Interactables/BP_PickableItem.ItemType` _asbp_pickable_item) "NewEnumerator2")
    (if (not (`/Game/Ravenous/Core/Interactables/Puzzle_02/BP_Chest.bIsOpen` (`self.ChestRef`)))
      (bind _returnvalue (== (`/Game/Ravenous/Core/Interactables/BP_PickableItem.DefaultValue` _asbp_pickable_item) (`self.RightValue`)))
      (if _returnvalue
        _
        (else
          _))
      (`/Game/Ravenous/Core/Interactables/Puzzle_02/BP_Chest.SetRightSlot` (`self.ChestRef`) (`self.RightValue`) _returnvalue))))

(event `self.Box.OnComponentEndOverlap`
  (params (OverlappedComponent :type "PrimitiveComponent Object Reference") (OtherActor :type "Actor Object Reference") (OtherComp :type "PrimitiveComponent Object Reference") (OtherBodyIndex :type Integer))
  (bind _asbp_pickable_item (cast `/Game/Ravenous/Core/Interactables/BP_PickableItem` OtherActor))
  (if (`|EnumEquality` (`/Game/Ravenous/Core/Interactables/BP_PickableItem.ItemType` _asbp_pickable_item) "NewEnumerator2")
    (if (`KismetStringLibrary.EqualEqual_StrStr` (`KismetSystemLibrary.GetDisplayName` (stale `self.Box.OnComponentBeginOverlap` _asbp_pickable_item)) (`KismetSystemLibrary.GetDisplayName` _asbp_pickable_item))
      (bind _returnvalue (`|SpawnActorFromClass` "/Game/Ravenous/Core/Interactables/Puzzle_02/BP_NoneItem.BP_NoneItem_C" (`KismetMathLibrary.MakeTransform` (`self.K2_GetActorLocation`)) "Undefined" "MultiplyWithRoot" null null))
      (`self.SetActorScale3D` _returnvalue (0.4 0.4 0.4)))))

(fn `UserConstructionScript`)