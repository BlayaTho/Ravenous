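; BP_TailPage is an interactable page item in Puzzle 02 that the player can pick up while its linked chest is closed.
; On Interact, it stores the player reference and, if the player holds no valid item, spawns an actor at the page's location.
; It then passes itself to the player's SetHandleItem, whether or not an item was held.
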(event `/Game/Ravenous/Core/Characters/Interface/BPI_Interaction.Interact`
  (params (ForDoor :type Boolean) (ForLock :type Boolean) (Name :type String) (PlayerRef :type "/Game/Ravenous/Core/Characters/Player/BP_FirstPersonCharacter Object Reference"))
  (if (not (`/Game/Ravenous/Core/Interactables/Puzzle_02/BP_Chest.bIsOpen` (`self.ChestRef`)))
    (bind _output_get (set `self.Player Ref` PlayerRef))
    (`/Engine/EditorBlueprintResources/StandardMacros.IsValid` (`/Game/Ravenous/Core/Characters/Player/BP_FirstPersonCharacter.HeldItem` _output_get)
      (:`Is Valid`
        _)
      (:`Is Not Valid`
        (`|SpawnActorFromClass` "/Game/Ravenous/Core/Interactables/Puzzle_02/BP_NoneItem.BP_NoneItem_C" (`KismetMathLibrary.MakeTransform` (`self.K2_GetActorLocation`)) "Undefined" "MultiplyWithRoot" null null)))
    (`/Game/Ravenous/Core/Characters/Player/BP_FirstPersonCharacter.SetHandleItem` _output_get self)))

(fn `UserConstructionScript`)