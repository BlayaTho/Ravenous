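; Puzzle 02 interactable drawer with two hinged doors that stays locked until the player interacts while holding a drawer handle item.
; Unlocking destroys the held handle and clears the closed state, so later interactions can move the doors.
; The interacted component's name selects the left or right door, each toggled by a FlipFlop-driven timeline that lerps its yaw in mirrored directions.
; A DoOnce per door blocks input until its timeline finishes.
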(event `/Game/Ravenous/Core/Characters/Interface/BPI_Interaction.Interact`
  (params (ForDoor :type Boolean) (ForLock :type Boolean) (Name :type String) (PlayerRef :type "/Game/Ravenous/Core/Characters/Player/BP_FirstPersonCharacter Object Reference"))
  (set `self.Player Ref` PlayerRef)
  (if (`self.bIsClosed`)
    (if (== (`GameplayStatics.GetObjectClass` (`/Game/Ravenous/Core/Characters/Player/BP_FirstPersonCharacter.HeldItem` (`self.Player Ref`))) "/Game/Ravenous/Core/Interactables/Puzzle_02/BP_DrawerHandle.BP_DrawerHandle_C")
      (set `self.bIsClosed` false)
      (`/Game/Ravenous/Core/Characters/Player/BP_FirstPersonCharacter.DestroyHeldItem` (`self.Player Ref`)))
    (else
      (`|ExecutionSequence`
        (:`then_0`
          (if (`KismetStringLibrary.EqualEqual_StrStr` Name (`KismetSystemLibrary.GetObjectName` (`self.SM_RightDoor`)))
            (`/Engine/EditorBlueprintResources/StandardMacros.DoOnce` false :!label _label
              (:`Completed`
                (`/Engine/EditorBlueprintResources/StandardMacros.FlipFlop`
                  (:`A`
                    (bind (_direction _rotationlerp) (`Timeline|Timeline` :!via `PlayFromStart` :!label _label_2)
                      (:`Update`
                        (`SceneComponent.K2_SetRelativeRotation` (`self.SM_RightDoor`) (`KismetMathLibrary.MakeRotator` 0.0 0.0 (`KismetMathLibrary.Lerp` 0.0 (* (`self.RotationValue`) -1.0) _rotationlerp)) false false))
                      (:`Finished`
                        (goto _label :!via `Reset`))))
                  (:`B`
                    (goto _label_2 :!via `ReverseFromEnd`)))))))
        (:`then_1`
          (if (`KismetStringLibrary.EqualEqual_StrStr` Name (`KismetSystemLibrary.GetObjectName` (`self.SM_LeftDoor`)))
            (`/Engine/EditorBlueprintResources/StandardMacros.DoOnce` false :!label _label_3
              (:`Completed`
                (`/Engine/EditorBlueprintResources/StandardMacros.FlipFlop`
                  (:`A`
                    (bind (_direction_2 _rotationlerp_2) (`Timeline|Timeline_0` :!via `PlayFromStart` :!label _label_4)
                      (:`Update`
                        (`SceneComponent.K2_SetRelativeRotation` (`self.SM_LeftDoor`) (`KismetMathLibrary.MakeRotator` 0.0 0.0 (`KismetMathLibrary.Lerp` 0.0 (`self.RotationValue`) _rotationlerp_2)) false false))
                      (:`Finished`
                        (goto _label_3 :!via `Reset`))))
                  (:`B`
                    (goto _label_4 :!via `ReverseFromEnd`)))))))))))

(fn `UserConstructionScript`)