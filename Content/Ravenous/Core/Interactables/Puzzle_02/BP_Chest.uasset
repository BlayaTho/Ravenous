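; BP_Chest is a puzzle chest in Puzzle_02 that opens when every slot is marked as correctly filled.
; SetRightSlot writes one entry in the IsAtRightSlot boolean array, then re-checks the whole array, stopping at the first false value.
; When all entries are true it sets IsOpen and plays a timeline that lerps DefaultSceneRoot1's roll to swing it open.
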(event `SetRightSlot`
  (params (Index :type Integer) (NewValue :type Boolean))
  (`KismetArrayLibrary.Array_Set` (`self.bIsAtRightSlot`) Index NewValue)
  (`self.CheckIfShouldOpen`))

(event `CheckIfShouldOpen`
  (for _array_element (`self.bIsAtRightSlot`)
    (if _array_element
      (set `self.bIsAllGood` true)
      (else
        (set `self.bIsAllGood` false)
        (break))))
  (if (`self.bIsAllGood`)
    (set `self.bIsOpen` true)
    (`self.OpenChest`)
    (else
      (set `self.bIsOpen` false))))

(event `OpenChest`
  (if (`self.bIsOpen`)
    (bind (_direction _openinglerp) (`Timeline|Timeline`)
      (:`Update`
        (`SceneComponent.K2_SetRelativeRotation` (`self.DefaultSceneRoot1`) (`KismetMathLibrary.MakeRotator` (`KismetMathLibrary.Lerp` 0.0 50.0 _openinglerp)) false false)))))

(fn `UserConstructionScript`)