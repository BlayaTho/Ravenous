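; BP_NavLink is a smart nav link that lets AI open an associated door when reaching it.
; On SmartLinkReached, it skips doors already completely open, otherwise calling OpenDoorCompletely on the Door reference with the AI flag set.
; A dot product of link and door forward vectors picks the swing direction, using a loose tolerance around opposite facing.
; Both open-state branches print debug strings.
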(event `self.ReceiveSmartLinkReached`
  (params (Agent :type "Actor Object Reference") (Destination :type "Vector Structure (by ref)"))
  (bind _door (`self.door`))
  (bind _door_2 (`self.door`))
  (if (`/Game/Ravenous/Core/Interactables/BP_Door.DoorCompletelyOpen` _door)
    (`KismetSystemLibrary.PrintString` "Porte Deja ouverte")
    (else
      (`KismetSystemLibrary.PrintString` "ZEBI")
      (if (`KismetMathLibrary.NearlyEqual_FloatFloat` (`KismetMathLibrary.Dot_VectorVector` (`self.GetActorForwardVector`) (`self.GetActorForwardVector` _door)) -1.0 0.65)
        (`/Game/Ravenous/Core/Interactables/BP_Door.OpenDoorCompletely` _door_2 false true)
        (else
          (`/Game/Ravenous/Core/Interactables/BP_Door.OpenDoorCompletely` _door_2 true true))))))

(fn `UserConstructionScript`)