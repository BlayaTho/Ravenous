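; Test AI pawn Blueprint that wanders endlessly between TargetPoint actors placed in the level.
; The construction script caches every TargetPoint in the level into an array.
; From BeginPlay, MoveIA sends the pawn to a random cached point with AI MoveTo, then waits a fixed delay and calls itself again, whether the move succeeds or fails.
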(event `self.ReceiveBeginPlay`
  (`self.MoveIA`))

(event `MoveIA`
  (`|AIMoveTo` self (`self.K2_GetActorLocation` (`KismetArrayLibrary.Array_Random` (`self.TargetPoints`))) null
    (:`OnSuccess`
      _)
    (:`OnFail`
      _))
  (`KismetSystemLibrary.Delay` 4.0)
  (`self.MoveIA`))

(fn `UserConstructionScript`
  (`KismetArrayLibrary.Array_Clear` (`self.TargetPoints`))
  (bind _outactors (`GameplayStatics.GetAllActorsOfClass` "/Script/Engine.TargetPoint"))
  (set `self.TargetPoints` _outactors))