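; Rawr is a sitting monster AI that turns red and chases the player, despawns when the player hides out of sight, and prints a death message on contact.
; PawnSensing sightings build tolerance until it triggers aggression, or trigger it immediately through a gate opened by close-radius overlap.
; ChasePlayer re-issues AIMoveTo toward the player or their hideout point.
; While standing, Tick sphere-traces to the player to track visibility.
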(event `self.CloseDetectionRadius.OnComponentBeginOverlap`
  (params (OverlappedComponent :type "PrimitiveComponent Object Reference") (OtherActor :type "Actor Object Reference") (OtherComp :type "PrimitiveComponent Object Reference") (OtherBodyIndex :type Integer) (bFromSweep :type Boolean) (SweepResult :type "HitResult Structure (by ref)"))
  ;[0.1146 0.1146 0.1146] Attack If Player Is Too Close
  (cast `/Game/Ravenous/Core/Characters/Player/BP_FirstPersonCharacter` OtherActor)
  (goto _label :!via `Open`))

(event `self.PawnSensing.OnSeePawn`
  (params (Pawn :type "Pawn Object Reference"))
  (bind _asbp_first_person_character (cast `/Game/Ravenous/Core/Characters/Player/BP_FirstPersonCharacter` Pawn))
  (set `self.PlayerRef` _asbp_first_person_character)
  (set `self.bIsSeeingPlayer` true)
  (`|ExecutionSequence`
    (:`then_0`
      ;[0.1146 0.1146 0.1146] Attack If Player Is Too Close
      (`/Engine/EditorBlueprintResources/StandardMacros.Gate` true :!label _label
        (:`Exit`
          ;;[1 0 0] Add Scream + Stand Up Anim
          (`/Engine/EditorBlueprintResources/StandardMacros.DoOnce` false
            (:`Completed`
              (`MeshComponent.SetVectorParameterValueOnMaterials` (`self.Mesh`) "Color" (1.0 0.0 0.0))
              (set `self.bIsSitting` false)
              (`self.ChasePlayer`))))))
    (:`then_1`
      (if (== (`self.ToleranceValue`) 100.0)
        (`|ExecutionSequence`
          (:`then_0`
            (if (`self.bIsSitting`)
              ;[1 0 0] Add Scream + Stand Up Anim
              (`/Engine/EditorBlueprintResources/StandardMacros.DoOnce` false
                (:`Completed`
                  (`MeshComponent.SetVectorParameterValueOnMaterials` (`self.Mesh`) "Color" (1.0 0.0 0.0))
                  (`KismetSystemLibrary.Delay` 5.0)
                  (if (`|EnumEquality` (`/Game/Ravenous/Core/Characters/Player/BP_FirstPersonCharacter.MobilityState` (`self.PlayerRef`)) "NewEnumerator0")
                    (`self.AIDispawn`)
                    (else
                      (set `self.bIsSitting` false)
                      (`self.ChasePlayer`)))))))
          (:`then_1`
            (if (`|EnumEquality` (`/Game/Ravenous/Core/Characters/Player/BP_FirstPersonCharacter.MobilityState` (`self.PlayerRef`)) "NewEnumerator0")
              (`KismetSystemLibrary.PrintString` "Hello")
              (`self.ChasePlayer`))))
        (else
          (set `self.ToleranceValue` (`KismetMathLibrary.FClamp` (+ (`self.ToleranceValue`) 10.0) 0.0 100.0))
          (`KismetSystemLibrary.PrintString` "Rawr is being See"))))))

(event `AIDispawn`
  ;[0.1146 0.1146 0.1146] Dispawn
  (`KismetSystemLibrary.PrintString` "Rawr DESPAWN" true true (struct :`G` 1.0 :`B` 0.382696 :`A` 1.0))
  (`self.K2_DestroyActor`))

(event `self.ReceiveBeginPlay`)

(event `self.ReceiveTick`
  (params (DeltaSeconds :type "Float (single-precision)"))
  (bind _returnvalue (`self.K2_GetActorLocation` (`self.PlayerRef`)))
  (if (not (`self.bIsSitting`))
    (`|ExecutionSequence`
      (:`then_0`
        (bind (_outhits _returnvalue_2) (`KismetSystemLibrary.SphereTraceMulti` :`Start` (`self.K2_GetActorLocation`) :`End` _returnvalue :`Radius` 5.0 :`TraceChannel` "TraceTypeQuery4" :`DrawDebugType` "ForDuration"))
        (if _returnvalue_2
          (`/Engine/EditorBlueprintResources/StandardMacros.DoOnce` false :!label _label_2
            (:`Completed`
              (set `self.bIsSeeingPlayer` false)
              (set `self.LastVisibleLocation` _returnvalue)))
          (else
            (`|ExecutionSequence`
              (:`then_0`
                (goto _label_2 :!via `Reset`))
              (:`then_1`
                (set `self.bIsSeeingPlayer` true))))))
      (:`then_1`
        ;[0.1146 0.1146 0.1146] Dispawn AI If Player Is HIde And Not See
        (if (and (not (`self.bIsSeeingPlayer`)) (`|EnumEquality` (`/Game/Ravenous/Core/Characters/Player/BP_FirstPersonCharacter.MobilityState` (`self.PlayerRef`)) "NewEnumerator0"))
          (`self.AIDispawn`))))))

(event `ChasePlayer`
  (if (`|EnumEquality` (`/Game/Ravenous/Core/Characters/Player/BP_FirstPersonCharacter.MobilityState` (`self.PlayerRef`)) "NewEnumerator0")
    (`|AIMoveTo` self (`/Game/Ravenous/Core/Characters/Player/BP_FirstPersonCharacter.HideOutPointRef` (`self.PlayerRef`)) null
      (:`OnSuccess`
        _)
      (:`OnFail`
        _))
    (`self.ChasePlayer`)
    (else
      (`KismetSystemLibrary.PrintString` "Rawr is Chasing")
      (`|AIMoveTo` self (0.0 0.0 0.0) (`self.PlayerRef`)
        (:`OnSuccess`
          _)
        (:`OnFail`
          _))
      (`self.ChasePlayer`))))

(event `self.CapsuleComponent.OnComponentHit`
  (params (HitComponent :type "PrimitiveComponent Object Reference") (OtherActor :type "Actor Object Reference") (OtherComp :type "PrimitiveComponent Object Reference") (NormalImpulse :type "Vector Structure") (Hit :type "HitResult Structure (by ref)"))
  ;[0.1146 0.1146 0.1146] Hit Player
  (cast `/Game/Ravenous/Core/Characters/Player/BP_FirstPersonCharacter` OtherActor)
  (`KismetSystemLibrary.PrintString` "DEAD" true true (struct :`R` 1.0 :`A` 1.0)))

(fn `UserConstructionScript`)