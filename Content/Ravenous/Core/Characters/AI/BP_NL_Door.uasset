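; BP_NL_Door is a smart nav link that opens its referenced door when an AI agent reaches it.
; If the door is not completely open, it compares agent and door forward vectors with a dot product.
; Roughly opposed facing opens the door completely with the Back flag set, otherwise without it, both flagged as AI-triggered.
; An already open door only prints a debug string.
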(event `self.ReceiveSmartLinkReached`
  (params (Agent :type "Actor Object Reference") (Destination :type "Vector Structure (by ref)"))
  (bind _doorref (`self.DoorRef`))
  (bind _doorref_2 (`self.DoorRef`))
  (if (`/Game/Ravenous/Core/Interactables/BP_Door.bIsDoorCompletelyOpen` _doorref)
    (`KismetSystemLibrary.PrintString` "Porte Deja ouverte")
    (else
      (`KismetSystemLibrary.PrintString` "ZEBI")
      (if (`KismetMathLibrary.NearlyEqual_FloatFloat` (`KismetMathLibrary.Dot_VectorVector` (`self.GetActorForwardVector` Agent) (`self.GetActorForwardVector` _doorref)) -1.0 0.65)
        (`/Game/Ravenous/Core/Interactables/BP_Door.OpenDoorCompletely` _doorref_2 true true)
        (else
          (`/Game/Ravenous/Core/Interactables/BP_Door.OpenDoorCompletely` _doorref_2 false true))))))

(fn `UserConstructionScript`)