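; BP_Pendulum is an environment prop that continuously swings its pendulum weight from side to side.
; From BeginPlay, the SecondMovement timeline lerps the weight's relative roll from LastPos to NextPos.
; When each swing finishes, it stores the current roll, a FlipFlop alternates the target between small positive and negative angles, and the Seconds event calls itself to restart the timeline.
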(event `self.ReceiveBeginPlay`
  (`self.Seconds`))

(event `Seconds`
  (bind _relativerotation_roll (`KismetMathLibrary.BreakRotator` (`SceneComponent.RelativeRotation` (`self.S_PendulumWeight_`))))
  (bind (_direction _leprot) (`Timeline|SecondMovement` :!via `PlayFromStart`)
    (:`Update`
      (`SceneComponent.K2_SetRelativeRotation` (`self.S_PendulumWeight_`) (`KismetMathLibrary.MakeRotator` (`KismetMathLibrary.Lerp` (`self.LastPos`) (`self.NextPos`) _leprot)) false false))
    (:`Finished`
      (set `self.LastPos` _relativerotation_roll)
      (`/Engine/EditorBlueprintResources/StandardMacros.FlipFlop`
        (:`A`
          (set `self.NextPos` 3.0))
        (:`B`
          (set `self.NextPos` -3.0)))
      (`self.Seconds`))))

(fn `UserConstructionScript`)