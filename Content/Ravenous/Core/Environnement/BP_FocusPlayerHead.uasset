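; BP_FocusPlayerHead is a creepy plastic baby head prop that keeps turning to face the player.
; Tick sets the mesh's yaw from a look-at rotation toward the cached first-person character, with a fixed roll and yaw offset.
; On BeginPlay, after a one-tick delay, the CryingDemon and CryingDemonIntense flags choose which crying demon audio cue plays, if any.
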(event `self.ReceiveBeginPlay`
  (bind _womancrying_demon_cue (`self.WomanCrying_Demon_Cue`))
  (bind _womancrying_demonintense_cue (`self.WomanCrying_DemonIntense_Cue`))
  (`AudioComponent.Stop` _womancrying_demon_cue)
  (`AudioComponent.Stop` _womancrying_demonintense_cue)
  (bind _asbp_first_person_character (cast `/Game/Ravenous/Core/Characters/Player/BP_FirstPersonCharacter` (`GameplayStatics.GetPlayerCharacter` 0)))
  (set `self.Player_Ref` _asbp_first_person_character)
  (`KismetSystemLibrary.DelayUntilNextTick`)
  (if (`self.CryingDemon?`)
    (`AudioComponent.Play` _womancrying_demon_cue 0.0)
    (elif (`self.CryingDemonIntense?`)
      (`AudioComponent.Play` _womancrying_demonintense_cue 0.0))))

(event `self.ReceiveTick`
  (params (DeltaSeconds :type "Float (single-precision)"))
  (bind (_returnvalue_roll _returnvalue_pitch _returnvalue_yaw) (`KismetMathLibrary.BreakRotator` (`KismetMathLibrary.FindLookAtRotation` (`SceneComponent.K2_GetComponentLocation` (`self.S_PlasticBaby_Head_29_StaticMeshComponent0`)) (`self.K2_GetActorLocation` (`self.Player_Ref`)))))
  (`SceneComponent.K2_SetRelativeRotation` (`self.S_PlasticBaby_Head_29_StaticMeshComponent0`) (`KismetMathLibrary.MakeRotator` -180.0 0.0 (+ _returnvalue_yaw 90.0)) false false))

(fn `UserConstructionScript`)