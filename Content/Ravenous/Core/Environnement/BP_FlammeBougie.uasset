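; Candle prop Blueprint with a billboard flame, offered in long, mid and small sizes.
; The construction script uses two booleans to pick the mesh and flame height, building the mid size from the long mesh squashed vertically.
; It then randomizes the mesh yaw and chooses between two flame materials, varying candles whenever construction runs.
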(fn `UserConstructionScript`
  (bind _staticmesh (`self.StaticMesh`))
  (bind _materialbillboard (`self.MaterialBillboard`))
  (bind _materialbillboard_2 (`self.MaterialBillboard`))
  (`|ExecutionSequence`
    (:`then_0`
      (if (`self.bCandleLong`)
        (`StaticMeshComponent.SetStaticMesh` _staticmesh "/Game/Ravenous/Art/Salon/Props/S_CandleLong_/S_CandleLong_lp.S_CandleLong_lp")
        (`SceneComponent.K2_SetRelativeLocation` _materialbillboard (0.0 0.0 18.0) false false)
        (elif (`self.bCandleMid`)
          (`StaticMeshComponent.SetStaticMesh` _staticmesh "/Game/Ravenous/Art/Salon/Props/S_CandleLong_/S_CandleLong_lp.S_CandleLong_lp")
          (`SceneComponent.SetRelativeScale3D` _staticmesh (1.0 1.0 0.75))
          (`SceneComponent.K2_SetRelativeLocation` _materialbillboard (0.0 0.0 14.0) false false)
          (else
            (`StaticMeshComponent.SetStaticMesh` _staticmesh "/Game/Ravenous/Art/Salon/Props/S_Candle_Small_/S_CandleSmall_lp.S_CandleSmall_lp")
            (`SceneComponent.K2_SetRelativeLocation` _materialbillboard (0.0 0.0 8.5) false false)))))
    (:`then_1`
      (`SceneComponent.K2_SetRelativeRotation` (`self.StaticMesh`) (`KismetMathLibrary.MakeRotator` 0.0 0.0 (`KismetMathLibrary.RandomFloatInRange` 0.0 360.0)) false false)
      (if (`KismetMathLibrary.RandomBool`)
        (`PrimitiveComponent.SetMaterial` _materialbillboard_2 0 "/Game/Ravenous/Assets/Materials/M_Flame.M_Flame")
        (else
          (`PrimitiveComponent.SetMaterial` _materialbillboard_2 0 "/Game/Ravenous/Assets/Materials/M_Flame_Inst.M_Flame_Inst"))))))