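; BP_EnviroPhone is an environment phone prop whose two eyes follow the player.
; BeginPlay caches the first-person player character.
; Every tick, each eye computes a look-at rotation to the player and applies it as relative rotation, subtracting the actor's yaw and a fixed offset from the yaw to compensate for orientation.
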(event `self.ReceiveBeginPlay`
  (bind _asbp_first_person_character (cast `/Game/Ravenous/Core/Characters/Player/BP_FirstPersonCharacter` (`GameplayStatics.GetPlayerCharacter` 0)))
  (set `self.PlayerRef` _asbp_first_person_character))

(event `self.ReceiveTick`
  (params (DeltaSeconds :type "Float (single-precision)"))
  (bind (_returnvalue_roll _returnvalue_pitch _returnvalue_yaw) (`KismetMathLibrary.BreakRotator` (`self.K2_GetActorRotation`)))
  (bind (_returnvalue_roll_2 _returnvalue_pitch_2 _returnvalue_yaw_2) (`KismetMathLibrary.BreakRotator` (`self.K2_GetActorRotation`)))
  (bind (_returnvalue_roll_3 _returnvalue_pitch_3 _returnvalue_yaw_3) (`KismetMathLibrary.BreakRotator` (`KismetMathLibrary.FindLookAtRotation` (`SceneComponent.K2_GetComponentLocation` (`self.EyeR`)) (`self.K2_GetActorLocation` (`self.PlayerRef`)))))
  (bind (_returnvalue_roll_4 _returnvalue_pitch_4 _returnvalue_yaw_4) (`KismetMathLibrary.BreakRotator` (`KismetMathLibrary.FindLookAtRotation` (`SceneComponent.K2_GetComponentLocation` (`self.EyeL`)) (`self.K2_GetActorLocation` (`self.PlayerRef`)))))
  (`SceneComponent.K2_SetRelativeRotation` (`self.EyeL`) (`KismetMathLibrary.MakeRotator` _returnvalue_roll_4 _returnvalue_pitch_4 (- (- _returnvalue_yaw_4 _returnvalue_yaw_2) 75.0)) false false)
  (`SceneComponent.K2_SetRelativeRotation` (`self.EyeR`) (`KismetMathLibrary.MakeRotator` _returnvalue_roll_3 _returnvalue_pitch_3 (- (- _returnvalue_yaw_3 _returnvalue_yaw) 75.0)) false false))

(fn `UserConstructionScript`)