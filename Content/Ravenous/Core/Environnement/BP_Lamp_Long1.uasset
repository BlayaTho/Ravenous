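; Long lamp environment actor whose point light flickers when its LightFlickering event is called.
; A looping timer toggles the light's visibility on each tick, playing a flicker sound at the actor unless WoSound is set.
; TurnOff picks an odd or even toggle count, so a lit lamp ends dark or lit before the timer clears.
; The toggle counter is never reset between calls.
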(event `LightFlickering`
  (params (bTurnOff :type Boolean) (bWoSound :type Boolean))
  (set `self.MaxTurn` (`KismetMathLibrary.SelectInt` 12 11 bTurnOff))
  (bind _returnvalue (`KismetSystemLibrary.K2_SetTimerDelegate` (delegate `CustomEvent`) 0.1 true)))

(event `CustomEvent`
  (bind _pointlight16_lightcomponent0 (`self.PointLight16_LightComponent0`))
  (if (not (stale `LightFlickering` bWoSound))
    ;[0.09166 0.4458 1] LightFlickering Sound
    (`GameplayStatics.PlaySoundAtLocation` "/Game/Ravenous/Sound/Light/LightFlickering_Cue.LightFlickering_Cue" (`self.K2_GetActorLocation`) (struct) 1.0 1.0 0.0 null null null null))
  (`SceneComponent.SetVisibility` _pointlight16_lightcomponent0 (not (`SceneComponent.bVisible` _pointlight16_lightcomponent0)) false)
  (`/Engine/EditorBlueprintResources/StandardMacros.IncrementInt` (`self.TurnIndex`)
    (:`  `
      (if (> (`self.TurnIndex`) (`self.MaxTurn`))
        (`KismetSystemLibrary.K2_ClearAndInvalidateTimerHandle` (stale `LightFlickering` _returnvalue))))))

(fn `UserConstructionScript`)