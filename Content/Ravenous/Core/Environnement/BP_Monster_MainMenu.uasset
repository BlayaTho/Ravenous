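; BP_Monster_MainMenu is the monster in the main menu, which periodically plays a hand animation on its skeletal mesh.
; From BeginPlay, a self-calling AnimationRandom event waits a random few seconds, plays A_MainMenuHand once without looping, then repeats.
; Disconnected branches for two alternate hand animations, using a random choice and a HandOut flag, never run.
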(event `self.ReceiveBeginPlay`
  (`self.AnimationRandom`))

(event `AnimationRandom`
  (`KismetSystemLibrary.Delay` (`KismetMathLibrary.RandomFloatInRange` 3.0 7.0))
  (`SkeletalMeshComponent.PlayAnimation` (`self.SkeletalMesh`) "/Game/Ravenous/Animations/Animations/A_MainMenuHand.A_MainMenuHand" false)
  (`self.AnimationRandom`))

(fn `UserConstructionScript`)