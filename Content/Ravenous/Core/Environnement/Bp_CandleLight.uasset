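; Bp_CandleLight is a candle light actor for the environment, built around a flickering point light.
; The construction script applies exposed attenuation radius, intensity, source length and source radius values to the point light.
; On BeginPlay, the Flickering timeline drives the light's intensity between half and full of the configured value.
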(event `self.ReceiveBeginPlay`
  (bind _intensity (`self.Intensity`))
  (bind (_direction _intensity_2) (`Timeline|Flickering`)
    (:`Update`
      (`LightComponent.SetIntensity` (`self.PointLight`) (`KismetMathLibrary.Lerp` (/ _intensity 2.0) _intensity _intensity_2)))))

(fn `UserConstructionScript`
  (bind _pointlight (`self.PointLight`))
  (`LocalLightComponent.SetAttenuationRadius` _pointlight (`self.AttenuationRadius`))
  (`LightComponent.SetIntensity` _pointlight (`self.Intensity`))
  (`PointLightComponent.SetSourceLength` _pointlight (`self.SourceLenght`))
  (`PointLightComponent.SetSourceRadius` _pointlight (`self.SourceRadius`)))