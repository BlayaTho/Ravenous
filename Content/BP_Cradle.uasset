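; BP_Cradle is an interactable cradle that hints to the player that something is missing.
; On BeginPlay it creates a W_LucyDialogue widget and adds it to the viewport.
; Interacting empty-handed or with an item of the wrong type shows a short dialogue line, throttled by a DoOnce that resets after a delay.
; Holding the matching item type triggers nothing here.
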(event `self.ReceiveBeginPlay`
  (bind _returnvalue (`|CreateWidget` "/Game/Ravenous/UI/Widgets/W_LucyDialogue.W_LucyDialogue_C"))
  (bind _output_get (set `self.W_Text` _returnvalue))
  (`UserWidget.AddToViewport` _output_get 0))

(event `/Game/Ravenous/Core/Characters/Interface/BPI_Interaction.Interact`
  (params (ForDoor :type Boolean) (ForLock :type Boolean) (Name :type String) (PlayerRef :type "/Game/Ravenous/Core/Characters/Player/BP_FirstPersonCharacter Object Reference"))
  (`/Engine/EditorBlueprintResources/StandardMacros.IsValid` PlayerRef
    (:`Is Valid`
      (`/Engine/EditorBlueprintResources/StandardMacros.IsValid` (`/Game/Ravenous/Core/Characters/Player/BP_FirstPersonCharacter.HeldItem` PlayerRef)
        (:`Is Valid`
          (if (not (`|EnumEquality` (`/Game/Ravenous/Core/Interactables/Bp_PickableItem.ItemType` (`/Game/Ravenous/Core/Characters/Player/BP_FirstPersonCharacter.HeldItem` PlayerRef)) "NewEnumerator6"))
            (`/Engine/EditorBlueprintResources/StandardMacros.DoOnce` false :!label _label
              (:`Completed`
                (`/Game/Ravenous/UI/Widgets/W_LucyDialogue.StartDialogue` (`self.W_Text`) "Something's missing..." 0.75 null)
                (`KismetSystemLibrary.Delay` 3.0)
                (goto _label :!via `Reset`)))))
        (:`Is Not Valid`
          (goto _label))))))

(fn `UserConstructionScript`)