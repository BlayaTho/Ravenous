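; BP_Cone is an interactable cone whose Interaction component shifts and tilts once when the player uses it.
; BeginPlay caches the first-person character, and the inspection input checks that character's TouchInteractebalePart flag before acting.
; A DoOnce with no reset then plays a timeline that lerps the component's relative X and Z position and pitch.
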(event `self.ReceiveBeginPlay`
  ;[0.224 0.224 0.224] Begin Play
  (bind _asbp_first_person_character (cast `/Game/TheDoorsGame/Blueprints/Player/BP_FirstPersonCharacter` (`GameplayStatics.GetPlayerCharacter` 0)))
  (bind _output_get (set `self.As BP First Person Character` _asbp_first_person_character))
  (`parent.ReceiveBeginPlay`))

(event `EnhancedInput|/Game/TheDoorsGame/Input/Actions/Player/IA_InteractInspection`
  (params (ActionValue :type Boolean) (ElapsedSeconds :type "Float (double-precision)") (TriggeredSeconds :type "Float (double-precision)") (InputAction :type "InputAction Object Reference" :default "/Game/TheDoorsGame/Input/Actions/Player/IA_InteractInspection.IA_InteractInspection"))
  (:`Started`
    (if (`/Game/TheDoorsGame/Blueprints/Player/BP_FirstPersonCharacter.TouchInteractebalePart?` (stale `self.ReceiveBeginPlay` _output_get))
      (`/Engine/EditorBlueprintResources/StandardMacros.DoOnce` false
        (:`Completed`
          (bind (_direction _lerp) (`Timeline|Timeline` :!via `PlayFromStart`)
            (:`Update`
              (`SceneComponent.K2_SetRelativeLocationAndRotation` (`self.Interaction`) (`KismetMathLibrary.MakeVector` (`KismetMathLibrary.Lerp` 0.0 10.0 _lerp) 0.0 (`KismetMathLibrary.Lerp` 10.0 17.8 _lerp)) (`KismetMathLibrary.MakeRotator` 0.0 (`KismetMathLibrary.Lerp` 0.0 -50.0 _lerp)) false false))))))))

(fn `UserConstructionScript`
  (`parent.UserConstructionScript`))