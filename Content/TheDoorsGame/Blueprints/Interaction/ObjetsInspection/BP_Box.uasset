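; BP_Box is an inspectable box object with a movable part named "Interaction", built on a parent class that defines its base behavior.
; While that part is targeted, Tick shows the interaction widget and hides it once no part is targeted.
; IA_Interact plays a timeline once, sliding the part along Y and Z.
; Endfonction resets the DoOnce and reverses the timeline to return the part.
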(event `self.ReceiveBeginPlay`
  ;[0.224 0.224 0.224] Begin Play
  (`parent.ReceiveBeginPlay`)
  (bind _asw_interaction_inspection (cast `/Game/TheDoorsGame/UI/Widgets/W_InteractionInspection` (`WidgetComponent.GetUserWidgetObject` (`self.Widget`))))
  (set `self.W_Widget` _asw_interaction_inspection))

(event `EnhancedInput|/Game/TheDoorsGame/Input/Actions/Player/IA_Interact`
  (params (ActionValue :type Boolean) (ElapsedSeconds :type "Float (double-precision)") (TriggeredSeconds :type "Float (double-precision)") (InputAction :type "InputAction Object Reference" :default "/Game/TheDoorsGame/Input/Actions/Player/IA_Interact.IA_Interact"))
  (:`Started`
    (if (`self.TouchInteractebalePart?`)
      (`|ExecutionSequence`
        (:`then_0`
          (if (`KismetStringLibrary.EqualEqual_StrStr` (`self.PartName`) "Interaction")
            (`/Engine/EditorBlueprintResources/StandardMacros.DoOnce` false :!label _label
              (:`Completed`
                (bind (_direction _lerp) (`Timeline|Timeline` :!via `PlayFromStart` :!label _label_2)
                  (:`Update`
                    (`SceneComponent.K2_SetRelativeLocationAndRotation` (`self.Interaction`) (`KismetMathLibrary.MakeVector` 0.0 (`KismetMathLibrary.Lerp` 0.0 45.0 _lerp) (`KismetMathLibrary.Lerp` 10.0 20.0 _lerp)) (`KismetMathLibrary.MakeRotator` 0.0) false false)))))))))))

(event `self.ReceiveTick`
  (params (DeltaSeconds :type "Float (single-precision)"))
  (if (`self.TouchInteractebalePart?`)
    (`|ExecutionSequence`
      (:`then_0`
        (if (`KismetStringLibrary.EqualEqual_StrStr` (`self.PartName`) "Interaction")
          (`SceneComponent.SetHiddenInGame` (`self.Widget`) false false))))
    (else
      (`SceneComponent.SetHiddenInGame` (`self.Widget`) true false))))

(event `EnhancedInput|/Game/TheDoorsGame/Input/Actions/Player/IA_InteractInspection`
  (params (ActionValue :type Boolean) (ElapsedSeconds :type "Float (double-precision)") (TriggeredSeconds :type "Float (double-precision)") (InputAction :type "InputAction Object Reference" :default "/Game/TheDoorsGame/Input/Actions/Player/IA_InteractInspection.IA_InteractInspection")))

(event `self.endfonction`
  (`|ExecutionSequence`
    (:`then_0`
      (goto _label :!via `Reset`))
    (:`then_1`
      (goto _label_2 :!via `Reverse`))))

(fn `UserConstructionScript`
  (`parent.UserConstructionScript`))