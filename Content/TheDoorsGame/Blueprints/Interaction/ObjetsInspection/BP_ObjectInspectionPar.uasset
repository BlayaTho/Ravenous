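; Parent Blueprint for inspectable objects and notes, handing the item, its transform and note text to the first-person character's Inspection when interacted with.
; During inspection it takes input so move rotates the item (yaw only for notes) and lock-view exits.
; For non-notes, it shows an input widget and runs a looping camera trace recording the hit "Interactable"-tagged component's name.
; Interact input and Endfonction are empty stubs.
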(event `self.ReceiveBeginPlay`
  ;[0.224 0.224 0.224] Begin Play
  (bind _asbp_first_person_character (cast `/Game/TheDoorsGame/Blueprints/Player/BP_FirstPersonCharacter` (`GameplayStatics.GetPlayerCharacter` 0)))
  (set `self.As BP First Person Character` _asbp_first_person_character)
  (bind _returnvalue (`|CreateWidget` "/Game/TheDoorsGame/UI/Widgets/tutowidget/W_InputInspection.W_InputInspection_C"))
  (set `self.W_input` _returnvalue))

(event `/Game/TheDoorsGame/Blueprints/Interface/BPI_Interaction.Interact`
  (params (ForDoor :type Boolean) (ForLock :type Boolean) (Name :type String))
  (bind _as_bp_first_person_character (`self.As BP First Person Character`))
  ;[0.3177 0.3177 0.3177] Start / Stop Inspection
  (if (`/Game/TheDoorsGame/Blueprints/Player/BP_FirstPersonCharacter.CanInspect?` _as_bp_first_person_character)
    (`/Game/TheDoorsGame/Blueprints/Player/BP_FirstPersonCharacter.Inspection` _as_bp_first_person_character (`self.K2_GetActorLocation`) (`self.isNotes?`) (`self.TexteNote`) (`self.K2_GetActorRotation`) (`self.Item`))))

(event `StartInspect`
  (params (Inspector :type "Pawn Object Reference"))
  ;[0.3177 0.3177 0.3177] Start / Stop Inspection
  (`self.EnableInput` (`GameplayStatics.GetPlayerController` 0))
  (if (not (`self.isNotes?`))
    (bind _returnvalue (`KismetSystemLibrary.K2_SetTimer` null "ScanObjectF" 0.2 true))
    (set `self.TimerScan` _returnvalue)
    (`UserWidget.AddToViewport` (`self.W_input`) 0)))

(event `EnhancedInput|/Game/TheDoorsGame/Input/Actions/Player/IA_Interact`
  (params (ActionValue :type Boolean) (ElapsedSeconds :type "Float (double-precision)") (TriggeredSeconds :type "Float (double-precision)") (InputAction :type "InputAction Object Reference" :default "/Game/TheDoorsGame/Input/Actions/Player/IA_Interact.IA_Interact"))
  ;[0.3177 0.3177 0.3177] Start / Stop Inspection
)

(event `EnhancedInput|/Game/TheDoorsGame/Input/Actions/Player/IA_LockView`
  (params (ActionValue :type Boolean) (ElapsedSeconds :type "Float (double-precision)") (TriggeredSeconds :type "Float (double-precision)") (InputAction :type "InputAction Object Reference" :default "/Game/TheDoorsGame/Input/Actions/Player/IA_LockView.IA_LockView"))
  (bind _returnvalue (`GameplayStatics.GetPlayerController` 0))
  ;[0.3177 0.3177 0.3177] Start / Stop Inspection
  (:`Started`
    (`/Game/TheDoorsGame/Blueprints/Player/BP_FirstPersonCharacter.StopInspection` (`self.As BP First Person Character`) (`self.isNotes?`))
    (`KismetSystemLibrary.K2_ClearAndInvalidateTimerHandle` (`self.TimerScan`))
    (set `self.TouchInteractebalePart?` false)
    (`self.endfonction`)
    (`KismetSystemLibrary.Delay` 1.0)
    (`self.DisableInput` _returnvalue)
    (`self.EnableInput` (stale `StartInspect` Inspector) _returnvalue)
    (`Widget.RemoveFromParent` (`self.W_input`))))

(event `EnhancedInput|/Game/TheDoorsGame/Input/Actions/Player/IA_Move`
  (params (ActionValue :type "Vector2D Structure") (ElapsedSeconds :type "Float (double-precision)") (TriggeredSeconds :type "Float (double-precision)") (InputAction :type "InputAction Object Reference" :default "/Game/TheDoorsGame/Input/Actions/Player/IA_Move.IA_Move"))
  (bind _returnvalue (* ActionValue_X -3.0))
  (bind _item (`self.Item`))
  (bind _relativerotation (`SceneComponent.RelativeRotation` _item))
  ;[0.224 0.224 0.224] Rotate Object
  (:`Triggered`
    (if (not (`self.isNotes?`))
      (`SceneComponent.K2_SetRelativeRotation` _item (`KismetMathLibrary.ComposeRotators` _relativerotation (`KismetMathLibrary.MakeRotator` 0.0 (* ActionValue_Y -2.0) _returnvalue)) false false)
      (else
        (`SceneComponent.K2_SetRelativeRotation` _item (`KismetMathLibrary.ComposeRotators` _relativerotation (`KismetMathLibrary.MakeRotator` 0.0 0.0 _returnvalue)) false false)))))

(event `ScanObjectF`
  (bind _firstpersoncamera (`/Game/TheDoorsGame/Blueprints/Player/BP_FirstPersonCharacter.FirstPersonCamera` (`self.As BP First Person Character`)))
  (bind _returnvalue (`SceneComponent.K2_GetComponentLocation` _firstpersoncamera))
  ;[0.125 0.125 0.125] Scan Object in inspection
  (bind (_outhit _returnvalue_2) (`KismetSystemLibrary.LineTraceSingle` :`Start` _returnvalue :`End` (+ _returnvalue (* (`SceneComponent.GetForwardVector` _firstpersoncamera) 10000.0)) :`TraceChannel` "TraceTypeQuery1" :`bIgnoreSelf` false :`DrawTime` 0.1))
  (if _returnvalue_2
    (bind (_bblockinghit _binitialoverlap _time _distance _location _impactpoint _normal _impactnormal _physmat _hitactor _hitcomponent) (`GameplayStatics.BreakHitResult` _outhit))
    (if (`ActorComponent.ComponentHasTag` _hitcomponent "Interactable")
      (set `self.TouchInteractebalePart?` _returnvalue_2)
      (set `self.PartName` (`KismetSystemLibrary.GetObjectName` _hitcomponent))
      (else
        (set `self.TouchInteractebalePart?` false :!label _label)
        (set `self.PartName` "")))
    (else
      (goto _label))))

(fn `endfonction`
  (return))

(fn `UserConstructionScript`)