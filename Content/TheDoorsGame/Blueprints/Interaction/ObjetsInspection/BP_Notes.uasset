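; BP_Notes is an inspectable note object whose text and appearance come from a data table.
; On BeginPlay, after the parent's logic, it looks up its RowName in DT_Notes.
; When the row is found, it stores the note text, applies the row's material to the Item component and sets the IsNotes flag.
; The construction script only calls the parent.
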(event `self.ReceiveBeginPlay`
  (`parent.ReceiveBeginPlay`)
  (bind _returnvalue (`|GetDataTableRow` "/Game/TheDoorsGame/Blueprints/Data/DT_Notes.DT_Notes" (`self.Row Name`))
    (:`then`
      (set `self.TexteNote` (break `/Game/TheDoorsGame/Blueprints/Data/S_InfoTextNote` _returnvalue))
      (set `self.Out Row Material` (`.Material_11_4CB103D146D109E3D2E1F5A5F058CCCC` (break `/Game/TheDoorsGame/Blueprints/Data/S_InfoTextNote` _returnvalue)))
      (`PrimitiveComponent.SetMaterial` (`self.Item`) 0 (`self.Out Row Material`))
      (set `self.isNotes?` true))))

(fn `UserConstructionScript`
  (`parent.UserConstructionScript`))