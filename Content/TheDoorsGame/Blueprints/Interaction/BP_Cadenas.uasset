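; BP_Cadenas is an interactable combination padlock puzzle.
; Interact hands input to the lock and a looping timer blends the view to it; IA_Interact returns both to the player.
; IA_Move selects cylinders built from Base's children, and a timeline rolls them 36° per digit.
; Each turn updates RotationArray and compares it to SolutionRotationArray, though only the last comparison decides the win message and light.
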(event `self.ReceiveBeginPlay`
  ;[1 1 1] Begin play
  (bind _asbp_first_person_character (cast `/Game/TheDoorsGame/Blueprints/Player/BP_FirstPersonCharacter` (`GameplayStatics.GetPlayerCharacter` 0)))
  (set `self.As BP First Person Character` _asbp_first_person_character))

(event `/Game/TheDoorsGame/Blueprints/Interface/BPI_Interaction.Interact`
  (params (ForDoor :type Boolean) (ForLock :type Boolean))
  (bind _returnvalue (`GameplayStatics.GetPlayerController` 0))
  ;[1 1 1] Entrée et sortie du mode interaction avec le cadena
  (set `self.isLooking?` true)
  (`self.DisableInput` (`self.As BP First Person Character`) _returnvalue)
  (`self.EnableInput` _returnvalue)
  (bind _returnvalue_2 (`KismetSystemLibrary.K2_SetTimer` null "StartView" 0.01 true))
  (set `self.TimerTick` _returnvalue_2))

(event `EnhancedInput|/Game/TheDoorsGame/Input/Actions/Player/IA_Interact`
  (params (ActionValue :type Boolean) (ElapsedSeconds :type "Float (double-precision)") (TriggeredSeconds :type "Float (double-precision)") (InputAction :type "InputAction Object Reference" :default "/Game/TheDoorsGame/Input/Actions/Player/IA_Interact.IA_Interact"))
  ;[1 1 1] Entrée et sortie du mode interaction avec le cadena
  (:`Started`
    (`self.EndLooking`)))

(event `EndLooking`
  (bind _returnvalue (`GameplayStatics.GetPlayerController` 0))
  ;[1 1 1] Entrée et sortie du mode interaction avec le cadena
  (set `self.isLooking?` false)
  (`self.DisableInput` _returnvalue)
  (`self.EnableInput` (`self.As BP First Person Character`) _returnvalue)
  (`KismetSystemLibrary.Delay` 0.35)
  (`KismetSystemLibrary.K2_ClearAndInvalidateTimerHandle` (`self.TimerTick`)))

(event `StartView`
  ;[1 1 1] Toggle cam ticked
  (if (`self.isLooking?`)
    (`self.ToggleCam` true)
    (else
      (`self.ToggleCam` false))))

(event `EnhancedInput|/Game/TheDoorsGame/Input/Actions/Player/IA_Move`
  (params (ActionValue :type "Vector2D Structure") (ElapsedSeconds :type "Float (double-precision)") (TriggeredSeconds :type "Float (double-precision)") (InputAction :type "InputAction Object Reference" :default "/Game/TheDoorsGame/Input/Actions/Player/IA_Move.IA_Move"))
  (bind _rotationarray (`self.RotationArray`))
  (bind _output (`|GetArrayItem` (`self.CylinderArray`) (`self.indexSelection`)))
  (bind _output_2 (`|GetArrayItem` _rotationarray (`self.indexSelection`)))
  (:`Started`
    (if (not (`self.InRotation`))
      (`|ExecutionSequence`
        (:`then_0`
          ;[0.224 0.224 0.224] Quel cylindre j'ai selectionné en se basant sur l'index du tableau
          (if (> ActionValue_X 0.0)
            (bind _result (`/Engine/EditorBlueprintResources/StandardMacros.IncrementInt` (`self.indexSelection`))
              (:`  `
                (set `self.indexSelection` (`KismetMathLibrary.Clamp` _result 0 (`self.IndexMax`)))))
            (elif (< ActionValue_X 0.0)
              (bind _result_2 (`/Engine/EditorBlueprintResources/StandardMacros.DecrementInt` (`self.indexSelection`))
                (:`  `
                  (set `self.indexSelection` (`KismetMathLibrary.Clamp` _result_2 0 (`self.IndexMax`))))))))
        (:`then_1`
          ;[0.2135 0.2135 0.2135] Selon si le joueur monte ou descent (input) on prend la rotation actuel du cylindre et on ajoute ou enleve le ° pour tourner d'un cran
          (set `self.InRotation` true)
          (if (> ActionValue_Y 0.0)
            (bind _output_get (set `self.CylindreActual` _output))
            (bind _relativerotation_roll (`KismetMathLibrary.BreakRotator` (`SceneComponent.RelativeRotation` _output_get)))
            (bind _output_get_2 (set `self.Relative Rotation` _relativerotation_roll))
            (set `self.TargetRelativeRotation` (- _output_get_2 36.0))
            (set `self.IsDescending` true)
            ;[0.2135 0.2135 0.2135] Rotation du cylindre selectionné
            (bind (_direction _lerp) (`Timeline|RotateCylindre` :!via `PlayFromStart` :!label _label)
              (:`Update`
                (`SceneComponent.K2_SetRelativeRotation` (`self.CylindreActual`) (`KismetMathLibrary.MakeRotator` (`KismetMathLibrary.Lerp` (`self.Relative Rotation`) (`self.TargetRelativeRotation`) _lerp)) false false))
              (:`Finished`
                ;[0.2135 0.2135 0.2135] Referencement de la position actuel du cylindre dans un tableau (pour verifier plus tard la bonne combi)
                (if (`self.IsDescending`)
                  (if (== _output_2 0)
                    (set `self.IndexStocked` 9)
                    (else
                      (set `self.IndexStocked` (- _output_2 1))))
                  (`KismetArrayLibrary.Array_Set` _rotationarray (`self.indexSelection`) (`self.IndexStocked`))
                  (else
                    (if (== _output_2 9)
                      (set `self.IndexStocked` 0)
                      (else
                        (set `self.IndexStocked` (+ _output_2 1))))
                    (`KismetArrayLibrary.Array_Set` _rotationarray (`self.indexSelection`) (`self.IndexStocked`))))
                ;[0.2135 0.2135 0.2135] Verification de la combinaison en comparant la solution inscrite dans le tableau et la position enregistrée de chaque cylindre
                (set `self.InRotation` false)
                (for (_array_element _array_index) (`self.RotationArray`)
                  (if (== _array_element (`|GetArrayItem` (`self.SolutionRotationArray`) _array_index))
                    (set `self.GoodSolution?` true)
                    (else
                      (set `self.GoodSolution?` false))))
                (if (`self.GoodSolution?`)
                  (`KismetSystemLibrary.PrintString` "YOU WIN")
                  (`SceneComponent.SetVisibility` (`self.PointLight`) true false))))
            (elif (< ActionValue_Y 0.0)
              (bind _output_get_3 (set `self.CylindreActual` _output))
              (bind _relativerotation_roll_2 (`KismetMathLibrary.BreakRotator` (`SceneComponent.RelativeRotation` _output_get_3)))
              (bind _output_get_4 (set `self.Relative Rotation` _relativerotation_roll_2))
              (set `self.TargetRelativeRotation` (+ _output_get_4 36.0))
              (set `self.IsDescending` false)
              (goto _label :!via `PlayFromStart`)
              (else
                (set `self.InRotation` false)))))))))

(fn `ToggleCam`
  (params (`Start?` :type Boolean))
  (returns (`Succes?` :type Boolean))
  (bind _returnvalue (`GameplayStatics.GetPlayerController` 0))
  (if `Start?`
    (`PlayerController.SetViewTargetWithBlend` _returnvalue self 0.3 "VTBlend_Cubic" 0.0 false)
    (else
      (`PlayerController.SetViewTargetWithBlend` _returnvalue (`self.As BP First Person Character`) 0.3 "VTBlend_Cubic" 0.0 false)))
  (return true))

(fn `UserConstructionScript`
  (`KismetArrayLibrary.Array_Clear` (`self.RotationArray`))
  (`KismetArrayLibrary.Array_Clear` (`self.CylinderArray`))
  ;[1 1 1] Tableau de refs de cylindre basé sur le nombre de cyl que l'objet possede
  (bind _output_get (set `self.CylinderArray` (`SceneComponent.GetChildrenComponents` (`self.base`) false)))
  (set `self.IndexMax` (- (`KismetArrayLibrary.Array_Length` _output_get) 1))
  ;[1 1 1] Nombre d'index de rotation basé sur le nombre de cylindre de l'objet
  (for _ (`self.CylinderArray`)
    (`KismetArrayLibrary.Array_Add` (`self.RotationArray`))))