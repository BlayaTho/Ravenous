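; Interactive first-person door that the player drags open while holding LMB, and closes by interacting once fully open.
; Overlap boxes track the player's side.
; From behind, a timeline aligns player and camera and cracks the door, then a looping timer turns it with ForwardBackward input under clamped view yaw, auto-swinging it fully open past a threshold.
; The front-side path is unfinished, with its movement and rotation logic disconnected.
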(event `self.ReceiveBeginPlay`
  (bind _asbp_first_person_character (cast `/Game/TheDoorsGame/Blueprints/Player/BP_FirstPersonCharacter` (`GameplayStatics.GetPlayerCharacter` 0)))
  (set `self.As BP First Person Character` _asbp_first_person_character))

(event `TickBack`
  (bind _returnvalue (`GameplayStatics.GetPlayerCameraManager` 0))
  (bind _as_bp_first_person_character (`self.As BP First Person Character`))
  (bind _as_bp_first_person_character_2 (`self.As BP First Person Character`))
  (bind _as_bp_first_person_character_3 (`self.As BP First Person Character`))
  (bind _door (`self.Door`))
  (bind (_returnvalue_x _returnvalue_y _returnvalue_z) (`KismetMathLibrary.BreakVector` (`self.K2_GetActorLocation` _as_bp_first_person_character_2)))
  (bind (_returnvalue_x_2 _returnvalue_y_2) (`KismetMathLibrary.BreakVector` (`SceneComponent.K2_GetComponentLocation` (`self.PositionPlayerBack`))))
  (bind (_relativerotation_roll _relativerotation_pitch _relativerotation_yaw) (`KismetMathLibrary.BreakRotator` (`SceneComponent.RelativeRotation` (`self.Door`))))
  (bind (_relativerotation_roll_2 _relativerotation_pitch_2 _relativerotation_yaw_2) (`KismetMathLibrary.BreakRotator` (`SceneComponent.RelativeRotation` _door)))
  (if (`/Game/TheDoorsGame/Blueprints/Player/BP_FirstPersonCharacter.isHoldingLMB` _as_bp_first_person_character_3)
    (`self.K2_SetActorLocation` _as_bp_first_person_character_2 (`KismetMathLibrary.MakeVector` _returnvalue_x_2 _returnvalue_y_2 _returnvalue_z) false false)
    (if (<= _relativerotation_yaw 0.0)
      (set `/Game/TheDoorsGame/Blueprints/Player/BP_FirstPersonCharacter.inDoorInteraction` false (`self.As BP First Person Character`) :!label _label)
      (set `self.CanStartIntera` false)
      (set `PlayerCameraManager.ViewYawMin` (`/Game/TheDoorsGame/Blueprints/Player/BP_FirstPersonCharacter.View Yaw Min` _as_bp_first_person_character) _returnvalue)
      (set `PlayerCameraManager.ViewYawMax` (`/Game/TheDoorsGame/Blueprints/Player/BP_FirstPersonCharacter.View Yaw Max` _as_bp_first_person_character) _returnvalue)
      (`PrimitiveComponent.SetCollisionEnabled` (`self.BoxBack`) "QueryOnly")
      (`PrimitiveComponent.SetCollisionEnabled` (`self.BoxFront`) "QueryOnly")
      (elif (not (>= _relativerotation_yaw 70.0))
        (`SceneComponent.K2_AddRelativeRotation` (`self.Door`) (`KismetMathLibrary.MakeRotator` 0.0 0.0 (* (`/Game/TheDoorsGame/Blueprints/Player/BP_FirstPersonCharacter.ForwardBackward` (`self.As BP First Person Character`)) 0.6)) false false)
        (else
          (set `self.TargetAngleOpen` 100.0)
          (`/Engine/EditorBlueprintResources/StandardMacros.DoOnce` false :!label _label_2
            (:`Completed`
              (`|ExecutionSequence`
                (:`then_0`
                  (set `self.DoorCompletelyOpen` true)
                  (goto _label))
                (:`then_1`
                  (bind (_direction _lerp) (`Timeline|Timeline_0` :!via `PlayFromStart`)
                    (:`Update`
                      (`SceneComponent.K2_SetRelativeRotation` _door (`KismetMathLibrary.MakeRotator` 0.0 0.0 (`KismetMathLibrary.Lerp` _relativerotation_yaw_2 (`self.TargetAngleOpen`) _lerp)) false false))))))))))
    (else
      (set `/Game/TheDoorsGame/Blueprints/Player/BP_FirstPersonCharacter.inDoorInteraction` false _as_bp_first_person_character_3)
      (set `self.CanStartIntera` false)
      (goto _label))))

(event `self.Interact`
  (bind _returnvalue (`GameplayStatics.GetPlayerCameraManager` 0))
  (bind _as_bp_first_person_character (`self.As BP First Person Character`))
  (bind _as_bp_first_person_character_2 (`self.As BP First Person Character`))
  (bind _door (`self.Door`))
  (bind (_returnvalue_roll _returnvalue_pitch _returnvalue_yaw) (`KismetMathLibrary.BreakRotator` (`Pawn.GetControlRotation` (`self.As BP First Person Character`))))
  (bind (_returnvalue_x _returnvalue_y) (`KismetMathLibrary.BreakVector` (`SceneComponent.K2_GetComponentLocation` (`self.PositionPlayerBack`))))
  (bind (_returnvalue_x_2 _returnvalue_y_2 _returnvalue_z) (`KismetMathLibrary.BreakVector` (`self.K2_GetActorLocation` _as_bp_first_person_character_2)))
  (bind (_relativerotation_roll _relativerotation_pitch _relativerotation_yaw) (`KismetMathLibrary.BreakRotator` (`SceneComponent.RelativeRotation` _door)))
  (if (`self.DoorCompletelyOpen`)
    (bind (_direction _lerp) (`Timeline|Timeline_1` :!via `PlayFromStart`)
      (:`Update`
        (`SceneComponent.K2_SetRelativeRotation` _door (`KismetMathLibrary.MakeRotator` 0.0 0.0 (`KismetMathLibrary.Lerp` _relativerotation_yaw 0.0 _lerp)) false false))
      (:`Finished`
        (set `self.DoorCompletelyOpen` false)))
    (elif (`self.PlayerFront`)
      (`self.OuvertureFront`)
      (elif (`self.PlayerBack`)
        (set `self.FloatSens` -1.0)
        (set `/Game/TheDoorsGame/Blueprints/Player/BP_FirstPersonCharacter.inDoorInteraction` true (`self.As BP First Person Character`))
        (bind (_direction_2 _lerp_2) (`Timeline|Timeline` :!via `PlayFromStart`)
          (:`Update`
            (`self.K2_SetActorLocation` _as_bp_first_person_character_2 (`KismetMathLibrary.VLerp` (`self.K2_GetActorLocation` _as_bp_first_person_character_2) (`KismetMathLibrary.MakeVector` _returnvalue_x _returnvalue_y _returnvalue_z) _lerp_2) false false)
            (`SceneComponent.K2_SetRelativeRotation` (`self.Door`) (`KismetMathLibrary.MakeRotator` 0.0 0.0 (`KismetMathLibrary.Lerp` 0.0 10.0 _lerp_2)) false false)
            (`Controller.SetControlRotation` (`GameplayStatics.GetPlayerController` 0) (`KismetMathLibrary.RInterpTo` (`Pawn.GetControlRotation` _as_bp_first_person_character) (`KismetMathLibrary.FindLookAtRotation` (`SceneComponent.K2_GetComponentLocation` (`/Game/TheDoorsGame/Blueprints/Player/BP_FirstPersonCharacter.FirstPersonCamera` _as_bp_first_person_character)) (`SceneComponent.K2_GetComponentLocation` (`self.PositionLookCamBack`))) (`GameplayStatics.GetWorldDeltaSeconds`) 5.0)))
          (:`Finished`
            (bind _returnvalue_2 (`KismetSystemLibrary.K2_SetTimer` null "TickBack" 0.01 true))
            (set `self.TimerTickBack` _returnvalue_2)
            (`self.resetDoOnce`)
            (set `PlayerCameraManager.ViewYawMin` (- _returnvalue_yaw 45.0) _returnvalue)
            (set `PlayerCameraManager.ViewYawMax` (+ _returnvalue_yaw 45.0) _returnvalue)
            (`PrimitiveComponent.SetCollisionEnabled` (`self.BoxBack`) "NoCollision")
            (`PrimitiveComponent.SetCollisionEnabled` (`self.BoxFront`) "NoCollision")))))))

(event `resetDoOnce`
  (goto _label_2 :!via `Reset`))

(event `self.BoxFront.OnComponentBeginOverlap`
  (params (OverlappedComponent :type "PrimitiveComponent Object Reference") (OtherActor :type "Actor Object Reference") (OtherComp :type "PrimitiveComponent Object Reference") (OtherBodyIndex :type Integer) (bFromSweep :type Boolean) (SweepResult :type "HitResult Structure (by ref)"))
  (cast `/Game/TheDoorsGame/Blueprints/Player/BP_FirstPersonCharacter` OtherActor)
  (set `self.PlayerFront` true)
  (set `/Game/TheDoorsGame/Blueprints/Player/BP_FirstPersonCharacter.CanInteractWithDoor` true (`self.As BP First Person Character`)))

(event `self.BoxFront.OnComponentEndOverlap`
  (params (OverlappedComponent :type "PrimitiveComponent Object Reference") (OtherActor :type "Actor Object Reference") (OtherComp :type "PrimitiveComponent Object Reference") (OtherBodyIndex :type Integer))
  (set `self.PlayerFront` false)
  (set `/Game/TheDoorsGame/Blueprints/Player/BP_FirstPersonCharacter.CanInteractWithDoor` false (`self.As BP First Person Character`)))

(event `self.BoxBack.OnComponentBeginOverlap`
  (params (OverlappedComponent :type "PrimitiveComponent Object Reference") (OtherActor :type "Actor Object Reference") (OtherComp :type "PrimitiveComponent Object Reference") (OtherBodyIndex :type Integer) (bFromSweep :type Boolean) (SweepResult :type "HitResult Structure (by ref)"))
  (cast `/Game/TheDoorsGame/Blueprints/Player/BP_FirstPersonCharacter` OtherActor)
  (set `self.PlayerBack` true)
  (set `/Game/TheDoorsGame/Blueprints/Player/BP_FirstPersonCharacter.CanInteractWithDoor` true (`self.As BP First Person Character`)))

(event `self.BoxBack.OnComponentEndOverlap`
  (params (OverlappedComponent :type "PrimitiveComponent Object Reference") (OtherActor :type "Actor Object Reference") (OtherComp :type "PrimitiveComponent Object Reference") (OtherBodyIndex :type Integer))
  (set `self.PlayerBack` false)
  (set `/Game/TheDoorsGame/Blueprints/Player/BP_FirstPersonCharacter.CanInteractWithDoor` false (`self.As BP First Person Character`)))

(event `CustomEvent`
  (bind _asbp_first_person_character (cast `/Game/TheDoorsGame/Blueprints/Player/BP_FirstPersonCharacter` (`GameplayStatics.GetPlayerCharacter` 0)))
  (set `self.As BP First Person Character` _asbp_first_person_character))

(event `OuvertureFront`
  (bind _returnvalue (`GameplayStatics.GetPlayerCameraManager` 0))
  (bind (_returnvalue_roll _returnvalue_pitch _returnvalue_yaw) (`KismetMathLibrary.BreakRotator` (`Pawn.GetControlRotation` (`self.As BP First Person Character`))))
  (set `/Game/TheDoorsGame/Blueprints/Player/BP_FirstPersonCharacter.inDoorInteraction` true (`self.As BP First Person Character`))
  (bind (_direction _lerp) (`Timeline|Timeline_2` :!via `PlayFromStart`)
    (:`Finished`
      (set `self.CanStartIntera` true)
      (`self.resetDoOnce`)
      (set `PlayerCameraManager.ViewYawMin` (- _returnvalue_yaw 45.0) _returnvalue)
      (set `PlayerCameraManager.ViewYawMax` (+ _returnvalue_yaw 45.0) _returnvalue)
      (`PrimitiveComponent.SetCollisionEnabled` (`self.BoxBack`) "NoCollision")
      (`PrimitiveComponent.SetCollisionEnabled` (`self.BoxFront`) "NoCollision"))))

(event `CustomEvent_4`
  (bind _returnvalue (`GameplayStatics.GetPlayerCameraManager` 0))
  (bind _as_bp_first_person_character (`self.As BP First Person Character`))
  (bind _door (`self.Door`))
  (bind (_relativerotation_roll _relativerotation_pitch _relativerotation_yaw) (`KismetMathLibrary.BreakRotator` (`SceneComponent.RelativeRotation` _door)))
  (`/Engine/EditorBlueprintResources/StandardMacros.DoOnce` false :!via `Reset`
    (:`Completed`
      (`|ExecutionSequence`
        (:`then_0`
          (set `self.DoorCompletelyOpen` true)
          (set `/Game/TheDoorsGame/Blueprints/Player/BP_FirstPersonCharacter.inDoorInteraction` false (`self.As BP First Person Character`))
          (set `self.CanStartIntera` false)
          (set `PlayerCameraManager.ViewYawMin` (`/Game/TheDoorsGame/Blueprints/Player/BP_FirstPersonCharacter.View Yaw Min` _as_bp_first_person_character) _returnvalue)
          (set `PlayerCameraManager.ViewYawMax` (`/Game/TheDoorsGame/Blueprints/Player/BP_FirstPersonCharacter.View Yaw Max` _as_bp_first_person_character) _returnvalue)
          (`PrimitiveComponent.SetCollisionEnabled` (`self.BoxBack`) "QueryOnly")
          (`PrimitiveComponent.SetCollisionEnabled` (`self.BoxFront`) "QueryOnly"))
        (:`then_1`
          (bind (_direction _lerp) (`Timeline|Timeline_3` :!via `PlayFromStart`)
            (:`Update`
              (`SceneComponent.K2_SetRelativeRotation` _door (`KismetMathLibrary.MakeRotator` 0.0 0.0 (`KismetMathLibrary.Lerp` _relativerotation_yaw (`self.TargetAngleOpen`) _lerp)) false false))))))))

(fn `UserConstructionScript`)