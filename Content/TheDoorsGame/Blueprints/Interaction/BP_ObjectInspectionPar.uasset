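; BP_ObjectInspectionPar is an interactable object, apparently a parent class, that the player can inspect and rotate.
; Interact passes the actor's transform to the first-person character's Inspection, and StartInspect enables input on the object.
; IA_Move rotates the Item component, while IA_Interact returns input to the Inspector and calls StopInspection.
; BeginPlay is empty and the cast that sets the character reference is disconnected, so that reference is never assigned here.
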(event `self.ReceiveBeginPlay`
  ;[0.224 0.224 0.224] Begin Play
)

(event `/Game/TheDoorsGame/Blueprints/Interface/BPI_Interaction.Interact`
  ;[0.3177 0.3177 0.3177] Start / Stop Inspection
  (`/Game/TheDoorsGame/Blueprints/Player/BP_FirstPersonCharacter.Inspection` (`self.As BP First Person Character`) (`self.GetTransform`)))

(event `StartInspect`
  (params (Inspector :type "Pawn Object Reference"))
  ;[0.3177 0.3177 0.3177] Start / Stop Inspection
  (`self.EnableInput` (`GameplayStatics.GetPlayerController` 0)))

(event `EnhancedInput|/Game/TheDoorsGame/Input/Actions/Player/IA_Interact`
  (params (ActionValue :type Boolean) (ElapsedSeconds :type "Float (double-precision)") (TriggeredSeconds :type "Float (double-precision)") (InputAction :type "InputAction Object Reference" :default "/Game/TheDoorsGame/Input/Actions/Player/IA_Interact.IA_Interact"))
  (bind _returnvalue (`GameplayStatics.GetPlayerController` 0))
  ;[0.3177 0.3177 0.3177] Start / Stop Inspection
  (:`Started`
    (`self.DisableInput` _returnvalue)
    (`self.EnableInput` (stale `StartInspect` Inspector) _returnvalue)
    (`/Game/TheDoorsGame/Blueprints/Player/BP_FirstPersonCharacter.StopInspection` (`self.As BP First Person Character`))))

(event `EnhancedInput|/Game/TheDoorsGame/Input/Actions/Player/IA_Move`
  (params (ActionValue :type "Vector2D Structure") (ElapsedSeconds :type "Float (double-precision)") (TriggeredSeconds :type "Float (double-precision)") (InputAction :type "InputAction Object Reference" :default "/Game/TheDoorsGame/Input/Actions/Player/IA_Move.IA_Move"))
  (bind _item (`self.Item`))
  (:`Triggered`
    (`SceneComponent.K2_SetRelativeRotation` _item (`KismetMathLibrary.ComposeRotators` (`SceneComponent.RelativeRotation` _item) (`KismetMathLibrary.MakeRotator` 0.0 (* ActionValue_Y -2.0) (* ActionValue_X -3.0))) false false)))

(fn `UserConstructionScript`)