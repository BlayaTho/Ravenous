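; Parent Blueprint for objects the player can inspect and rotate up close.
; Interact calls Inspection on the cached first-person character, and StartInspect moves input from the Inspector to this object.
; While it has input, the move action applies pitch and yaw to the Item component's relative rotation.
; The interact action returns input to the Inspector and calls the character's Inspect.
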(event `self.ReceiveBeginPlay`
  (bind _asbp_first_person_character (cast `/Game/TheDoorsGame/Blueprints/Player/BP_FirstPersonCharacter` (`GameplayStatics.GetPlayerCharacter` 0)))
  (set `self.As BP First Person Character` _asbp_first_person_character))

(event `/Game/TheDoorsGame/Blueprints/Interface/BPI_Interaction.Interact`
  (`/Game/TheDoorsGame/Blueprints/Player/BP_FirstPersonCharacter.Inspection` (`self.As BP First Person Character`)))

(event `StartInspect`
  (params (Inspector :type "Pawn Object Reference"))
  (bind _returnvalue (`GameplayStatics.GetPlayerController` 0))
  (`self.DisableInput` Inspector _returnvalue)
  (`self.EnableInput` _returnvalue))

(event `EnhancedInput|/Game/TheDoorsGame/Input/Actions/Player/IA_Interact`
  (params (ActionValue :type Boolean) (ElapsedSeconds :type "Float (double-precision)") (TriggeredSeconds :type "Float (double-precision)") (InputAction :type "InputAction Object Reference" :default "/Game/TheDoorsGame/Input/Actions/Player/IA_Interact.IA_Interact"))
  (bind _returnvalue (`GameplayStatics.GetPlayerController` 0))
  (:`Started`
    (`self.DisableInput` _returnvalue)
    (`self.EnableInput` (stale `StartInspect` Inspector) _returnvalue)
    (`/Game/TheDoorsGame/Blueprints/Player/BP_FirstPersonCharacter.Inspect` (`self.As BP First Person Character`))))

(event `EnhancedInput|/Game/TheDoorsGame/Input/Actions/Player/IA_Move`
  (params (ActionValue :type "Vector2D Structure") (ElapsedSeconds :type "Float (double-precision)") (TriggeredSeconds :type "Float (double-precision)") (InputAction :type "InputAction Object Reference" :default "/Game/TheDoorsGame/Input/Actions/Player/IA_Move.IA_Move"))
  (bind _item (`self.Item`))
  (:`Triggered`
    (`SceneComponent.K2_SetRelativeRotation` _item (`KismetMathLibrary.ComposeRotators` (`SceneComponent.RelativeRotation` _item) (`KismetMathLibrary.MakeRotator` 0.0 (* ActionValue_Y -2.0) (* ActionValue_X -3.0))) false false)))

(fn `UserConstructionScript`)