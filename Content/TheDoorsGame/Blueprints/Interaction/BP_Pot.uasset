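; BP_Pot is an inspectable pot with two parts that each animate once when the player interacts with them during inspection.
; On the IA_InteractInspection input, it checks TouchInteractebalePart and matches PartName to the touched component.
; A timeline per part lerps the relative transform: Interaction shifts and tilts, while Interaction1 moves along Z.
; A DoOnce gates each animation.
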(event `self.ReceiveBeginPlay`
  ;[0.224 0.224 0.224] Begin Play
  (`parent.ReceiveBeginPlay`))

(event `EnhancedInput|/Game/TheDoorsGame/Input/Actions/Player/IA_InteractInspection`
  (params (ActionValue :type Boolean) (ElapsedSeconds :type "Float (double-precision)") (TriggeredSeconds :type "Float (double-precision)") (InputAction :type "InputAction Object Reference" :default "/Game/TheDoorsGame/Input/Actions/Player/IA_InteractInspection.IA_InteractInspection"))
  (bind _partname (`self.PartName`))
  (:`Started`
    (if (`self.TouchInteractebalePart?`)
      (`|ExecutionSequence`
        (:`then_0`
          (if (`KismetStringLibrary.EqualEqual_StrStr` _partname "Interaction")
            (`/Engine/EditorBlueprintResources/StandardMacros.DoOnce` false
              (:`Completed`
                (bind (_direction _lerp) (`Timeline|Timeline` :!via `PlayFromStart`)
                  (:`Update`
                    (`SceneComponent.K2_SetRelativeLocationAndRotation` (`self.Interaction`) (`KismetMathLibrary.MakeVector` (`KismetMathLibrary.Lerp` 0.0 10.0 _lerp) 0.0 (`KismetMathLibrary.Lerp` 10.0 17.8 _lerp)) (`KismetMathLibrary.MakeRotator` 0.0 (`KismetMathLibrary.Lerp` 0.0 -50.0 _lerp)) false false)))))))
        (:`then_1`
          (if (`KismetStringLibrary.EqualEqual_StrStr` _partname "Interaction1")
            (`/Engine/EditorBlueprintResources/StandardMacros.DoOnce` false
              (:`Completed`
                (bind (_direction_2 _lerp_2) (`Timeline|Timeline_0` :!via `PlayFromStart`)
                  (:`Update`
                    (`SceneComponent.K2_SetRelativeLocationAndRotation` :`self` (`self.Interaction1`) :`NewLocation` (`KismetMathLibrary.MakeVector` 0.0 0.0 (`KismetMathLibrary.Lerp` -10.0 -20.0 _lerp_2)))))))))))))

(fn `UserConstructionScript`
  (`parent.UserConstructionScript`))