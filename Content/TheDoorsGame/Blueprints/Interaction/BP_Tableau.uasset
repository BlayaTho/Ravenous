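; BP_Tableau is an interactable tableau that tips over once when the player uses it.
; Interact passes a DoOnce, then a Timeline lerps the mesh's roll to swing it to its end angle.
; When IsFirstFrame is set, it also calls StartWidgetCrouch on the first-person character and drops collision immediately.
; Otherwise, collision is disabled only when the rotation finishes.
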(event `/Game/TheDoorsGame/Blueprints/Interface/BPI_Interaction.Interact`
  (params (ForDoor :type Boolean) (ForLock :type Boolean) (Name :type String))
  (`/Engine/EditorBlueprintResources/StandardMacros.DoOnce` false
    (:`Completed`
      (if (`self.isFirstFrame`)
        (bind _asbp_first_person_character (cast `/Game/TheDoorsGame/Blueprints/Player/BP_FirstPersonCharacter` (`GameplayStatics.GetPlayerCharacter` 0)))
        (`/Game/TheDoorsGame/Blueprints/Player/BP_FirstPersonCharacter.StartWidgetCrouch` _asbp_first_person_character)
        (`PrimitiveComponent.SetCollisionEnabled` (`self.Tableau`) "NoCollision")
        (bind (_direction _lerp) (`Timeline|Timeline` :!via `PlayFromStart` :!label _label)
          (:`Update`
            (`SceneComponent.K2_SetRelativeRotation` (`self.Tableau`) (`KismetMathLibrary.MakeRotator` (`KismetMathLibrary.Lerp` -20.0 90.0 _lerp)) false false))
          (:`Finished`
            (if (not (`self.isFirstFrame`))
              (`PrimitiveComponent.SetCollisionEnabled` (`self.Tableau`) "NoCollision"))))
        (else
          (goto _label :!via `PlayFromStart`))))))

(fn `UserConstructionScript`)