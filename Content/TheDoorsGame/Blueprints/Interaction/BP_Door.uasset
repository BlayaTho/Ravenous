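; Interactive first-person door that the player swings by holding click and moving, with optional Victor key unlocking.
; A dot product picks front or back; timelines align player and camera and crack the door.
; Looping timers then apply movement input to the yaw until it auto-completes open or closes.
; A separate lock view blends to a side-specific door camera with clamped look, while overlap boxes gate interaction and lock prompts.
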(event `Ouverture Back`
  (bind _returnvalue (`GameplayStatics.GetPlayerCameraManager` 0))
  (bind _as_bp_first_person_character (`self.As BP First Person Character`))
  (bind _as_bp_first_person_character_2 (`self.As BP First Person Character`))
  (bind (_returnvalue_x _returnvalue_y _returnvalue_z) (`KismetMathLibrary.BreakVector` (`self.K2_GetActorLocation` _as_bp_first_person_character_2)))
  (bind (_returnvalue_x_2 _returnvalue_y_2) (`KismetMathLibrary.BreakVector` (`SceneComponent.K2_GetComponentLocation` (`self.PositionPlayerBack`))))
  (bind (_returnvalue_roll _returnvalue_pitch _returnvalue_yaw) (`KismetMathLibrary.BreakRotator` (`Pawn.GetControlRotation` (`self.As BP First Person Character`))))
  ;[0.04688 0.04688 0.04688] Position Ouverture Back
  (set `/Game/TheDoorsGame/Blueprints/Player/BP_FirstPersonCharacter.inDoorInteraction` true (`self.As BP First Person Character`))
  (bind (_direction _lerp) (`Timeline|Timeline` :!via `PlayFromStart`)
    (:`Update`
      (`self.K2_SetActorLocation` _as_bp_first_person_character_2 (`KismetMathLibrary.VLerp` (`self.K2_GetActorLocation` _as_bp_first_person_character_2) (`KismetMathLibrary.MakeVector` _returnvalue_x_2 _returnvalue_y_2 _returnvalue_z) _lerp) false false)
      (`SceneComponent.K2_SetRelativeRotation` (`self.Door`) (`KismetMathLibrary.MakeRotator` 0.0 0.0 (`KismetMathLibrary.Lerp` 0.0 10.0 _lerp)) false false)
      (`Controller.SetControlRotation` (`GameplayStatics.GetPlayerController` 0) (`KismetMathLibrary.RInterpTo` (`Pawn.GetControlRotation` _as_bp_first_person_character) (`KismetMathLibrary.FindLookAtRotation` (`SceneComponent.K2_GetComponentLocation` (`/Game/TheDoorsGame/Blueprints/Player/BP_FirstPersonCharacter.FirstPersonCamera` _as_bp_first_person_character)) (`SceneComponent.K2_GetComponentLocation` (`self.PositionLookCamBack`))) (`GameplayStatics.GetWorldDeltaSeconds`) 5.0)))
    (:`Finished`
      (bind _returnvalue_2 (`KismetSystemLibrary.K2_SetTimer` null "TickOuvertureBack" 0.005 true))
      (set `self.TimerTickBack` _returnvalue_2)
      (`self.resetDoOnce`)
      (set `PlayerCameraManager.ViewYawMin` (- _returnvalue_yaw 45.0) _returnvalue)
      (set `PlayerCameraManager.ViewYawMax` (+ _returnvalue_yaw 45.0) _returnvalue)
      (`PrimitiveComponent.SetCollisionEnabled` (`self.BoxBack`) "NoCollision")
      (`PrimitiveComponent.SetCollisionEnabled` (`self.BoxFront`) "NoCollision"))))

(event `Ouverture Front`
  (bind _returnvalue (`GameplayStatics.GetPlayerCameraManager` 0))
  (bind _as_bp_first_person_character (`self.As BP First Person Character`))
  (bind _as_bp_first_person_character_2 (`self.As BP First Person Character`))
  (bind (_returnvalue_roll _returnvalue_pitch _returnvalue_yaw) (`KismetMathLibrary.BreakRotator` (`Pawn.GetControlRotation` (`self.As BP First Person Character`))))
  (bind (_returnvalue_x _returnvalue_y) (`KismetMathLibrary.BreakVector` (`SceneComponent.K2_GetComponentLocation` (`self.PositionPlayerFront`))))
  (bind (_returnvalue_x_2 _returnvalue_y_2 _returnvalue_z) (`KismetMathLibrary.BreakVector` (`self.K2_GetActorLocation` _as_bp_first_person_character_2)))
  ;[0.04688 0.04688 0.04688] Position Ouverture Front
  (set `/Game/TheDoorsGame/Blueprints/Player/BP_FirstPersonCharacter.inDoorInteraction` true (`self.As BP First Person Character`))
  (bind (_direction _lerp) (`Timeline|Timeline_5` :!via `PlayFromStart`)
    (:`Update`
      (`self.K2_SetActorLocation` _as_bp_first_person_character_2 (`KismetMathLibrary.VLerp` (`self.K2_GetActorLocation` _as_bp_first_person_character_2) (`KismetMathLibrary.MakeVector` _returnvalue_x _returnvalue_y _returnvalue_z) _lerp) false false)
      (`SceneComponent.K2_SetRelativeRotation` (`self.Door`) (`KismetMathLibrary.MakeRotator` 0.0 0.0 (`KismetMathLibrary.Lerp` 0.0 -10.0 _lerp)) false false)
      (`Controller.SetControlRotation` (`GameplayStatics.GetPlayerController` 0) (`KismetMathLibrary.RInterpTo` (`Pawn.GetControlRotation` _as_bp_first_person_character) (`KismetMathLibrary.FindLookAtRotation` (`SceneComponent.K2_GetComponentLocation` (`/Game/TheDoorsGame/Blueprints/Player/BP_FirstPersonCharacter.FirstPersonCamera` _as_bp_first_person_character)) (`SceneComponent.K2_GetComponentLocation` (`self.PositionLookCamFront`))) (`GameplayStatics.GetWorldDeltaSeconds`) 5.0)))
    (:`Finished`
      (bind _returnvalue_2 (`KismetSystemLibrary.K2_SetTimer` null "TickOuvertureFront" 0.005 true))
      (set `self.TimerTickFront` _returnvalue_2)
      (`self.resetDoOnce`)
      (set `PlayerCameraManager.ViewYawMin` (- _returnvalue_yaw 45.0) _returnvalue)
      (set `PlayerCameraManager.ViewYawMax` (+ _returnvalue_yaw 45.0) _returnvalue)
      (`PrimitiveComponent.SetCollisionEnabled` (`self.BoxBack`) "NoCollision")
      (`PrimitiveComponent.SetCollisionEnabled` (`self.BoxFront`) "NoCollision"))))

(event `self.ReceiveTick`
  (params (DeltaSeconds :type "Float (single-precision)")))

(event `self.ReceiveBeginPlay`
  ;[0.08333 0.08333 0.08333] BeginPlay
  (bind _asbp_first_person_character (cast `/Game/TheDoorsGame/Blueprints/Player/BP_FirstPersonCharacter` (`GameplayStatics.GetPlayerCharacter` 0)))
  (set `self.As BP First Person Character` _asbp_first_person_character)
  (bind _returnvalue (`|CreateWidget` "/Game/TheDoorsGame/UI/Widgets/W_LockView.W_LockView_C"))
  (set `self.W_LockView` _returnvalue)
  (bind _asw_lock_door (cast `/Game/TheDoorsGame/UI/Widgets/W_LockDoor` (`WidgetComponent.GetUserWidgetObject` (`self.Widget_Front`))))
  (set `self.W_LockDoorFront` _asw_lock_door)
  (bind _asw_lock_door_2 (cast `/Game/TheDoorsGame/UI/Widgets/W_LockDoor` (`WidgetComponent.GetUserWidgetObject` (`self.Widget_Back`))))
  (set `self.W_LockDoorBack` _asw_lock_door_2))

(event `CloseDoor`
  (bind _door (`self.Door`))
  (bind (_relativerotation_roll _relativerotation_pitch _relativerotation_yaw) (`KismetMathLibrary.BreakRotator` (`SceneComponent.RelativeRotation` _door)))
  ;[0.09375 0.09375 0.09375] CloseDoor
  (`/Engine/EditorBlueprintResources/StandardMacros.DoOnce` false :!label _label
    (:`Completed`
      (set `self.Relative Rotation Z (Yaw)` _relativerotation_yaw)
      (bind (_direction _lerp) (`Timeline|TimelineCloseDoor` :!via `PlayFromStart`)
        (:`Update`
          (`SceneComponent.K2_SetRelativeRotation` _door (`KismetMathLibrary.MakeRotator` 0.0 0.0 (`KismetMathLibrary.Lerp` (`self.Relative Rotation Z (Yaw)`) 0.0 _lerp)) false false))
        (:`Finished`
          (`self.StopDoorInteractionF`))))))

(event `resetDoOnce`
  (bind _door (`self.Door`))
  (bind (_relativerotation_roll _relativerotation_pitch _relativerotation_yaw) (`KismetMathLibrary.BreakRotator` (`SceneComponent.RelativeRotation` _door)))
  (`|ExecutionSequence`
    (:`then_0`
      (goto _label :!via `Reset`))
    (:`then_1`
      (goto _label_2 :!via `Reset`))))

(event `/Game/TheDoorsGame/Blueprints/Interface/BPI_Interaction.Interact`
  (params (ForDoor :type Boolean) (ForLock :type Boolean) (Name :type String))
  (bind _as_bp_first_person_character (`self.As BP First Person Character`))
  (bind _returnvalue (`KismetMathLibrary.NearlyEqual_FloatFloat` (`KismetMathLibrary.Dot_VectorVector` (`self.GetActorForwardVector` (`self.As BP First Person Character`)) (`self.GetActorForwardVector`)) -1.0 0.65))
  ;[0.08333 0.08333 0.08333] Debut Interaction porte
  (`|ExecutionSequence`
    (:`then_0`
      (if (`self.DoorCompletelyOpen`)
        (`self.CloseDoor`)))
    (:`then_1`
      (if (and ForDoor (`self.CanOpen?`))
        (if (not (`self.DoorCompletelyOpen`))
          (if _returnvalue
            (`self.Ouverture Front`)
            (else
              (`self.Ouverture Back`)))
          (`/Game/TheDoorsGame/UI/Widgets/tutowidget/W_InputDoor.AnimMove` (`/Game/TheDoorsGame/Blueprints/Player/BP_FirstPersonCharacter.W_inputDoor` (`self.As BP First Person Character`))))
        (elif (and (`self.NeedVictorKey?`) (`/Game/TheDoorsGame/Blueprints/Player/BP_FirstPersonCharacter.VictorKey?` _as_bp_first_person_character))
          (`ChildActorComponent.SetChildActorClass` (`/Game/TheDoorsGame/Blueprints/Player/BP_FirstPersonCharacter.CaryItem` _as_bp_first_person_character) null)
          (set `self.CanOpen?` true))))
    (:`then_2`
      (if (and ForLock (not (`self.DoorCompletelyOpen`)) (`self.NoAnim`))
        (if _returnvalue
          (set `self.PlayerFront` true)
          (else
            (set `self.PlayerFront` false)))
        (`self.SetValue` (`self.PlayerFront`))
        (bind _returnvalue_2 (`KismetSystemLibrary.K2_SetTimer` null "StartLockView" 0.01 true))
        (set `self.TimerTickLockView` _returnvalue_2)))))

(event `OpenDoorCompletely`
  (params (`Back?` :type Boolean))
  (bind _door (`self.Door`))
  (bind (_relativerotation_roll _relativerotation_pitch _relativerotation_yaw) (`KismetMathLibrary.BreakRotator` (`SceneComponent.RelativeRotation` _door)))
  ;[0.0625 0.0625 0.0625] Open Door Completely
  (`/Engine/EditorBlueprintResources/StandardMacros.DoOnce` false :!label _label_2
    (:`Completed`
      (if `Back?`
        (set `self.TargetAngleOpen` 100.0)
        (else
          (set `self.TargetAngleOpen` -100.0)))
      (`|ExecutionSequence`
        (:`then_0`
          (`self.StopDoorInteractionF`))
        (:`then_1`
          (set `self.Relative Rotation Z (Yaw)` _relativerotation_yaw)
          (bind (_direction _lerp) (`Timeline|Timeline_0` :!via `PlayFromStart`)
            (:`Update`
              (`SceneComponent.K2_SetRelativeRotation` _door (`KismetMathLibrary.MakeRotator` 0.0 0.0 (`KismetMathLibrary.Lerp` (`self.Relative Rotation Z (Yaw)`) (`self.TargetAngleOpen`) _lerp)) false false))
            (:`Finished`
              (set `self.DoorCompletelyOpen` true)
              (`/Game/TheDoorsGame/UI/Widgets/W_LockDoor.LanceAnim` (`self.W_LockDoorBack`) false)
              (`/Game/TheDoorsGame/UI/Widgets/W_LockDoor.LanceAnim` (`self.W_LockDoorFront`) false))))))))

(event `self.BoxFront.OnComponentBeginOverlap`
  (params (OverlappedComponent :type "PrimitiveComponent Object Reference") (OtherActor :type "Actor Object Reference") (OtherComp :type "PrimitiveComponent Object Reference") (OtherBodyIndex :type Integer) (bFromSweep :type Boolean) (SweepResult :type "HitResult Structure (by ref)"))
  (bind _as_bp_first_person_character (`self.As BP First Person Character`))
  ;[0.09896 0.09896 0.09896] Scan Position Joueur
  (cast `/Game/TheDoorsGame/Blueprints/Player/BP_FirstPersonCharacter` OtherActor)
  (set `/Game/TheDoorsGame/Blueprints/Player/BP_FirstPersonCharacter.CanInteractWithDoor` true _as_bp_first_person_character)
  (`/Game/TheDoorsGame/Blueprints/Player/BP_FirstPersonCharacter.PlayerInZoneLook` _as_bp_first_person_character self)
  (if (not (`self.DoorCompletelyOpen`))
    (`/Game/TheDoorsGame/UI/Widgets/W_LockDoor.LanceAnim` (`self.W_LockDoorFront`) true)))

(event `self.BoxFront.OnComponentEndOverlap`
  (params (OverlappedComponent :type "PrimitiveComponent Object Reference") (OtherActor :type "Actor Object Reference") (OtherComp :type "PrimitiveComponent Object Reference") (OtherBodyIndex :type Integer))
  ;[0.09896 0.09896 0.09896] Scan Position Joueur
  (cast `/Game/TheDoorsGame/Blueprints/Player/BP_FirstPersonCharacter` OtherActor)
  (set `/Game/TheDoorsGame/Blueprints/Player/BP_FirstPersonCharacter.CanInteractWithDoor` false (`self.As BP First Person Character`))
  (if (not (`self.DoorCompletelyOpen`))
    (`/Game/TheDoorsGame/UI/Widgets/W_LockDoor.LanceAnim` (`self.W_LockDoorFront`) false)))

(event `SetValue`
  (params (`Front?` :type Boolean))
  ;[0.09896 0.09896 0.09896] SetValueLockview
  (if `Front?`
    (`ActorComponent.SetActive` (`self.CameraFront`) true false)
    (`ActorComponent.SetActive` (`self.CameraBack`) false false)
    (set `self.YawMin` -195.0)
    (set `self.YawMax` -165.0)
    (set `self.Yaw` -180.0)
    (else
      (`ActorComponent.SetActive` (`self.CameraFront`) false false)
      (`ActorComponent.SetActive` (`self.CameraBack`) true false)
      (set `self.YawMin` -15.0)
      (set `self.YawMax` 15.0)
      (set `self.Yaw` 0.0))))

(event `self.BoxBack.OnComponentBeginOverlap`
  (params (OverlappedComponent :type "PrimitiveComponent Object Reference") (OtherActor :type "Actor Object Reference") (OtherComp :type "PrimitiveComponent Object Reference") (OtherBodyIndex :type Integer) (bFromSweep :type Boolean) (SweepResult :type "HitResult Structure (by ref)"))
  (bind _as_bp_first_person_character (`self.As BP First Person Character`))
  ;[0.09896 0.09896 0.09896] Scan Position Joueur
  (cast `/Game/TheDoorsGame/Blueprints/Player/BP_FirstPersonCharacter` OtherActor)
  (set `/Game/TheDoorsGame/Blueprints/Player/BP_FirstPersonCharacter.CanInteractWithDoor` true _as_bp_first_person_character)
  (`/Game/TheDoorsGame/Blueprints/Player/BP_FirstPersonCharacter.PlayerInZoneLook` _as_bp_first_person_character self)
  (if (not (`self.DoorCompletelyOpen`))
    (`/Game/TheDoorsGame/UI/Widgets/W_LockDoor.LanceAnim` (`self.W_LockDoorBack`) true)))

(event `self.BoxBack.OnComponentEndOverlap`
  (params (OverlappedComponent :type "PrimitiveComponent Object Reference") (OtherActor :type "Actor Object Reference") (OtherComp :type "PrimitiveComponent Object Reference") (OtherBodyIndex :type Integer))
  ;[0.09896 0.09896 0.09896] Scan Position Joueur
  (cast `/Game/TheDoorsGame/Blueprints/Player/BP_FirstPersonCharacter` OtherActor)
  (set `/Game/TheDoorsGame/Blueprints/Player/BP_FirstPersonCharacter.CanInteractWithDoor` false (`self.As BP First Person Character`))
  (if (not (`self.DoorCompletelyOpen`))
    (`/Game/TheDoorsGame/UI/Widgets/W_LockDoor.LanceAnim` (`self.W_LockDoorBack`) false)))

(event `reset`
  (`|ExecutionSequence`
    (:`then_0`
      (goto _label_3 :!via `Reset`))
    (:`then_1`
      (goto _label_5 :!via `Reset`))))

(event `ToogleCamera`
  (params (Start :type Boolean))
  (bind _returnvalue (`GameplayStatics.GetPlayerController` 0))
  (set `self.NoAnim` false)
  (if (`/Game/TheDoorsGame/Blueprints/Player/BP_FirstPersonCharacter.CanInteractWithDoor` (`self.As BP First Person Character`))
    (if Start
      (set `self.isLooking?` true)
      (`PlayerController.SetViewTargetWithBlend` _returnvalue self 0.5 "VTBlend_Cubic" 0.0 false)
      (`|ExecutionSequence`
        (:`then_0`
          (`/Engine/EditorBlueprintResources/StandardMacros.DoOnce` false :!label _label_3
            (:`Completed`
              (`UserWidget.AddToViewport` (`self.W_LockView`) 0)
              (`KismetSystemLibrary.Delay` 0.5)
              (set `self.NoAnim` true))))
        (:`then_1`
          (`self.EndToggle` true :!label _label_4)))
      (else
        (set `self.isLooking?` false)
        (`PlayerController.SetViewTargetWithBlend` _returnvalue (`self.As BP First Person Character`) 0.5 "VTBlend_Cubic" 0.0 false)
        (`|ExecutionSequence`
          (:`then_0`
            (`/Engine/EditorBlueprintResources/StandardMacros.DoOnce` false :!label _label_5
              (:`Completed`
                (`Widget.RemoveFromParent` (`self.W_LockView`))
                (`KismetSystemLibrary.Delay` 0.5)
                (set `self.NoAnim` true))))
          (:`then_1`
            (goto _label_4)))))
    (else
      (`self.EndToggle` false))))

(event `StartLockView`
  ;[0.07292 0.07292 0.07292] Tick LockView
  (if (`self.HoldingRMB`)
    (`self.ToogleCamera` true)
    (else
      (`self.ToogleCamera` false))))

(event `EnhancedInput|/Game/TheDoorsGame/Input/Actions/Player/IA_LockView`
  (params (ActionValue :type Boolean) (ElapsedSeconds :type "Float (double-precision)") (TriggeredSeconds :type "Float (double-precision)") (InputAction :type "InputAction Object Reference" :default "/Game/TheDoorsGame/Input/Actions/Player/IA_LockView.IA_LockView"))
  ;[0.07292 0.07292 0.07292] Tick LockView
  (:`Completed`
    (set `self.HoldingRMB` false)))

(event `EndToggle`
  (params (`Success?` :type Boolean))
  ;[0.07292 0.07292 0.07292] Tick LockView
  (if `Success?`
    (`self.MoveCamera`)))

(event `MoveCamera`
  (bind _returnvalue (`GameplayStatics.GetPlayerController` 0))
  (bind _as_bp_first_person_character (`self.As BP First Person Character`))
  ;[0.09896 0.09896 0.09896] LockView Calcul
  (if (`self.isLooking?`)
    (`self.DisableInput` _as_bp_first_person_character _returnvalue)
    (`self.EnableInput` _returnvalue)
    (if (`self.PlayerFront`)
      (bind _returnvalue_2 (`KismetMathLibrary.MakeRotator` 0.0 (* (stale `EnhancedInput|/Game/TheDoorsGame/Input/Actions/Player/IA_Look` _output_get) -1.0) (stale `EnhancedInput|/Game/TheDoorsGame/Input/Actions/Player/IA_Look` _output_get_2)))
      (`SceneComponent.K2_SetRelativeRotation` (`self.CameraFront`) _returnvalue_2 false false)
      (else
        (`SceneComponent.K2_SetRelativeRotation` (`self.CameraBack`) _returnvalue_2 false false)))
    (`KismetSystemLibrary.Delay` 0.001)
    (`self.MoveCamera`)
    (else
      (`self.DisableInput` _returnvalue)
      (`self.EnableInput` _as_bp_first_person_character _returnvalue)
      (`KismetSystemLibrary.K2_ClearAndInvalidateTimerHandle` (`self.TimerTickLockView`))
      (set `self.HoldingRMB` true)
      (`self.reset`))))

(event `EnhancedInput|/Game/TheDoorsGame/Input/Actions/Player/IA_Look`
  (params (ActionValue :type "Vector2D Structure") (ElapsedSeconds :type "Float (double-precision)") (TriggeredSeconds :type "Float (double-precision)") (InputAction :type "InputAction Object Reference" :default "/Game/TheDoorsGame/Input/Actions/Player/IA_Look.IA_Look"))
  (bind _as_bp_first_person_character (`self.As BP First Person Character`))
  ;[0.09896 0.09896 0.09896] LockView Calcul
  (:`Triggered`
    (if (`self.isLooking?`)
      (bind _output_get (set `self.Pitch` (`KismetMathLibrary.FClamp` (+ (`self.Pitch`) ActionValue_Y) -10.0 10.0)))
      (bind _output_get_2 (set `self.Yaw` (`KismetMathLibrary.FClamp` (+ (`self.Yaw`) ActionValue_X) (`self.YawMin`) (`self.YawMax`))))
      (else
        (`Pawn.AddControllerPitchInput` _as_bp_first_person_character ActionValue_Y)
        (`Pawn.AddControllerYawInput` _as_bp_first_person_character ActionValue_X)))))

(fn `StopDoorInteractionF`
  (bind _returnvalue (`GameplayStatics.GetPlayerCameraManager` 0))
  (bind _as_bp_first_person_character (`self.As BP First Person Character`))
  ;[0.07812 0.07812 0.07812] StopDoorInteraction
  (`KismetSystemLibrary.K2_ClearAndInvalidateTimerHandle` (`self.TimerTickFront`))
  (`KismetSystemLibrary.K2_ClearAndInvalidateTimerHandle` (`self.TimerTickBack`))
  (set `/Game/TheDoorsGame/Blueprints/Player/BP_FirstPersonCharacter.inDoorInteraction` false (`self.As BP First Person Character`))
  (set `PlayerCameraManager.ViewYawMin` (`/Game/TheDoorsGame/Blueprints/Player/BP_FirstPersonCharacter.View Yaw Min` _as_bp_first_person_character) _returnvalue)
  (set `PlayerCameraManager.ViewYawMax` (`/Game/TheDoorsGame/Blueprints/Player/BP_FirstPersonCharacter.View Yaw Max` _as_bp_first_person_character) _returnvalue)
  (`PrimitiveComponent.SetCollisionEnabled` (`self.BoxBack`) "QueryOnly")
  (`PrimitiveComponent.SetCollisionEnabled` (`self.BoxFront`) "QueryOnly")
  (set `self.DoorCompletelyOpen` false)
  (`/Game/TheDoorsGame/UI/Widgets/tutowidget/W_InputDoor.Endanim` (`/Game/TheDoorsGame/Blueprints/Player/BP_FirstPersonCharacter.W_inputDoor` (`self.As BP First Person Character`))))

(fn `TickOuvertureBack`
  (bind _as_bp_first_person_character (`self.As BP First Person Character`))
  (bind _as_bp_first_person_character_2 (`self.As BP First Person Character`))
  (bind (_returnvalue_x _returnvalue_y) (`KismetMathLibrary.BreakVector` (`SceneComponent.K2_GetComponentLocation` (`self.PositionPlayerBack`))))
  (bind (_returnvalue_x_2 _returnvalue_y_2 _returnvalue_z) (`KismetMathLibrary.BreakVector` (`self.K2_GetActorLocation` _as_bp_first_person_character_2)))
  (bind (_relativerotation_roll _relativerotation_pitch _relativerotation_yaw) (`KismetMathLibrary.BreakRotator` (`SceneComponent.RelativeRotation` (`self.Door`))))
  (bind (_relativerotation_roll_2 _relativerotation_pitch_2 _relativerotation_yaw_2) (`KismetMathLibrary.BreakRotator` (`SceneComponent.RelativeRotation` (`self.Door`))))
  ;[0.04167 0.04167 0.04167] Tick Ouverture Back
  (`self.K2_SetActorLocation` _as_bp_first_person_character_2 (`KismetMathLibrary.MakeVector` _returnvalue_x _returnvalue_y _returnvalue_z) false false)
  (if (`/Game/TheDoorsGame/Blueprints/Player/BP_FirstPersonCharacter.isHoldingLMB` _as_bp_first_person_character)
    (if (<= _relativerotation_yaw 0.0)
      (`self.StopDoorInteractionF`)
      (elif (>= _relativerotation_yaw 70.0)
        (`self.OpenDoorCompletely` true)
        (else
          (`SceneComponent.K2_AddRelativeRotation` (`self.Door`) (`KismetMathLibrary.MakeRotator` 0.0 0.0 (* (`/Game/TheDoorsGame/Blueprints/Player/BP_FirstPersonCharacter.ForwardBackward` (`self.As BP First Person Character`)) 0.3)) false false))))
    (elif (== (`/Game/TheDoorsGame/Blueprints/Player/BP_FirstPersonCharacter.ForwardBackward` _as_bp_first_person_character) -1.0)
      (`self.CloseDoor` :!label _label)
      (elif (or (>= _relativerotation_yaw_2 30.0) (and (>= _relativerotation_yaw_2 20.0) (== (`/Game/TheDoorsGame/Blueprints/Player/BP_FirstPersonCharacter.ForwardBackward` (`self.As BP First Person Character`)) 1.0)))
        (`self.OpenDoorCompletely` true)
        (else
          (goto _label))))))

(fn `TickOuvertureFront`
  (bind _as_bp_first_person_character (`self.As BP First Person Character`))
  (bind (_returnvalue_x _returnvalue_y _returnvalue_z) (`KismetMathLibrary.BreakVector` (`self.K2_GetActorLocation` _as_bp_first_person_character)))
  (bind (_returnvalue_x_2 _returnvalue_y_2) (`KismetMathLibrary.BreakVector` (`SceneComponent.K2_GetComponentLocation` (`self.PositionPlayerFront`))))
  (bind (_relativerotation_roll _relativerotation_pitch _relativerotation_yaw) (`KismetMathLibrary.BreakRotator` (`SceneComponent.RelativeRotation` (`self.Door`))))
  (bind _forwardbackward (`/Game/TheDoorsGame/Blueprints/Player/BP_FirstPersonCharacter.ForwardBackward` (`self.As BP First Person Character`)))
  (bind (_relativerotation_roll_2 _relativerotation_pitch_2 _relativerotation_yaw_2) (`KismetMathLibrary.BreakRotator` (`SceneComponent.RelativeRotation` (`self.Door`))))
  ;[0.04167 0.04167 0.04167] Tick Ouverture Front
  (`self.K2_SetActorLocation` _as_bp_first_person_character (`KismetMathLibrary.MakeVector` _returnvalue_x_2 _returnvalue_y_2 _returnvalue_z) false false)
  (if (`/Game/TheDoorsGame/Blueprints/Player/BP_FirstPersonCharacter.isHoldingLMB` (`self.As BP First Person Character`))
    (if (>= _relativerotation_yaw_2 0.0)
      (`self.StopDoorInteractionF`)
      (elif (not (<= _relativerotation_yaw_2 -70.0))
        (`SceneComponent.K2_AddRelativeRotation` (`self.Door`) (`KismetMathLibrary.MakeRotator` 0.0 0.0 (* (`/Game/TheDoorsGame/Blueprints/Player/BP_FirstPersonCharacter.ForwardBackward` (`self.As BP First Person Character`)) -0.3)) false false)
        (else
          (`self.OpenDoorCompletely` false))))
    (elif (== _forwardbackward -1.0)
      (`self.CloseDoor` :!label _label)
      (elif (or (<= _relativerotation_yaw -30.0) (and (<= _relativerotation_yaw -20.0) (== _forwardbackward 1.0)))
        (`self.OpenDoorCompletely` false)
        (else
          (goto _label))))))

(fn `UserConstructionScript`)